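; BP_FalseHammer is an activatable hammer hazard that fakes its strike by swapping between two pairs of cube meshes rather than moving.
; On Activate it waits a configurable delay, shows the strike cubes, hides the rest cubes and sends a zero-damage Hit to BPI_Hittable actors overlapping its box.
; Tick watches the Hit flag and restores the rest pose half a second later.
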(event EventBeginPlay
  (Rendering|SetVisibility (Variables|Default|GetCube3) false false)
  (Rendering|SetVisibility (Variables|Default|GetCube4) false false))

(event Collision|EventActorBeginOverlap
  (params (OtherActor :type Actor%20Object%20Reference)))

(event EventTick
  (params (DeltaSeconds :type Float%20%28single-precision%29))
  (if (Variables|Default|Gethit)
    (Utilities|FlowControl|Delay 0.5)
    (Rendering|SetVisibility (Variables|Default|GetCube3) false false)
    (Rendering|SetVisibility (Variables|Default|GetCube4) false false)
    (Rendering|SetVisibility (Variables|Default|GetCube1) true false)
    (Rendering|SetVisibility (Variables|Default|GetCube2) true false)
    (Variables|Default|Sethit false)))

(event EventActivate
  (Utilities|FlowControl|Delay (Variables|Default|Getdelay))
  (Rendering|SetVisibility (Variables|Default|GetCube3) true false)
  (Rendering|SetVisibility (Variables|Default|GetCube4) true false)
  (Rendering|SetVisibility (Variables|Default|GetCube1) false false)
  (Rendering|SetVisibility (Variables|Default|GetCube2) false false)
  (Variables|Default|Sethit true)
  (for _array_element (Collision|GetOverlappingActors (Variables|Default|GetBox) 0 :!class /Script/Engine.PrimitiveComponent)
    (bind _asbpi_hittable (Utilities|Casting|CastToBPI_Hittable _array_element))
    (Default|Hit _asbpi_hittable 0.0)))

(fn ConstructionScript)