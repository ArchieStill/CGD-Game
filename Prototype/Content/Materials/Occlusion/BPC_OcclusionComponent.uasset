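; Actor component that manages a material occlusion effect on a static mesh actor, for objects between player and camera.
; BeginPlay creates a dynamic MI_Environment instance and assigns it to the owner's first material slot.
; Hit flags the object as occluded and resets a frame counter.
; Tick counts frames without hits and zeroes ApplyEffect once the short threshold passes; enabling the effect happens outside this graph.
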(event Custom|Hit
  ;[0 0 0] Used to disable occlusion effect when no longer in between Player and Camera
  (if (Variables|Default|GetOccluled)
    _
    (else
      (Variables|Default|SetOccluled true)))
  (Variables|Default|SetTime 0))

(event EventBeginPlay
  ;[0 0 0] Creates Dynamic Material Instance so the parameters can be adjusted at runtime.
  (bind _returnvalue (Rendering|Material|CreateDynamicMaterialInstance "/Game/Materials/Occlusion/MI_Environment.MI_Environment" "None" "None" :!class /Script/Engine.KismetMaterialLibrary))
  (Variables|Default|SetDynamicMaterialInstance _returnvalue)
  (bind _asstatic_mesh_actor (Utilities|Casting|CastToStaticMeshActor (Components|GetOwner)))
  (Rendering|Material|SetMaterial (Variables|/Script/Engine.StaticMeshActor|GetStaticMeshComponent _asstatic_mesh_actor) 0 _returnvalue))

(event EventTick
  (params (DeltaSeconds :type Float%20%28single-precision%29))
  ;[0 0 0] Checks each frame if object should be occluded or not.
  (if (Variables|Default|GetOccluled)
    (bind _result (Math|Integer|IncrementInt (Variables|Default|GetTime))
      (:%20%20
        (if (>= _result 2)
          (Rendering|Material|SetScalarParameterValue (Variables|Default|GetDynamicMaterialInstance) "ApplyEffect" 0.0 :!class /Script/Engine.MaterialInstanceDynamic)
          (Variables|Default|SetOccluled false))))))