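; BP_Pushable is an actor that slides one grid-like step along world X or Y, away from the player, when hit.
; The Hit event, whatever the hitting actor, picks the dominant axis of the offset from player 0 and sets a velocity, timer and target.
; Tick moves it for one second without sweeping, then snaps to the target; further hits are ignored while moving.
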(event EventBeginPlay)

(event Collision|EventActorBeginOverlap
  (params (OtherActor :type Actor%20Object%20Reference)))

(event EventHit
  (params (Damage :type Float%20%28double-precision%29))
  (bind _returnvalue (Game|GetPlayerCharacter 0))
  (bind _returnvalue_2 (Transformation|GetActorLocation))
  (bind _returnvalue_3 (Transformation|GetActorLocation _returnvalue))
  (bind _returnvalue_4 (- _returnvalue_2 _returnvalue_3))
  (bind _returnvalue_5 (Math|Vector|VectorGetAbs _returnvalue_4))
  (if (not (Variables|Default|Getmoving))
    (Variables|Default|Setmoving true)
    (if (> (.x _returnvalue_5) (.y _returnvalue_5))
      (if (> (.X (Math|Vector|BreakVector _returnvalue_4)) 0.0)
        (Variables|Default|SetVelocity "100.000000,0.000000,0.000000")
        (else
          (Variables|Default|SetVelocity "-100.000000,0.000000,0.000000")))
      (elif (> (.Y (Math|Vector|BreakVector _returnvalue_4)) 0.0)
        (Variables|Default|SetVelocity "0.000000,100.000000,0.000000")
        (else
          (Variables|Default|SetVelocity "0.000000,-100.000000,0.000000"))))
    (Variables|Default|SetmoveTimer 1.0)
    (Variables|Default|SetDesiredPos (+ (Transformation|GetActorLocation) (Variables|Default|GetVelocity)))))

(event EventTick
  (params (DeltaSeconds :type Float%20%28single-precision%29))
  (if (Variables|Default|Getmoving)
    (bind _output_get (Variables|Default|SetmoveTimer (- (Variables|Default|GetmoveTimer) DeltaSeconds)))
    (if (< _output_get 0.0)
      (Transformation|SetActorLocation (Variables|Default|GetDesiredPos) false false)
      (Variables|Default|Setmoving false)
      (else
        (Transformation|SetActorLocation (+ (Transformation|GetActorLocation) (* (Variables|Default|GetVelocity) DeltaSeconds)) false false)))))

(fn ConstructionScript)