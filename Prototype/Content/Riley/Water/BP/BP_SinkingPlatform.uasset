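; Platform actor that, once overlapped by BP_RisingWater, moves in step with the water's vertical travel range.
; On BeginPlay it finds the water actor, sets its Start and End heights just above the water's own, and snaps the platform to Start.
; The overlap plays a Timeline that lerps the platform to End, at a play rate inverse to the water's PlatformPlayRate.
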(event OnComponentBeginOverlap(Platform)
  (params (OverlappedComponent :type Primitive%20Component%20Object%20Reference) (OtherActor :type Actor%20Object%20Reference) (OtherComp :type Primitive%20Component%20Object%20Reference) (OtherBodyIndex :type Integer) (bFromSweep :type Boolean) (SweepResult :type Hit%20Result%20Structure%20%28by%20ref%29))
  (if (== (Utilities|GetClass (Variables|Default|GetRisingWater)) (Utilities|GetClass OtherActor))
    (bind _alpha (Timeline|Timeline Play)
      (:Update
        (Transformation|SetWorldLocation (Variables|Default|GetPlatform) (Math|Vector|Lerp(Vector) (Transformation|GetWorldLocation (Variables|Default|GetStart)) (Transformation|GetWorldLocation (Variables|Default|GetEnd)) _alpha) false false)))))

(event EventBeginPlay
  (bind _returnvalue (Actor|GetActorOfClass "/Game/Riley/Water/BP/BP_RisingWater.BP_RisingWater_C"))
  (Variables|Default|SetRisingWater _returnvalue)
  (CallFunction|SetStartEndLoc)
  (Transformation|SetWorldLocation (Variables|Default|GetPlatform) (Transformation|GetWorldLocation (Variables|Default|GetStart)) false false)
  (Components|Timeline|SetPlayRate (Variables|Default|GetTimeline) (/ 1.0 (Variables|/Game/Riley/Water/BP/BP_RisingWater.BP_RisingWater_C|GetPlatformPlayRate (Variables|Default|GetRisingWater)))))

(fn ConstructionScript)

(fn SetStartEndLoc
  (bind _start (Variables|Default|GetStart))
  (bind _end (Variables|Default|GetEnd))
  (bind _returnvalue (Transformation|GetWorldLocation _start))
  (bind _returnvalue_2 (Transformation|GetWorldLocation _end))
  ;[1 1 1] Setting start and end to be basically the same as the rising water bar a small gap allowing it to begin overlap at start
  (Transformation|SetWorldLocation _start (Math|Vector|MakeVector (.x _returnvalue) (.y _returnvalue) (+ (.z (Transformation|GetWorldLocation (Variables|/Game/Riley/Water/BP/BP_RisingWater.BP_RisingWater_C|GetStart (Variables|Default|GetRisingWater)))) 7e+01)) false false)
  (Transformation|SetWorldLocation _end (Math|Vector|MakeVector (.x _returnvalue_2) (.y _returnvalue_2) (+ (.z (Transformation|GetWorldLocation (Variables|/Game/Riley/Water/BP/BP_RisingWater.BP_RisingWater_C|GetEnd (Variables|Default|GetRisingWater)))) 7e+01)) false false))