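; BP_CliffCharacterCutscenes is a cutscene version of the Cliff character that holds one animation for its whole shot.
; On BeginPlay it checks the Run, Idle, Falling and NoAnim flags in that priority order and plays the matching looping animation directly on SkCliff.
; NoAnim calls PlayAnimation with no asset, and an AnimPlay setter is left unconnected.
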(event EventBeginPlay
  (if (Variables|Default|GetRun)
    (Components|Animation|PlayAnimation (Variables|Default|Getsk-Cliff) "/Game/ART+VISUALS/AnimationFolder/Run_Anim.Run_Anim" true)
    (elif (Variables|Default|GetIdle)
      (Components|Animation|PlayAnimation (Variables|Default|Getsk-Cliff) "/Game/ART+VISUALS/AnimationFolder/Idle_Anim.Idle_Anim" true)
      (elif (Variables|Default|GetFalling)
        (Components|Animation|PlayAnimation (Variables|Default|Getsk-Cliff) "/Game/ART+VISUALS/AnimationFolder/JumpAir_Anim.JumpAir_Anim" true)
        (elif (Variables|Default|GetNoAnim)
          (Components|Animation|PlayAnimation (Variables|Default|Getsk-Cliff) 0 true))))))

(fn ConstructionScript)