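; BP_Game_Instance is the game instance that owns save data, loading a BP_SaveGame from its slot synchronously on Init.
; LoadGameData creates a fresh save object when none exists, and calls OnGameLoaded only after an asynchronous load.
; SavethePlayer copies player data into the cached save and writes it through SaveGameData, synchronously or asynchronously.
; GetGameData exposes the cached save object.
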(event EventInit
  (CallFunction|LoadGameData false))

(event EventSaveGameData
  (params (Async :type Boolean))
  (bind _slot_name (Variables|Default|GetSlot%20Name))
  (bind _savedata (Variables|Default|GetSaveData))
  (if Async
    (|AsyncSaveGametoSlot _savedata _slot_name)
    (else
      (SaveGame|SaveGametoSlot _savedata _slot_name))))

(event EventLoadGameData
  (params (Async :type Boolean))
  (bind _returnvalue (SaveGame|DoesSaveGameExist (Variables|Default|GetSlot%20Name)))
  (if _returnvalue
    (if Async
      (bind _savegame (|AsyncLoadGamefromSlot (Variables|Default|GetSlot%20Name))
        (:Completed
          (bind _asbp_save_game (Utilities|Casting|CastToBP_SaveGame _savegame))
          (Variables|Default|SetSaveData _asbp_save_game)
          (Default|CallOnGameLoaded)))
      (else
        (bind _returnvalue_2 (SaveGame|LoadGamefromSlot (Variables|Default|GetSlot%20Name)))
        (bind _asbp_save_game_2 (Utilities|Casting|CastToBP_SaveGame _returnvalue_2))
        (Variables|Default|SetSaveData _asbp_save_game_2)))
    (else
      (bind _returnvalue_3 (SaveGame|CreateSaveGameObject "/Game/Sam/Save/BP_SaveGame.BP_SaveGame_C"))
      (Variables|Default|SetSaveData _returnvalue_3))))

(event EventSavethePlayer
  (params (PlayerSaveData :type S%20Player%20Save%20Structure) (Async :type Boolean))
  (Variables|/Game/Sam/Save/BP_SaveGame.BP_SaveGame_C|SetPlayerSave (Variables|Default|GetSaveData) PlayerSaveData)
  (CallFunction|SaveGameData Async))

(fn GetGameData
  (return (Variables|Default|GetSaveData)))