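; Hammer booby trap that swings an arm when set off and kills the third-person character on contact.
; SetOffTrap latches the triggered and hostile flags once, and Tick then plays a timeline that pitches ArmPivot.
; While hostile, KillBox overlaps run the character's death component sequence; the trap turns harmless when the swing finishes.
; The re-trigger gate lives here because moving it to the parent failed, per the author's note.
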(event OnComponentBeginOverlap(KillBox)
  (params (OverlappedComponent :type Primitive%20Component%20Object%20Reference) (OtherActor :type Actor%20Object%20Reference) (OtherComp :type Primitive%20Component%20Object%20Reference) (OtherBodyIndex :type Integer) (bFromSweep :type Boolean) (SweepResult :type Hit%20Result%20Structure%20%28by%20ref%29))
  (if (Variables|Default|GetTrapHostile)
    (bind _asbp_third_person_character (Utilities|Casting|CastToBP_ThirdPersonCharacter OtherActor))
    (Default|ExecuteDeathSequence (Actor|GetComponentbyClass _asbp_third_person_character "/Game/DeathSystem/BPC_DeathComponent.BPC_DeathComponent_C"))))

(event EventBeginPlay
  (|CallParentFunction) ; This node is disabled and will not be called.\nDrag off pins to build functionality.
)

(event Collision|EventActorBeginOverlap
  (params (OtherActor :type Actor%20Object%20Reference))
  (|CallParentFunction OtherActor) ; This node is disabled and will not be called.\nDrag off pins to build functionality.
)

(event EventTick
  (params (DeltaSeconds :type Float%20%28single-precision%29))
  (|CallParentFunction DeltaSeconds)
  (if (Variables|Default|GetTrapTriggered)
    (bind _newarmrotation (Timeline|ArmTimeline Play)
      (:Update
        (Transformation|SetRelativeRotation (Variables|Default|GetArmPivot) (Math|Rotator|MakeRotator 0.0 _newarmrotation 0.0) false false))
      (:Finished
        (Variables|Default|SetTrapHostile false)))))

(event EventSetOffTrap
  ;[1 1 1] Tried to add this to parent function but it got sassy and didn't work. Basic gate to stop re-triggers
  (if (not (Variables|Default|GetTrapTriggered))
    (Variables|Default|SetTrapTriggered true)
    (Variables|Default|SetTrapHostile true)))

(fn ConstructionScript
  (|CallParentFunction))