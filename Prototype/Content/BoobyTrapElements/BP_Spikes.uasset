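; BP_Spikes is a booby-trap floor spike that kills the player character by executing the death sequence on its death component.
; A TrapActivationBox entering DetectionBox arms the trap, plays a sound and, after a short delay, briefly opens a lethal window for HitBox overlaps.
; Tick drives the Spear_Movement timeline to move spear and HitBox vertically, restarting it continually while idle and clearing activation when it finishes.
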(event OnComponentBeginOverlap(DetectionBox)
  (params (OverlappedComponent :type Primitive%20Component%20Object%20Reference) (OtherActor :type Actor%20Object%20Reference) (OtherComp :type Primitive%20Component%20Object%20Reference) (OtherBodyIndex :type Integer) (bFromSweep :type Boolean) (SweepResult :type Hit%20Result%20Structure%20%28by%20ref%29))
  ;[1 1 1] Floor Trap Activate
  (bind _astrap_activation_box (Utilities|Casting|CastToTrapActivationBox OtherActor))
  (Default|GetFloorDetection _astrap_activation_box)
  (if (not (Variables|Default|GetFloorTrapActivated))
    (Variables|Default|SetFloorTrapActivated true)
    ;[1 1 1] Play Audio
    (Audio|PlaySound2D "/Game/Audio/Samples/Effects/Spike_Trap_v1.Spike_Trap_v1" 0.5 1.0 0.0 0 0)
    (Utilities|FlowControl|Delay 0.5)
    (Variables|Default|Setcan%20spike true)
    (Utilities|FlowControl|Delay 0.1)
    (Variables|Default|Setcan%20spike false)))

(event OnComponentBeginOverlap(HitBox)
  (params (OverlappedComponent :type Primitive%20Component%20Object%20Reference) (OtherActor :type Actor%20Object%20Reference) (OtherComp :type Primitive%20Component%20Object%20Reference) (OtherBodyIndex :type Integer) (bFromSweep :type Boolean) (SweepResult :type Hit%20Result%20Structure%20%28by%20ref%29))
  ;[1 1 1] Player Overlap
  (if (Variables|Default|Getcan%20spike)
    (bind _asbp_third_person_character (Utilities|Casting|CastToBP_ThirdPersonCharacter OtherActor))
    (Default|ExecuteDeathSequence (Actor|GetComponentbyClass _asbp_third_person_character "/Game/DeathSystem/BPC_DeathComponent.BPC_DeathComponent_C"))))

(event EventTick
  (params (DeltaSeconds :type Float%20%28single-precision%29))
  ;[1 1 1] Spear Movement
  (if (Variables|Default|GetFloorTrapActivated)
    (bind _movement (Timeline|Spear_Movement Play)
      (:Update
        (Transformation|SetRelativeLocation (Variables|Default|GetSpear) (Math|Vector|MakeVector 0.0 0.0 _movement) false false)
        (Transformation|SetRelativeLocation (Variables|Collision|GetHitBox) (Math|Vector|MakeVector 0.0 0.0 _movement) false false))
      (:Finished
        (Variables|Default|SetFloorTrapActivated false)))
    (else
      (Timeline|Spear_Movement PlayFromStart))))

(fn ConstructionScript
  (|CallParentFunction))