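; BP_DecoyTile is a booby-trap tile whose section wobbles and falls once the third-person character touches it.
; Overlap with DecoyCollider, or a guarded custom event, sets the TrapTriggered flag, which is never cleared here.
; While the flag is set, Tick keeps calling Play on the FallingPlatform timeline, whose tracks feed cumulative relative Y wobble and Z drop offsets to FallingSection.
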(event OnComponentBeginOverlap(decoyCollider)
  (params (OverlappedComponent :type Primitive%20Component%20Object%20Reference) (OtherActor :type Actor%20Object%20Reference) (OtherComp :type Primitive%20Component%20Object%20Reference) (OtherBodyIndex :type Integer) (bFromSweep :type Boolean) (SweepResult :type Hit%20Result%20Structure%20%28by%20ref%29))
  ;[1 1 1] Detect collision with falling platform
  (Utilities|Casting|CastToBP_ThirdPersonCharacter OtherActor)
  (Variables|Default|SetTrapTriggered true))

(event Custom|CustomEvent
  ;[1 1 1] Trap Triggered
  (if (not (Variables|Default|GetTrapTriggered))
    (Variables|Default|SetTrapTriggered true)))

(event EventBeginPlay
  (|CallParentFunction) ; This node is disabled and will not be called.\nDrag off pins to build functionality.
)

(event Collision|EventActorBeginOverlap
  (params (OtherActor :type Actor%20Object%20Reference))
  (|CallParentFunction OtherActor) ; This node is disabled and will not be called.\nDrag off pins to build functionality.
)

(event EventTick
  (params (DeltaSeconds :type Float%20%28single-precision%29))
  ;[1 1 1] Falling Platform
  (|CallParentFunction DeltaSeconds)
  (if (Variables|Default|GetTrapTriggered)
    (bind (_direction _falling _fallingwobble) (Timeline|Falling%20platform Play)
      (:Update
        (Transformation|AddRelativeLocation (Variables|Default|GetFalling_Section) (Math|Vector|MakeVector 0.0 _fallingwobble _falling) false false)))))

(fn ConstructionScript
  (|CallParentFunction))