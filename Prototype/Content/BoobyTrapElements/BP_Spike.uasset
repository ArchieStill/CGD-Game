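; BP_Spike is a booby trap element that moves a spear along its local vertical axis when the trap is set off.
; SetOffTrap uses the TrapTriggered flag as a one-way gate against re-triggers and prints a debug message.
; While that flag is set, Tick calls Play on the Spear_Movement timeline every frame, and its Movement track drives the Spear's relative Z location.
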(event EventBeginPlay
  (|CallParentFunction) ; This node is disabled and will not be called.\nDrag off pins to build functionality.
)

(event Collision|EventActorBeginOverlap
  (params (OtherActor :type Actor%20Object%20Reference))
  (|CallParentFunction OtherActor) ; This node is disabled and will not be called.\nDrag off pins to build functionality.
)

(event EventTick
  (params (DeltaSeconds :type Float%20%28single-precision%29))
  ;[1 1 1] Spear Movement
  (|CallParentFunction DeltaSeconds)
  (if (Variables|Default|GetTrapTriggered)
    (bind _movement (Timeline|Spear_Movement Play)
      (:Update
        (Transformation|SetRelativeLocation (Variables|Default|GetSpear) (Math|Vector|MakeVector 0.0 0.0 _movement) false false)))))

(event EventSetOffTrap
  ;[1 1 1] Tried to add this to parent function but it got sassy and didn't work. Basic gate to stop re-triggers
  (if (not (Variables|Default|GetTrapTriggered))
    (Variables|Default|SetTrapTriggered true)
    (Development|PrintString "ACTIVATE TRAOP")))

(fn ConstructionScript
  (|CallParentFunction))