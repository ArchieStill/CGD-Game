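; Poison dart projectile for booby traps that damages the third-person character on overlap and destroys itself.
; Tick line-traces a short way ahead, ignoring pressure plates and its owner, and destroys the dart on a hit, otherwise moving it forward by Speed per frame, unscaled by delta time.
; A one-second counter ages the dart until its life span, defaulted if unset, expires.
; Setter functions configure direction, speed and life span.
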(event OnComponentBeginOverlap(PlayerDetectCollidor)
  (params (OverlappedComponent :type Primitive%20Component%20Object%20Reference) (OtherActor :type Actor%20Object%20Reference) (OtherComp :type Primitive%20Component%20Object%20Reference) (OtherBodyIndex :type Integer) (bFromSweep :type Boolean) (SweepResult :type Hit%20Result%20Structure%20%28by%20ref%29))
  ;[1 1 1] Hacky way of ensuring player is detected when dart is firing
  (bind _asbp_third_person_character (Utilities|Casting|CastToBP_ThirdPersonCharacter OtherActor))
  (Default|TakeDamage _asbp_third_person_character 0.2)
  (Actor|DestroyActor self))

(event EventBeginPlay
  ;[1 1 1] If the Life Span is not set on creation automatically set it to 5, ensures program does not bug out
  (if (== (Variables|Default|GetLifeSpan) 0.0)
    (Variables|Default|SetLifeSpan 5.0))
  ;[1 1 1] Find any Pressure Plates and the owning Dart Box and ensure they are not considered in a line trace
  (bind _outactors (Actor|GetAllActorsOfClass "/Game/BoobyTrapElements/BP_PressurePlate.BP_PressurePlate_C"))
  (for _array_element _outactors
    (Utilities|Array|Add (Variables|Default|GetIgnoreActors) _array_element))
  (Utilities|Array|Add (Variables|Default|GetIgnoreActors) (Components|GetOwner)))

(event Collision|EventActorBeginOverlap
  (params (OtherActor :type Actor%20Object%20Reference)))

(event EventTick
  (params (DeltaSeconds :type Float%20%28single-precision%29))
  (bind _self self)
  (bind _self_2 self)
  (bind _defaultsceneroot (Variables|Default|GetDefaultSceneRoot _self_2))
  (bind _defaultsceneroot_2 (Variables|Default|GetDefaultSceneRoot _self))
  (bind _returnvalue (Transformation|GetWorldLocation _defaultsceneroot_2))
  ;[1 1 1] Check if the dart collided with something before anything, ensure it is destroyed on impact and does not cause errors
  (bind _outhit (Collision|LineTraceByChannel _returnvalue (+ (* (Math|Vector|GetForwardVector _defaultsceneroot_2) 2e+01) _returnvalue) "TraceTypeQuery1" false (Variables|Default|GetIgnoreActors) "None"))
  ;[1 1 1] WIP code for the dart breaking apart
  (if (.bblockinghit _outhit)
    (Actor|DestroyActor self)
    (else
      ;[1 1 1] Hard code the arrow moving along the direction it is pointing
      (Transformation|SetActorLocation (+ (* (Math|Vector|GetForwardVector _defaultsceneroot) (Variables|Default|GetSpeed)) (Transformation|GetWorldLocation _defaultsceneroot)) false false)
      ;[1 1 1] Increment timer that tracks a second passing, if a second passes access next stage
      (bind _output_get (Variables|Default|SetSecondTimer (+ DeltaSeconds (Variables|Default|GetSecondTimer))))
      (if (>= _output_get 1.0)
        ;[1 1 1] If a second passes, reset the second timer and check to see if the dart has existed for longer than its life span. If it has destroy the dart. If not, increment the age of the dart by one
        (Variables|Default|SetSecondTimer 0.0)
        (if (< (Variables|Default|GetCurrentAge) (Variables|Default|GetLifeSpan))
          (Variables|Default|SetCurrentAge (+ (Variables|Default|GetCurrentAge) 1.0))
          (else
            (Actor|DestroyActor)))))))

(fn ConstructionScript)

(fn SetFireDirection
  (params (Direction%20%28Rotation%29 :type Rotator))
  (Transformation|SetActorRotation Direction%20%28Rotation%29))

(fn SetDartLifeSpan
  (params (life%20Span%20%28seconds%29 :type Float%20%28double-precision%29))
  (Variables|Default|SetLifeSpan life%20Span%20%28seconds%29))

(fn SetDartSpeed
  (params (Speed :type Float%20%28double-precision%29))
  (Variables|Default|SetSpeed Speed))