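; BP_JumpTutorial is a tutorial actor that shows a jump widget above the third-person player character.
; The widget becomes visible on BeginPlay, then follows the character every Tick at a fixed height offset.
; It is hidden once the character's movement component reports falling, which covers any fall as well as a jump, and is not shown again.
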(event EventBeginPlay
  (Rendering|SetVisibility (Variables|Default|GetJumpWidget) true false))

(event EventTick
  (params (DeltaSeconds :type Float%20%28single-precision%29))
  (bind _jumpwidget (Variables|Default|GetJumpWidget))
  (bind _asbp_third_person_character (Utilities|Casting|CastToBP_ThirdPersonCharacter (Game|GetPlayerCharacter 0)))
  (Utilities|FlowControl|Sequence
    (:then_0
      (Transformation|SetWorldLocation _jumpwidget (Transformation|GetActorLocation _asbp_third_person_character) false false)
      (Transformation|AddWorldOffset _jumpwidget "0.000000,0.000000,150.000000" false false))
    (:then_1
      (if (AI|Components|NavMovement|IsFalling (Variables|/Script/Engine.Character|GetCharacterMovement _asbp_third_person_character))
        (Rendering|SetVisibility (Variables|Default|GetJumpWidget) false false)))))

(fn ConstructionScript)