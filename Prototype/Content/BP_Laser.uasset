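; BP_Laser is a laser beam actor that can be switched on and switches itself off once its lifetime expires.
; While active, it line-traces each tick along its arrow's forward vector and stretches the beam mesh's Z scale to the hit distance.
; Hit actors implementing BPI_LaserInteractable receive LaserHit with the impact location.
; SetActive resets the timer on activation and toggles the beam mesh's visibility.
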(event EventTick
  (params (DeltaSeconds :type Float%20%28single-precision%29))
  (bind _returnvalue (Transformation|GetActorLocation))
  (bind _staticmesh (Variables|Default|GetStaticMesh))
  (bind _returnvalue_2 (Transformation|GetWorldScale _staticmesh))
  (bind (_x _y) (Math|Vector|BreakVector _returnvalue_2))
  (if (Variables|Default|GetActive)
    (bind _output_get (Variables|Default|Settimer (+ DeltaSeconds (Variables|Default|Gettimer))))
    (if (> _output_get (Variables|Default|GetLifetime))
      (CallFunction|SetActive false)))
  (if (Variables|Default|GetActive)
    (bind (_outhit _returnvalue_3) (Collision|LineTraceForObjects _returnvalue (+ _returnvalue (* (Math|Vector|GetForwardVector (Variables|Default|GetArrow)) 1e+05)) (Utilities|Array|MakeArray "ObjectTypeQuery1" "ObjectTypeQuery3" "ObjectTypeQuery2" "ObjectTypeQuery4") false 0 "ForOneFrame"))
    (if _returnvalue_3
      (Transformation|SetWorldScale3D _staticmesh (Math|Vector|MakeVector _x _y (/ (.Distance (Collision|BreakHitResult _outhit)) 1e+02)))
      (bind _asbpi_laser_interactable (Utilities|Casting|CastToBPI_LaserInteractable (.HitActor (Collision|BreakHitResult _outhit))))
      (Default|LaserHit _asbpi_laser_interactable (.Location (Collision|BreakHitResult _outhit))))))

(fn ConstructionScript)

(fn SetActive
  (params (New%20Active :type Boolean))
  (bind _output_get (Variables|Default|SetActive New%20Active))
  (if _output_get
    (Variables|Default|Settimer 0.0))
  (Development|SetHiddeninGame (Variables|Default|GetStaticMesh) (not _output_get) false))