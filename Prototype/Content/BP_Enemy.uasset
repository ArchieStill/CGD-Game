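; Enemy Blueprint that resolves its charge attack against the third-person player character.
; When its Cube overlaps the player's CollisionCylinder while the blackboard's Charging flag is set, it checks whether the player is parrying.
; A parry damages the enemy, while an unparried hit damages the player and launches them upward along the enemy's forward direction.
; Both outcomes set the Hit blackboard key, and a parry also sets Parried.
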(event OnComponentBeginOverlap(Cube)
  (params (OverlappedComponent :type Primitive%20Component%20Object%20Reference) (OtherActor :type Actor%20Object%20Reference) (OtherComp :type Primitive%20Component%20Object%20Reference) (OtherBodyIndex :type Integer) (bFromSweep :type Boolean) (SweepResult :type Hit%20Result%20Structure%20%28by%20ref%29))
  (bind _returnvalue (Pawn|GetController))
  (bind _returnvalue_2 (Transformation|GetActorForwardVector))
  (bind _returnvalue_3 (AI|GetBlackboard _returnvalue))
  (bind _returnvalue_4 (* _returnvalue_2 1.25e+03))
  (bind (_x _y) (Math|Vector|BreakVector _returnvalue_4))
  (if (ScalableFloat|GetValueasBool (AI|GetBlackboard (Pawn|GetController)) (Utilities|Name|MakeLiteralName "Charging"))
    (bind _asbp_third_person_character (Utilities|Casting|CastToBP_ThirdPersonCharacter OtherActor))
    (if (== (Utilities|String|StringToName (Utilities|GetObjectName OtherComp)) "CollisionCylinder")
      (if (Variables|/Game/ThirdPerson/Blueprints/BP_ThirdPersonCharacter.BP_ThirdPersonCharacter_C|Getparrying _asbp_third_person_character)
        (CallFunction|TakeDamage 1.0)
        (AI|Components|Blackboard|SetValueasBool _returnvalue_3 (Utilities|Name|MakeLiteralName "Hit") true)
        (AI|Components|Blackboard|SetValueasBool _returnvalue_3 (Utilities|Name|MakeLiteralName "Parried") true)
        (else
          (Default|TakeDamage _asbp_third_person_character 4.0)
          (Character|LaunchCharacter _asbp_third_person_character (Math|Vector|MakeVector _x _y 7e+02) true true)
          (AI|Components|Blackboard|SetValueasBool (AI|GetBlackboard (Pawn|GetController)) (Utilities|Name|MakeLiteralName "Hit") true))))))

(event EventBeginPlay
  (|CallParentFunction))

(event Collision|EventActorBeginOverlap
  (params (OtherActor :type Actor%20Object%20Reference)))

(fn ConstructionScript)