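; BP_LaserRedirector is a laser puzzle piece that emits its own laser when another laser hits it.
; On BeginPlay it spawns an inactive BP_Laser at its Arrow component's location with the actor's rotation and attaches it to the Arrow.
; The LaserHit event activates that laser, and nothing in this Blueprint switches it off again.
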(event EventBeginPlay
  (bind _returnvalue (Game|SpawnActorfromClass "/Game/BP_Laser.BP_Laser_C" (Math|Transform|MakeTransform (Transformation|GetWorldLocation (Variables|Default|GetArrow)) (Transformation|GetActorRotation) "1.000000,1.000000,1.000000") "Undefined" "MultiplyWithRoot" 0 0))
  (bind _output_get (Variables|Default|SetLaser _returnvalue))
  (Default|SetActive _output_get false)
  (Transformation|AttachComponentToComponent _output_get (Variables|Default|GetArrow) "None" "KeepWorld" "KeepWorld" "KeepWorld" true))

(event EventLaserHit
  (params (Location :type Vector :default "0, 0, 0"))
  (Default|SetActive (Variables|Default|GetLaser) true))

(fn ConstructionScript)