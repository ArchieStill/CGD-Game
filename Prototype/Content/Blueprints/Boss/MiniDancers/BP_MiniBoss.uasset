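; BP_MiniBoss is a mini boss actor that travels along the level's BP_MB_Spline path from BeginPlay.
; It grabs the first spline actor found, then plays a Timeline at a rate of 1/TimeToComplete.
; Each update maps the Timeline alpha to spline distance and sets the actor's transform from world-space location and local-space rotation.
; Scale comes from the BossAttack3 component's relative scale.
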(event Custom|Move
  (bind _splineref (Variables|Default|GetSplineRef))
  (bind _spline (Variables|/Game/Blueprints/Boss/MiniDancers/BP_MB_Spline.BP_MB_Spline_C|GetSpline _splineref))
  (Components|Timeline|SetPlayRate (Variables|Default|GetTimeline) (/ 1.0 (Variables|Default|GetTimeToComplete)))
  (bind _move (Timeline|Timeline Play)
    (:Update
      (Transformation|SetActorTransform (Math|Transform|MakeTransform (Spline|GetLocationatDistanceAlongSpline _spline (Math|Float|Lerp 0.0 (Spline|GetSplineLength _spline) _move) "World") (Math|Rotator|MakeRotator (.roll (Spline|GetRotationatDistanceAlongSpline _spline (Math|Float|Lerp 0.0 (Spline|GetSplineLength _spline) _move) "Local")) (.pitch (Spline|GetRotationatDistanceAlongSpline _spline (Math|Float|Lerp 0.0 (Spline|GetSplineLength _spline) _move) "Local")) (.yaw (Spline|GetRotationatDistanceAlongSpline _spline (Math|Float|Lerp 0.0 (Spline|GetSplineLength _spline) _move) "Local"))) (Variables|/Script/Engine.SceneComponent|GetRelativeScale3D (Variables|Default|GetBossAttack3)))))))

(event EventBeginPlay
  (bind _returnvalue (Actor|GetActorOfClass "/Game/Blueprints/Boss/MiniDancers/BP_MB_Spline.BP_MB_Spline_C"))
  (Variables|Default|SetSplineRef _returnvalue)
  (CallFunction|Move))

(fn ConstructionScript)