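; BP_Cluster drives a repeating debris cluster strike, filed with the Boss assets, that begins as soon as it enters play.
; Each strike loops over all BP_SpawnCluster actors and gives each a one-in-four chance, via two chained random bools, to spawn a BP_DebrisCluster high above it.
; The strike event then waits a few seconds and calls itself again, with no stop condition.
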(event Custom|ClusterStrike
  ;[1 1 1] Cluster
  (bind _outactors (Actor|GetAllActorsOfClass "/Game/Blueprints/Boss/BP_SpawnCluster.BP_SpawnCluster_C"))
  (for _array_element _outactors
    (if (Math|Random|RandomBool)
      (if (Math|Random|RandomBool)
        (Game|SpawnActorfromClass "/Game/Blueprints/Boss/BP_DebrisCluster.BP_DebrisCluster_C" (Math|Transform|MakeTransform (Math|Vector|MakeVector (.x (Transformation|GetActorLocation _array_element)) (.y (Transformation|GetActorLocation _array_element)) (+ (.z (Transformation|GetActorLocation _array_element)) 4e+03)) "0, 0, 0" "1.000000,1.000000,1.000000") "Undefined" "MultiplyWithRoot" 0 0))))
  (Utilities|FlowControl|Delay 5.0)
  (CallFunction|ClusterStrike))

(event EventBeginPlay
  (CallFunction|ClusterStrike))

(event Collision|EventActorBeginOverlap
  (params (OtherActor :type Actor%20Object%20Reference)))

(event EventTick
  (params (DeltaSeconds :type Float%20%28single-precision%29)))

(fn ConstructionScript)