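; Boss-fight falling debris that spawns high above the player, with a ground shadow placed by a downward line trace.
; Tick sweeps it down until blocked: it kills the player, resolves debris collisions favoring powerup pieces, or lands.
; Empowered debris falls faster and spawns a shockwave on landing; blue powerup debris becomes a BP_ReinforceHammer pickup.
; Other landed debris stays until destroyed by the boss laser or Reset.
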(event Custom|empower
  (Variables|Default|SetFallspeed (* (Variables|Default|GetFallspeed) 1.5))
  (Variables|Default|Setempowered true))

(event Custom|Reset
  (bind _shadow (Variables|Default|Getshadow))
  (if (Utilities|IsValid _shadow)
    (Actor|DestroyActor _shadow))
  (Actor|DestroyActor))

(event EventBeginPlay
  ;[1 1 1] Spawns above the player
  (bind _returnvalue (Actor|GetActorOfClass "/Game/ThirdPerson/Blueprints/BP_ThirdPersonCharacter.BP_ThirdPersonCharacter_C"))
  (Transformation|SetActorLocation (Math|Vector|MakeVector (.x (Transformation|GetActorLocation _returnvalue)) (.y (Transformation|GetActorLocation _returnvalue)) (+ (.z (Transformation|GetActorLocation _returnvalue)) 2e+03)) false false)
  ;[1 1 1] Spawns shadow
  (bind _outhit (Collision|LineTraceForObjects (Math|Vector|MakeVector (.x (Transformation|GetActorLocation _returnvalue)) (.y (Transformation|GetActorLocation _returnvalue)) (+ (.z (Transformation|GetActorLocation _returnvalue)) 2e+03)) (- (Math|Vector|MakeVector (.x (Transformation|GetActorLocation _returnvalue)) (.y (Transformation|GetActorLocation _returnvalue)) (+ (.z (Transformation|GetActorLocation _returnvalue)) 2e+03)) "0.000000,0.000000,10000.000000") (Utilities|Array|MakeArray "ObjectTypeQuery1") false 0 "None"))
  (bind _returnvalue_2 (Game|SpawnActorfromClass "/Game/Blueprints/Boss/BP_DebrisShadow.BP_DebrisShadow_C" (Math|Transform|MakeTransform (.Location (Collision|BreakHitResult _outhit)) "0.000000,45.000000,0.000000" "1.000000,1.000000,1.000000") "Undefined" "MultiplyWithRoot" 0 0))
  (Variables|Default|Setshadow _returnvalue_2))

(event EventTick
  (params (DeltaSeconds :type Float%20%28single-precision%29))
  ;[1 1 1] Moves debris down if not on floor
  (if (not (Variables|Default|Getlanded))
    (bind _sweephitresult (Transformation|SetActorLocation (+ (* (Variables|Default|GetFallspeed) DeltaSeconds) (Transformation|GetActorLocation)) true false))
    (if (.bBlockingHit (Collision|BreakHitResult _sweephitresult))
      ;[1 1 1] Destroys the appropriate debris if 2 collide (prioritises keeping blue debris)
      (if (== (Utilities|GetClass (.HitActor (Collision|BreakHitResult _sweephitresult))) "BP_FallingDebris_C")
        (if (Variables|Default|GetIsPowerup)
          (bind _asbp_falling_debris (Utilities|Casting|CastToBP_FallingDebris (.HitActor (Collision|BreakHitResult _sweephitresult))))
          (Actor|DestroyActor _asbp_falling_debris)
          (else
            (Actor|DestroyActor (Variables|Default|Getshadow))
            (Actor|DestroyActor)))
        (else
          ;[1 1 1] Kills the player if it hits them
          (bind _asbp_third_person_character (Utilities|Casting|CastToBP_ThirdPersonCharacter (.HitActor (Collision|BreakHitResult _sweephitresult)))
            (:then
              (Default|ExecuteDeathSequence (Variables|/Game/ThirdPerson/Blueprints/BP_ThirdPersonCharacter.BP_ThirdPersonCharacter_C|GetBPC_Death%20Component _asbp_third_person_character)))
            (:CastFailed
              (Variables|Default|Setlanded true)
              (Actor|DestroyActor (Variables|Default|Getshadow))
              (if (Variables|Default|Getempowered)
                (Game|SpawnActorfromClass "/Game/Blueprints/Boss/Shockwave/BP_Shockwave.BP_Shockwave_C" (Math|Transform|MakeTransform (Transformation|GetWorldLocation (Variables|Default|Getcrystal%20spawn)) "0, 0, 0" "1.000000,1.000000,1.000000") "Undefined" "MultiplyWithRoot" 0 0))
              ;[1 1 1] Spawns a powerup if blue
              (if (Variables|Default|GetIsPowerup)
                (Game|SpawnActorfromClass "/Game/Blueprints/PuzzleObjects/BP_ReinforceHammer.BP_ReinforceHammer_C" (Math|Transform|MakeTransform (Transformation|GetActorLocation)) "Undefined" "MultiplyWithRoot" 0 0)
                (Actor|DestroyActor)))))))))

(event EventLaserHit
  (params (Location :type Vector :default "0, 0, 0") (Type :type Laser%20Type%20Structure))
  ;[1 1 1] destroys when hit by boss laser
  (Actor|DestroyActor))

(fn ConstructionScript)

(fn EnablePowerup
  (Rendering|Material|SetMaterial (Variables|Default|GetCube) 0 "/Game/Materials/M_Blue.M_Blue")
  (Variables|Default|SetIsPowerup true))