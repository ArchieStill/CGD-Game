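; BP_attackRing is a boss attack actor that damages the player character on overlap during a limited window.
; Tick counts down two timers: the hitbox timer clears CanHit when it expires, and the lifetime timer destroys the actor.
; While CanHit is true, a Box begin-overlap casts the other actor to BP_ThirdPersonCharacter and calls its TakeDamage with a fixed amount.
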(event OnComponentBeginOverlap(Box)
  (params (OverlappedComponent :type Primitive%20Component%20Object%20Reference) (OtherActor :type Actor%20Object%20Reference) (OtherComp :type Primitive%20Component%20Object%20Reference) (OtherBodyIndex :type Integer) (bFromSweep :type Boolean) (SweepResult :type Hit%20Result%20Structure%20%28by%20ref%29))
  (if (Variables|Default|GetCanHit)
    (bind _asbp_third_person_character (Utilities|Casting|CastToBP_ThirdPersonCharacter OtherActor))
    (Default|TakeDamage _asbp_third_person_character 1.0)))

(event EventTick
  (params (DeltaSeconds :type Float%20%28single-precision%29))
  (bind _output_get (Variables|Default|Sethtibox%20lifetime (- (Variables|Default|Gethtibox%20lifetime) DeltaSeconds)))
  (if (< _output_get 0.0)
    (Variables|Default|SetCanHit false))
  (bind _output_get_2 (Variables|Default|Setlifetime (- (Variables|Default|Getlifetime) DeltaSeconds)))
  (if (< _output_get_2 0.0)
    (Actor|DestroyActor)))

(fn ConstructionScript)