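; Boss shockwave actor that expands a torus horizontally and kills the player when caught inside its ring.
; A timeline started on BeginPlay drives the torus X/Y scale, then destroys the actor when finished.
; Each Tick compares player distance against the Inner and Outer marker distances, within a height tolerance, and triggers the death component.
; This distance check replaces overlap detection, whose handler is empty and old logic disconnected.
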(event OnComponentBeginOverlap(Torus_Shockwave)
  (params (OverlappedComponent :type Primitive%20Component%20Object%20Reference) (OtherActor :type Actor%20Object%20Reference) (OtherComp :type Primitive%20Component%20Object%20Reference) (OtherBodyIndex :type Integer) (bFromSweep :type Boolean) (SweepResult :type Hit%20Result%20Structure%20%28by%20ref%29)))

(event EventBeginPlay
  (bind _newtrack_0 (Timeline|Timeline_0 PlayFromStart)
    (:Update
      (Transformation|SetRelativeScale3D (Variables|Default|GetTorus_Shockwave) (Math|Vector|MakeVector _newtrack_0 _newtrack_0 1.0))
      (Physics|AddForce :Force "1.000000,0.000000,0.000000"))
    (:Finished
      (Actor|DestroyActor))))

(event EventTick
  (params (DeltaSeconds :type Float%20%28single-precision%29))
  (bind _returnvalue (Game|GetPlayerCharacter 0))
  (bind _returnvalue_2 (Transformation|GetActorLocation))
  (bind _returnvalue_3 (Transformation|GetActorLocation _returnvalue))
  (bind _returnvalue_4 (Math|Vector|Distance(Vector) _returnvalue_3 _returnvalue_2))
  (if (< (Math|Float|Absolute(Float) (- (.Z (Math|Vector|BreakVector _returnvalue_3)) (.z (Transformation|GetActorLocation)))) 2e+02)
    (if (and (> _returnvalue_4 (Math|Vector|Distance(Vector) _returnvalue_2 (Transformation|GetWorldLocation (Variables|Default|Getinner)))) (< _returnvalue_4 (Math|Vector|Distance(Vector) _returnvalue_2 (Transformation|GetWorldLocation (Variables|Default|Getouter)))))
      (bind _asbp_third_person_character (Utilities|Casting|CastToBP_ThirdPersonCharacter (Game|GetPlayerCharacter 0)))
      (Default|ExecuteDeathSequence (Variables|/Game/ThirdPerson/Blueprints/BP_ThirdPersonCharacter.BP_ThirdPersonCharacter_C|GetBPC_Death%20Component _asbp_third_person_character)))))

(fn ConstructionScript)