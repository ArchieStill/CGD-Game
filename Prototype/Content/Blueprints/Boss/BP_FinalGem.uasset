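; BP_FinalGem is a gem pickup, filed with the boss assets, that ends the level when the player collects it.
; After spawning, a half-speed Movement timeline moves it from its start position to the EndPos actor, lerping X and Y while a Height track adds a vertical arc scaled by MoveHeight.
; Once movement finishes, overlapping its sphere with the BP_ThirdPersonCharacter's capsule calls LevelEnd on that character.
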(event OnComponentBeginOverlap(Sphere)
  (params (OverlappedComponent :type Primitive%20Component%20Object%20Reference) (OtherActor :type Actor%20Object%20Reference) (OtherComp :type Primitive%20Component%20Object%20Reference) (OtherBodyIndex :type Integer) (bFromSweep :type Boolean) (SweepResult :type Hit%20Result%20Structure%20%28by%20ref%29))
  (if (Variables|Default|Getfinished)
    (bind _asbp_third_person_character (Utilities|Casting|CastToBP_ThirdPersonCharacter OtherActor))
    (if (== (Variables|/Script/Engine.Character|GetCapsuleComponent _asbp_third_person_character) OtherComp)
      (Default|LevelEnd _asbp_third_person_character "None"))))

(event EventBeginPlay
  (Utilities|FlowControl|DelayUntilNextTick)
  (Variables|Default|SetstartPos (Transformation|GetActorLocation))
  (Components|Timeline|SetPlayRate (Variables|Default|GetMovement) 0.5)
  (bind (_direction _movement _height) (Timeline|Movement PlayFromStart)
    (:Update
      (Transformation|SetActorLocation (Math|Vector|MakeVector (.x (Math|Vector|Lerp(Vector) (Variables|Default|GetstartPos) (Transformation|GetActorLocation (Variables|Default|GetendPos)) _movement)) (.y (Math|Vector|Lerp(Vector) (Variables|Default|GetstartPos) (Transformation|GetActorLocation (Variables|Default|GetendPos)) _movement)) (+ (.z (Variables|Default|GetstartPos)) (* _height (Variables|Default|GetmoveHeight)))) false false))
    (:Finished
      (Variables|Default|Setfinished true))))

(fn ConstructionScript)