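; Boss actor that alternates two sweeping laser attacks with a falling debris attack.
; BeginPlay spawns and attaches a BP_Laser typed from a data table; Tick runs the attack cycle through a CanAttack gate.
; Timelines turn the boss relative to the player and sweep the active laser in alternating directions.
; The debris attack glows the eyes and spawns three timed BP_FallingDebris; the crystal-enabling branch is disconnected.
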(event Custom|LaserAttack
  (params (backwards :type Boolean))
  (bind _returnvalue (Transformation|GetActorRotation))
  (bind _returnvalue_2 (Transformation|GetActorRotation))
  (Variables|Default|Setcan%20attack false)
  (Components|Timeline|SetPlayRate (Variables|Default|GetTimeline) 0.3)
  ;[1 1 1] Enables the laser
  (Default|SetActive (Variables|Default|GetLaser) true)
  (Components|Activation|SetActive (Variables|Default|GetNiagara) true false)
  (Variables|Default|SetrotationStart (.yaw (Transformation|GetActorRotation)))
  (bind _rotation (Timeline|Timeline PlayFromStart)
    (:Update
      (if backwards
        ;[1 1 1] minuses z rotation from the boss
        (Transformation|SetActorRotation (Math|Rotator|MakeRotator (.roll _returnvalue_2) (.pitch _returnvalue_2) (- (Variables|Default|GetrotationStart) (* _rotation (Variables|Default|GetrotationAmount)))))
        (else
          ;[1 1 1] Adds z rotation to the boss
          (Transformation|SetActorRotation (Math|Rotator|MakeRotator (.roll _returnvalue) (.pitch _returnvalue) (+ (Variables|Default|GetrotationStart) (* _rotation (Variables|Default|GetrotationAmount))))))))
    (:Finished
      ;[1 1 1] Disables the laser and sets the boss to be able to attack again
      (Default|SetActive (Variables|Default|GetLaser) false)
      (Variables|Default|Setcan%20attack true)
      (Components|Activation|SetActive (Variables|Default|GetNiagara) false false))))

(event Custom|Debris%20Attack
  ;[1 1 1] Summons 3 Debris, every other time, the middle one is a crystal
  (Rendering|Material|SetMaterial (Variables|Default|Geteyes) 0 "/Game/Materials/GlowRed.GlowRed")
  (Utilities|FlowControl|Delay 0.5)
  (Game|SpawnActorfromClass "/Game/Blueprints/Boss/BP_FallingDebris.BP_FallingDebris_C" (Math|Transform|MakeTransform "0, 0, 0" "0.000000,45.000000,0.000000") "AlwaysSpawn" "MultiplyWithRoot" 0 0)
  (Utilities|FlowControl|Delay 1.5)
  (bind _returnvalue (Game|SpawnActorfromClass "/Game/Blueprints/Boss/BP_FallingDebris.BP_FallingDebris_C" (Math|Transform|MakeTransform "0, 0, 0" "0.000000,45.000000,0.000000") "AlwaysSpawn" "MultiplyWithRoot" 0 0))
  (Utilities|FlowControl|Delay 1.5)
  (Game|SpawnActorfromClass "/Game/Blueprints/Boss/BP_FallingDebris.BP_FallingDebris_C" (Math|Transform|MakeTransform "0, 0, 0" "0.000000,45.000000,0.000000") "AlwaysSpawn" "MultiplyWithRoot" 0 0)
  (Variables|Default|Setcan%20attack true)
  (Variables|Default|SetspawnCrystal (not (Variables|Default|GetspawnCrystal)))
  (Rendering|Material|SetMaterial (Variables|Default|Geteyes) 0 "/Game/Materials/Transparent.Transparent"))

(event Custom|Rotate%20To%20Offset%20From%20Player
  (params (angle :type Float%20%28double-precision%29))
  (CallFunction|CalculateDesiredAngle angle)
  (bind _percent (Timeline|Timeline_0 PlayFromStart)
    (:Update
      (Transformation|SetActorRotation (Math|Rotator|MakeRotator 0.0 0.0 (+ (* _percent (Variables|Default|Getdesired%20rot%20amount)) (Variables|Default|Getstart%20angle)))))
    (:Finished
      (if (< (Variables|Default|Getdesired%20rot%20amount) 0.0)
        (Variables|Default|Setbackwards false)
        (else
          (Variables|Default|Setbackwards true))))))

(event Custom|RotateAngle
  (params (angle :type Float%20%28double-precision%29))
  (Variables|Default|Setstart%20angle (.yaw (Transformation|GetActorRotation)))
  (bind _percent (Timeline|Rotate PlayFromStart)
    (:Update
      (Transformation|SetActorRotation (Math|Rotator|MakeRotator 0.0 0.0 (+ (* _percent angle) (Variables|Default|Getstart%20angle)))))))

(event EventBeginPlay
  (bind _arrow (Variables|Default|GetArrow))
  ;[1 1 1] Setes up the laser
  ;;[1 1 1] was 17 scale
  (bind _returnvalue (Game|SpawnActorfromClass "/Game/Blueprints/PuzzleObjects/BP_Laser.BP_Laser_C" (Math|Transform|MakeTransform (Transformation|GetWorldLocation _arrow) (Transformation|GetWorldRotation _arrow) "0.000000,0.000000,1.000000") "Undefined" "MultiplyWithRoot" 0 0))
  (bind _output_get (Variables|Default|SetLaser _returnvalue))
  (Variables|/Game/Blueprints/PuzzleObjects/BP_Laser.BP_Laser_C|SetSelfSustaining _output_get true)
  (Default|AddActortoIgnore _output_get self)
  (Default|SetActive _output_get false)
  (bind _returnvalue_2 (Utilities|GetDataTableRow "/Game/LaserTypesTable.LaserTypesTable" (Utilities|Name|MakeLiteralName "Damage"))
    (:then
      (Default|SetLaserType _output_get _returnvalue_2)
      (Transformation|AttachActorToActor (Variables|Default|GetLaser) self "None" "KeepWorld" "KeepWorld" "KeepWorld" true)
      (Components|Activation|SetActive (Variables|Default|GetNiagara) false false))))

(event EventTick
  (params (DeltaSeconds :type Float%20%28single-precision%29))
  ;[1 1 1] repeatedly attacks
  (if (Variables|Default|Getcan%20attack)
    (Variables|Default|Setcan%20attack false)
    ;[1 1 1] Summons debris after 2 laser attacks
    (if (< (Variables|Default|Getlasers%20done) 2)
      ;[1 1 1] Performs a laser attack in alternating directions
      (if (Variables|Default|Get2nd%20laser)
        (Utilities|FlowControl|Delay 1.0)
        (else
          (Utilities|FlowControl|Delay 2.0)
          (CallFunction|RotatetoOffsetfromPlayer 67.5)
          (Utilities|FlowControl|Delay 1.0)))
      (CallFunction|LaserAttack (Variables|Default|Getbackwards))
      (Variables|Default|Setbackwards (not (Variables|Default|Getbackwards)))
      (Variables|Default|Set2nd%20laser (not (Variables|Default|Get2nd%20laser)))
      (Math|Integer|IncrementInt (Variables|Default|Getlasers%20done))
      (else
        (Variables|Default|Setlasers%20done 0)
        (CallFunction|RotatetoOffsetfromPlayer 0.0)
        (Utilities|FlowControl|Delay 1.0)
        (CallFunction|DebrisAttack)))))

(fn ConstructionScript)

(fn CalculateDesiredAngle
  (params (Angle :type Float%20%28double-precision%29))
  (bind _returnvalue (Transformation|GetActorRotation))
  (bind _returnvalue_2 (Game|GetPlayerCharacter 0))
  (bind _returnvalue_3 (Transformation|GetActorLocation))
  (bind _returnvalue_4 (Transformation|GetActorLocation _returnvalue_2))
  (bind _returnvalue_5 (Math|Rotator|FindLookatRotation _returnvalue_3 _returnvalue_4))
  (bind _returnvalue_6 (- (.yaw _returnvalue_5) (.yaw _returnvalue)))
  (Variables|Default|Setstart%20angle (.yaw (Transformation|GetActorRotation)))
  (if (< _returnvalue_6 0.0)
    (Variables|Default|Setdesired%20rot%20amount (+ _returnvalue_6 Angle))
    (else
      (Variables|Default|Setdesired%20rot%20amount (- _returnvalue_6 Angle)))))