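; Spike actor for the dark room boss that rises vertically and then holds in place.
; Tick switches on State: while rising it moves up by Speed, then clamps to MaxAltitude and becomes static.
; While static it counts SinkTimer down, but nothing in this graph starts the rise or acts on that timer.
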(event EventTick
  (params (DeltaSeconds :type Float%20%28single-precision%29))
  (bind _returnvalue (Transformation|GetActorLocation))
  (bind _max_altitude (Variables|Default|Getmax_altitude))
  (switch Utilities|FlowControl|Switch|SwitchonENM_SpikeState (Variables|Default|Getstate)
    (:NewEnumerator0
      (Variables|Default|Setsink_timer (- (Variables|Default|Getsink_timer) DeltaSeconds)))
    (:NewEnumerator1
      (Transformation|AddActorWorldOffset (Math|Vector|MakeVector 0.0 0.0 (* (Variables|Default|Getspeed) DeltaSeconds)))
      (Math|Float|CompareFloat (.z (Transformation|GetActorLocation)) _max_altitude
        (:>
          (Transformation|SetActorLocation (Math|Vector|MakeVector (.x _returnvalue) (.y _returnvalue) _max_altitude) false false)
          (Variables|Default|Setstate "NewEnumerator0"))))))

(fn ConstructionScript)