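; Area-of-effect actor that slows spinning platforms, bullets and basic turrets while they are inside its bounds.
; Overlap begin and end events cast to each type and write hard-coded slowed or normal values to platform speed, bullet speed or turret shot cooldown.
; When FollowPlayer is set through SetFollowPlayer, Tick copies the owner's X and Y each frame, keeping its own height, rotation and scale.
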(event OnComponentBeginOverlap(AreaOfEffect)
  (params (OverlappedComponent :type Primitive%20Component%20Object%20Reference) (OtherActor :type Actor%20Object%20Reference) (OtherComp :type Primitive%20Component%20Object%20Reference) (OtherBodyIndex :type Integer) (bFromSweep :type Boolean) (SweepResult :type Hit%20Result%20Structure%20%28by%20ref%29))
  ;[1 0.5776 0.002125] When an object enters the area of effect, it slows down as per established implemnentions
  (bind _asbp_spin_plat (Utilities|Casting|CastToBP_SpinPlat OtherActor)
    (:then
      (Variables|/Game/Blueprints/Objects/BP_SpinPlat.BP_SpinPlat_C|SetSpinPlatSpeed _asbp_spin_plat 1e+01))
    (:CastFailed
      (bind _asbp_bullet (Utilities|Casting|CastToBP_Bullet OtherActor)
        (:then
          (Variables|/Game/Blueprints/Projectiles/BP_ProjectileParent.BP_ProjectileParent_C|Setspeed _asbp_bullet 1e+02))
        (:CastFailed
          (bind _asbp_basic_turret (Utilities|Casting|CastToBP_BasicTurret OtherActor))
          (Variables|/Game/Blueprints/Enemies/BP_TurretParent.BP_TurretParent_C|Setmax_shot_cooldown _asbp_basic_turret 2.0))))))

(event OnComponentEndOverlap(AreaOfEffect)
  (params (OverlappedComponent :type Primitive%20Component%20Object%20Reference) (OtherActor :type Actor%20Object%20Reference) (OtherComp :type Primitive%20Component%20Object%20Reference) (OtherBodyIndex :type Integer))
  ;[1 0.5776 0.002125] When an object leaves the area of effect, it returns to its normal pace as per established implementations
  (bind _asbp_spin_plat (Utilities|Casting|CastToBP_SpinPlat OtherActor)
    (:then
      (Variables|/Game/Blueprints/Objects/BP_SpinPlat.BP_SpinPlat_C|SetSpinPlatSpeed _asbp_spin_plat 9e+01))
    (:CastFailed
      (bind _asbp_bullet (Utilities|Casting|CastToBP_Bullet OtherActor)
        (:then
          (Variables|/Game/Blueprints/Projectiles/BP_ProjectileParent.BP_ProjectileParent_C|Setspeed _asbp_bullet 1e+03))
        (:CastFailed
          (bind _asbp_basic_turret (Utilities|Casting|CastToBP_BasicTurret OtherActor))
          (Variables|/Game/Blueprints/Enemies/BP_TurretParent.BP_TurretParent_C|Setmax_shot_cooldown _asbp_basic_turret 1.0))))))

(event EventTick
  (params (DeltaSeconds :type Float%20%28single-precision%29))
  (bind _self self)
  (bind _returnvalue (Transformation|GetActorTransform _self))
  (bind _returnvalue_2 (Components|GetOwner _self))
  (bind _returnvalue_3 (Transformation|GetActorTransform _returnvalue_2))
  ;[1 0.5776 0.002125] If the component states the Area of Effect should be followed, the Area of Effect's X and Y co-ordinates are set every event tick to the player's X and Y. Have thought about making it so there's a raycast and the Area of Effect always stays on the ground but that seemed like overkill.
  (if (Variables|Default|GetFollow%20Player)
    (Transformation|SetActorTransform self (Math|Transform|MakeTransform (Math|Vector|MakeVector (.x (.location _returnvalue_3)) (.y (.location _returnvalue_3)) (.z (.location _returnvalue))) (.rotation _returnvalue) (.scale _returnvalue)))))

(fn ConstructionScript)

(fn SetFollowPlayer
  (params (Follow%20Player :type Boolean))
  (Variables|Default|SetFollow%20Player Follow%20Player))