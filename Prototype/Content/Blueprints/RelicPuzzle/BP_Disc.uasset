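; BP_Disc is the rolling piece of the relic tilt puzzle, playing an FMOD impact sound when its Ball component strikes walls.
; It finds the BP_Tilt_Demo1 actor on BeginPlay and reacts only to hits on that actor, excluding its Platform and Roof.
; A hit sounds only if speed drops past a threshold after a short delay, filtering out soft contacts.
; Rolling-sound logic is present but disconnected.
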(event OnComponentHit(Ball)
  (params (HitComponent :type Primitive%20Component%20Object%20Reference) (OtherActor :type Actor%20Object%20Reference) (OtherComp :type Primitive%20Component%20Object%20Reference) (NormalImpulse :type Vector :default "0, 0, 0") (Hit :type Hit%20Result%20Structure%20%28by%20ref%29))
  (bind _ball (Variables|Default|GetBall))
  (bind _tiltdemo (Variables|Default|GetTiltDemo))
  (bind _returnvalue (Transformation|GetComponentVelocity _ball))
  (bind _returnvalue_2 (Math|Vector|VectorLength _returnvalue))
  (if (== OtherActor _tiltdemo)
    (if (and (!= OtherComp (Variables|/Game/Blueprints/RelicPuzzle/BP_Tilt_Demo1.BP_Tilt_Demo1_C|GetPlatform _tiltdemo)) (!= OtherComp (Variables|/Game/Blueprints/RelicPuzzle/BP_Tilt_Demo1.BP_Tilt_Demo1_C|Getroof _tiltdemo)))
      (Variables|Default|SetBallVelocity (Math|Vector|VectorLength (Transformation|GetComponentVelocity (Variables|Default|GetBall))))
      (Utilities|FlowControl|Delay 0.1)
      (if (and (< _returnvalue_2 (Variables|Default|GetBallVelocity)) (> (Math|Float|Absolute(Float) (- _returnvalue_2 (Variables|Default|GetBallVelocity))) 35.0))
        (Class|FMODAudioComponent|Play (Variables|Default|GetFMODWallHit))))))

(event EventBeginPlay
  (bind _returnvalue (Actor|GetActorOfClass "/Game/Blueprints/RelicPuzzle/BP_Tilt_Demo1.BP_Tilt_Demo1_C"))
  (Variables|Default|SetTiltDemo _returnvalue))

(event Collision|EventActorBeginOverlap
  (params (OtherActor :type Actor%20Object%20Reference)))

(event EventTick
  (params (DeltaSeconds :type Float%20%28single-precision%29)))

(fn ConstructionScript)