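; BP_Tilt_Demo1 is a staged relic puzzle board where a BP_Disc hits triggers to advance through layouts.
; Component tags on the Platform's children pick which pieces each stage shows or hides by changing visibility and height.
; Each one-shot trigger lights part of the RelicStatue, with the first two also switching layouts.
; The final trigger plays explosion effects, makes the player jump, calls the statue's Spit and destroys the puzzle.
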(event OnComponentBeginOverlap(TriggerLvl1)
  (params (OverlappedComponent :type Primitive%20Component%20Object%20Reference) (OtherActor :type Actor%20Object%20Reference) (OtherComp :type Primitive%20Component%20Object%20Reference) (OtherBodyIndex :type Integer) (bFromSweep :type Boolean) (SweepResult :type Hit%20Result%20Structure%20%28by%20ref%29))
  ;[1 1 1] Comment
  (if (Class|GameplayStatics|ObjectIsA OtherActor "/Game/Blueprints/RelicPuzzle/BP_Disc.BP_Disc_C")
    (Actor|GetActorOfClass "/Game/Blueprints/RelicPuzzle/BP_Disc.BP_Disc_C")
    (Components|DestroyComponent (Variables|Default|GetTriggerLvl1))
    (Utilities|FlowControl|Delay 0.2)
    (CallFunction|Lvl1)
    (Rendering|SetVisibility (Variables|/Game/Blueprints/RelicPuzzle/BP_RelicStatue.BP_RelicStatue_C|GetPointLight (Variables|Default|GetRelicStatue)) true false)))

(event OnComponentBeginOverlap(TriggerLvl2)
  (params (OverlappedComponent :type Primitive%20Component%20Object%20Reference) (OtherActor :type Actor%20Object%20Reference) (OtherComp :type Primitive%20Component%20Object%20Reference) (OtherBodyIndex :type Integer) (bFromSweep :type Boolean) (SweepResult :type Hit%20Result%20Structure%20%28by%20ref%29))
  ;[1 1 1] Comment
  (if (Class|GameplayStatics|ObjectIsA OtherActor "/Game/Blueprints/RelicPuzzle/BP_Disc.BP_Disc_C")
    (Actor|GetActorOfClass "/Game/Blueprints/RelicPuzzle/BP_Disc.BP_Disc_C")
    (Components|DestroyComponent (Variables|Default|GetTriggerLvl2))
    (CallFunction|Lvl2)
    (Rendering|SetVisibility (Variables|/Game/Blueprints/RelicPuzzle/BP_RelicStatue.BP_RelicStatue_C|GetPointLight1 (Variables|Default|GetRelicStatue)) true false)))

(event OnComponentBeginOverlap(TriggerComplete)
  (params (OverlappedComponent :type Primitive%20Component%20Object%20Reference) (OtherActor :type Actor%20Object%20Reference) (OtherComp :type Primitive%20Component%20Object%20Reference) (OtherBodyIndex :type Integer) (bFromSweep :type Boolean) (SweepResult :type Hit%20Result%20Structure%20%28by%20ref%29))
  (if (Class|GameplayStatics|ObjectIsA OtherActor "/Game/Blueprints/RelicPuzzle/BP_Disc.BP_Disc_C")
    (Components|DestroyComponent (Variables|Default|GetTriggerComplete))
    (Effects|SpawnEmitteratLocation 0 "0, 0, 0")
    (Rendering|SetVisibility (Variables|/Game/Blueprints/RelicPuzzle/BP_RelicStatue.BP_RelicStatue_C|GetRectLight (Variables|Default|GetRelicStatue)) true false)
    (Utilities|FlowControl|Delay 0.3)
    (Effects|SpawnEmitteratLocation "/Game/StarterContent/Particles/P_Explosion.P_Explosion" (Transformation|GetWorldLocation (Variables|Default|GetPlatform)))
    (Audio|PlaySound2D "/Game/StarterContent/Audio/Explosion01.Explosion01" 1.0 1.0 0.0 0 0)
    (Character|Jump (Game|GetPlayerCharacter 0))
    (Default|Spit (Variables|Default|GetRelicStatue))
    (Actor|DestroyActor)))

(event Custom|DefaultLvl
  (for _array_element (Components|GetChildrenComponents (Variables|Default|GetPlatform) false)
    (if (Components|ComponentHasTag _array_element "DefaultShow")
      (Transformation|SetRelativeLocation _array_element (Math|Vector|MakeVector (.x (Variables|/Script/Engine.SceneComponent|GetRelativeLocation _array_element)) (.y (Variables|/Script/Engine.SceneComponent|GetRelativeLocation _array_element)) 1e+02) false false)
      (Rendering|SetVisibility _array_element true false)
      (else
        (Rendering|SetVisibility _array_element false false)))))

(event Custom|Lvl2
  (for _array_element (Components|GetChildrenComponents (Variables|Default|GetPlatform) false)
    (if (Components|ComponentHasTag _array_element "ShowLvl2")
      (Transformation|SetRelativeLocation _array_element (Math|Vector|MakeVector (.x (Variables|/Script/Engine.SceneComponent|GetRelativeLocation _array_element)) (.y (Variables|/Script/Engine.SceneComponent|GetRelativeLocation _array_element)) 1e+02) false false)
      (Rendering|SetVisibility _array_element true false)
      (elif (Components|ComponentHasTag _array_element "HideLvl2")
        (Transformation|SetRelativeLocation _array_element (Math|Vector|MakeVector (.x (Variables|/Script/Engine.SceneComponent|GetRelativeLocation _array_element)) (.y (Variables|/Script/Engine.SceneComponent|GetRelativeLocation _array_element)) 0.0) false false)
        (Rendering|SetVisibility _array_element false false)))))

(event Custom|Lvl1
  (for _array_element (Components|GetChildrenComponents (Variables|Default|GetPlatform) false)
    (if (Components|ComponentHasTag _array_element "ShowLvl1")
      (Transformation|SetRelativeLocation _array_element (Math|Vector|MakeVector (.x (Variables|/Script/Engine.SceneComponent|GetRelativeLocation _array_element)) (.y (Variables|/Script/Engine.SceneComponent|GetRelativeLocation _array_element)) 1e+02) false false)
      (Rendering|SetVisibility _array_element true false)
      (elif (Components|ComponentHasTag _array_element "HideLvl1")
        (Transformation|SetRelativeLocation _array_element (Math|Vector|MakeVector (.x (Variables|/Script/Engine.SceneComponent|GetRelativeLocation _array_element)) (.y (Variables|/Script/Engine.SceneComponent|GetRelativeLocation _array_element)) 0.0) false false)
        (Rendering|SetVisibility _array_element false false)))))

(event EventBeginPlay
  (CallFunction|DefaultLvl))

(event EventTick
  (params (DeltaSeconds :type Float%20%28single-precision%29)))

(fn ConstructionScript)