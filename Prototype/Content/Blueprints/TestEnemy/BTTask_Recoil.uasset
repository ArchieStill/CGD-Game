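; Behavior tree task for a test enemy that recoils it backward after being parried.
; On execute, if the Parried blackboard flag is set it writes a point behind the pawn to ChargePos; otherwise it finishes at once.
; Each tick it sweeps the pawn toward that point at fixed speed, snapping on arrival, finishing and clearing Parried.
; It also prints the remaining horizontal distance every tick.
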(event EventReceiveTickAI
  (params (OwnerController :type AI%20Controller%20Object%20Reference) (ControlledPawn :type Pawn%20Object%20Reference) (DeltaSeconds :type Float%20%28single-precision%29))
  (bind _returnvalue (Utilities|Name|MakeLiteralName "ChargePos"))
  (bind _returnvalue_2 (AI|GetBlackboard OwnerController))
  (bind _returnvalue_3 (Transformation|GetActorLocation ControlledPawn))
  (bind _returnvalue_4 (AI|Components|Blackboard|GetValueasVector _returnvalue_2 _returnvalue))
  (bind _returnvalue_5 (- _returnvalue_4 _returnvalue_3))
  (bind _returnvalue_6 (Math|Vector|VectorLengthXY _returnvalue_5))
  (Development|PrintString (Utilities|String|ToString(Float) _returnvalue_6))
  (if (< _returnvalue_6 (* DeltaSeconds 2e+03))
    (Transformation|SetActorLocation ControlledPawn _returnvalue_4 false false)
    (AI|BehaviorTree|FinishExecute true)
    (AI|Components|Blackboard|SetValueasBool _returnvalue_2 (Utilities|Name|MakeLiteralName "Parried") false)
    (else
      (Transformation|SetActorLocation ControlledPawn (+ _returnvalue_3 (* (Math|Vector|Normalize _returnvalue_5) DeltaSeconds 2e+03)) true false))))

(event EventReceiveExecuteAI
  (params (OwnerController :type AI%20Controller%20Object%20Reference) (ControlledPawn :type Pawn%20Object%20Reference))
  (bind _returnvalue (AI|GetBlackboard OwnerController))
  (if (ScalableFloat|GetValueasBool _returnvalue (Utilities|Name|MakeLiteralName "Parried"))
    (AI|Components|Blackboard|SetValueasVector _returnvalue (Utilities|Name|MakeLiteralName "ChargePos") (+ (Transformation|GetActorLocation ControlledPawn) (* (Transformation|GetActorForwardVector ControlledPawn) -2e+02)))
    (else
      (AI|BehaviorTree|FinishExecute true))))