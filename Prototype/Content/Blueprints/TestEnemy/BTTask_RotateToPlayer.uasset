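; Behavior tree task that turns BP_Enemy to face player 0 and sets a charge target.
; On execute it zeroes the enemy's RotatingMovement rate.
; Each tick it wraps the yaw difference between the look-at and control rotation, then rotates the actor at a fixed degrees-per-second rate.
; When within one step, it snaps the remainder, writes a point ahead of the pawn to ChargePos and finishes successfully.
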(event EventReceiveExecuteAI
  (params (OwnerController :type AI%20Controller%20Object%20Reference) (ControlledPawn :type Pawn%20Object%20Reference))
  (bind _asbp_enemy (Utilities|Casting|CastToBP_Enemy ControlledPawn))
  (Variables|/Script/Engine.RotatingMovementComponent|SetRotationRate (Variables|/Game/Blueprints/TestEnemy/BP_Enemy.BP_Enemy_C|GetRotatingMovement _asbp_enemy) "0, 0, 0"))

(event EventReceiveTickAI
  (params (OwnerController :type AI%20Controller%20Object%20Reference) (ControlledPawn :type Pawn%20Object%20Reference) (DeltaSeconds :type Float%20%28single-precision%29))
  (Variables|Default|SetControlled%20Pawn ControlledPawn)
  (Variables|Default|SetOwner%20Controller OwnerController)
  (Variables|Default|Setdt DeltaSeconds)
  (bind _output_get (Variables|Default|Setangle (- (.Yaw (Math|Rotator|BreakRotator (Math|Rotator|FindLookatRotation (Transformation|GetActorLocation ControlledPawn) (Transformation|GetActorLocation (Game|GetPlayerCharacter 0))))) (.Yaw (Math|Rotator|BreakRotator (Pawn|GetControlRotation ControlledPawn :!class /Script/Engine.Pawn))))))
  (if (< _output_get -1.8e+02)
    (Variables|Default|Setangle (+ (Variables|Default|Getangle) 3.6e+02))
    (elif (> _output_get 1.8e+02)
      (Variables|Default|Setangle (- (Variables|Default|Getangle) 3.6e+02))))
  (if (< (Math|Float|Absolute(Float) (Variables|Default|Getangle)) (* (Variables|Default|Getdt) 9e+01))
    (Class|Actor|AddActorWorldRotation (Variables|Default|GetControlled%20Pawn) (Math|Rotator|MakeRotator 0.0 0.0 (Variables|Default|Getangle)))
    (AI|Components|Blackboard|SetValueasVector (AI|GetBlackboard (Variables|Default|GetOwner%20Controller)) (Utilities|Name|MakeLiteralName "ChargePos") (+ (* (Transformation|GetActorForwardVector (Variables|Default|GetControlled%20Pawn)) 7.5e+02) (Transformation|GetActorLocation (Variables|Default|GetControlled%20Pawn))))
    (AI|BehaviorTree|FinishExecute true)
    (elif (< (Variables|Default|Getangle) 0.0)
      (Class|Actor|AddActorWorldRotation (Variables|Default|GetControlled%20Pawn) (Math|Rotator|MakeRotator 0.0 0.0 (* (Variables|Default|Getdt) -9e+01)))
      (else
        (Class|Actor|AddActorWorldRotation (Variables|Default|GetControlled%20Pawn) (Math|Rotator|MakeRotator 0.0 0.0 (* (Variables|Default|Getdt) 9e+01)))))))