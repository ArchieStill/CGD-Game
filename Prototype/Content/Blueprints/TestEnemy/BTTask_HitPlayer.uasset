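; Behavior tree task that makes a test enemy charge at the ChargePos blackboard location, finishing on a hit or on arrival.
; On execute it clears the Hit flag and sets Charging in the blackboard.
; Each tick it moves the pawn with a swept SetActorLocation at fixed speed, snapping to the target when within one step in XY.
; Either ending clears Charging and reports success; Hit is only read and reset here.
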(event EventReceiveExecuteAI
  (params (OwnerController :type AI%20Controller%20Object%20Reference) (ControlledPawn :type Pawn%20Object%20Reference))
  (bind _returnvalue (AI|GetBlackboard OwnerController))
  (AI|Components|Blackboard|SetValueasBool _returnvalue (Utilities|Name|MakeLiteralName "Hit") false)
  (AI|Components|Blackboard|SetValueasBool _returnvalue (Utilities|Name|MakeLiteralName "Charging") true))

(event EventReceiveTickAI
  (params (OwnerController :type AI%20Controller%20Object%20Reference) (ControlledPawn :type Pawn%20Object%20Reference) (DeltaSeconds :type Float%20%28single-precision%29))
  (bind _returnvalue (Utilities|Name|MakeLiteralName "ChargePos"))
  (bind _returnvalue_2 (AI|GetBlackboard OwnerController))
  (bind _returnvalue_3 (Utilities|Name|MakeLiteralName "Hit"))
  (bind _returnvalue_4 (Transformation|GetActorLocation ControlledPawn))
  (bind _returnvalue_5 (AI|Components|Blackboard|GetValueasVector _returnvalue_2 _returnvalue))
  (bind _returnvalue_6 (- _returnvalue_5 _returnvalue_4))
  (if (ScalableFloat|GetValueasBool _returnvalue_2 _returnvalue_3)
    (AI|Components|Blackboard|SetValueasBool _returnvalue_2 _returnvalue_3 false)
    (AI|BehaviorTree|FinishExecute true)
    (AI|Components|Blackboard|SetValueasBool _returnvalue_2 (Utilities|Name|MakeLiteralName "Charging") false)
    (elif (< (Math|Vector|VectorLengthXY _returnvalue_6) (* DeltaSeconds 2e+03))
      (Transformation|SetActorLocation ControlledPawn _returnvalue_5 false false)
      (AI|BehaviorTree|FinishExecute true)
      (AI|Components|Blackboard|SetValueasBool _returnvalue_2 (Utilities|Name|MakeLiteralName "Charging") false)
      (else
        (Transformation|SetActorLocation ControlledPawn (+ _returnvalue_4 (* (Math|Vector|Normalize _returnvalue_6) DeltaSeconds 2e+03)) true false)))))