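; Test component that draws beam effects linking its owner to the third-person player character.
; On BeginPlay it spawns two Niagara beams; Tick pins the first between owner and player, while SetBeamValues positions the second.
; Each beam's alpha ramps up slowly or down quickly from its own fade flags, which are not set here.
; Tick prints debug values for the first fade; line trace and energy orb logic is left unconnected.
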(event EventBeginPlay
  (bind _asbp_third_person_character (Utilities|Casting|CastToBP_ThirdPersonCharacter (Game|GetPlayerCharacter 0)))
  (Variables|Default|SetAs%20BP%20Third%20Person%20Character _asbp_third_person_character)
  (bind _returnvalue (Niagara|SpawnSystematLocation "/Game/Particles/DynamicBeam.DynamicBeam" (Transformation|GetActorLocation (Components|GetOwner))))
  (Variables|Default|SetBeam _returnvalue)
  (Class|NiagaraComponent|SetVariablePosition (Variables|Default|GetBeam) "Beam End" "0, 0, 0")
  (Effects|Components|ParticleSystem|SetColorParameter (Variables|Default|GetBeam) "Colour" (Utilities|Struct|MakeLinearColor 5.0 5e+01 5.0 0.0))
  (bind _returnvalue_2 (Niagara|SpawnSystematLocation "/Game/Particles/DynamicBeam.DynamicBeam" (Transformation|GetActorLocation (Components|GetOwner))))
  (bind _output_get (Variables|Default|SetBeam2 _returnvalue_2))
  (Class|NiagaraComponent|SetVariablePosition _output_get "Beam End" "0, 0, 0")
  (Effects|Components|ParticleSystem|SetColorParameter (Variables|Default|GetBeam2) "Colour" (Utilities|Struct|MakeLinearColor 5.0 5e+01 5.0 0.0)))

(event EventTick
  (params (DeltaSeconds :type Float%20%28single-precision%29))
  (Utilities|FlowControl|Sequence
    (:then_1
      ;[0 0 0] Fade beam in and out when toggled
      (Transformation|SetWorldLocation (Variables|Default|GetBeam) (Transformation|GetActorLocation (Components|GetOwner)) false true)
      (Class|NiagaraComponent|SetVariablePosition (Variables|Default|GetBeam) "Beam End" (Transformation|GetActorLocation (Variables|Default|GetAs%20BP%20Third%20Person%20Character)))
      (if (Variables|Default|GetFadeIn)
        (Variables|Default|SetAlphaFadeValue (+ (Variables|Default|GetAlphaFadeValue) (* DeltaSeconds 1.0)))
        (elif (Variables|Default|GetFadeOut)
          (Variables|Default|SetAlphaFadeValue (- (Variables|Default|GetAlphaFadeValue) (* DeltaSeconds 5.0)))))
      (bind _output_get (Variables|Default|SetAlphaFadeValue (Math|Float|Clamp(Float) (Variables|Default|GetAlphaFadeValue))))
      (Effects|Components|ParticleSystem|SetColorParameter (Variables|Default|GetBeam) "Colour" (Utilities|Struct|MakeLinearColor 5.0 3e+01 3e+01 _output_get)))
    (:then_2
      (Development|PrintString (Utilities|String|Append "Fade In: " (Utilities|String|ToString(Boolean) (Variables|Default|GetFadeIn))) true true "(R=0.000000,G=0.660000,B=1.000000,A=1.000000)" 0.001)
      (Development|PrintString (Utilities|String|Append "Fade Out: " (Utilities|String|ToString(Boolean) (Variables|Default|GetFadeOut))) true true "(R=0.000000,G=0.660000,B=1.000000,A=1.000000)" 0.001)
      (Development|PrintString (Utilities|String|Append "Fade Value: " (Utilities|String|ToString(Float) (Variables|Default|GetAlphaFadeValue))) true true "(R=0.000000,G=0.660000,B=1.000000,A=1.000000)" 0.001))
    (:then_3
      ;[0 0 0] Fade beam in and out when toggled
      (if (Variables|Default|GetFadeIn%202)
        (Variables|Default|SetAlphaFadeValue%202 (+ (Variables|Default|GetAlphaFadeValue%202) (* DeltaSeconds 1.0)))
        (elif (Variables|Default|GetFadeOut%202)
          (Variables|Default|SetAlphaFadeValue%202 (- (Variables|Default|GetAlphaFadeValue%202) (* DeltaSeconds 5.0)))))
      (bind _output_get_2 (Variables|Default|SetAlphaFadeValue%202 (Math|Float|Clamp(Float) (Variables|Default|GetAlphaFadeValue%202))))
      (Effects|Components|ParticleSystem|SetColorParameter (Variables|Default|GetBeam2) "Colour" (Utilities|Struct|MakeLinearColor 5.0 3e+01 3e+01 _output_get_2)))))

(fn SetBeamValues
  (params (start :type Vector) (end :type Vector))
  (Transformation|SetWorldLocation (Variables|Default|GetBeam2) start false true)
  (Class|NiagaraComponent|SetVariablePosition (Variables|Default|GetBeam2) "Beam End" end))