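; BP_SnakeDeathBox is a trigger volume that kills the third-person player character with a snake-type death.
; When the character's capsule overlaps DeathCollidor, it sets the DeathType parameter on the character's FMOD death audio, plays it, then runs the death component's death sequence.
; A setter stores a Death Box Manager reference, which the overlap logic does not use.
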(event OnComponentBeginOverlap(DeathCollidor)
  (params (OverlappedComponent :type Primitive%20Component%20Object%20Reference) (OtherActor :type Actor%20Object%20Reference) (OtherComp :type Primitive%20Component%20Object%20Reference) (OtherBodyIndex :type Integer) (bFromSweep :type Boolean) (SweepResult :type Hit%20Result%20Structure%20%28by%20ref%29))
  (bind _asbp_third_person_character (Utilities|Casting|CastToBP_ThirdPersonCharacter OtherActor))
  (if (== (Variables|/Script/Engine.Character|GetCapsuleComponent _asbp_third_person_character) OtherComp)
    (Class|FMODAudioComponent|SetParameter (Variables|/Game/ThirdPerson/Blueprints/BP_ThirdPersonCharacter.BP_ThirdPersonCharacter_C|GetFMODDeath _asbp_third_person_character) "DeathType" 2.0)
    (Class|FMODAudioComponent|Play (Variables|/Game/ThirdPerson/Blueprints/BP_ThirdPersonCharacter.BP_ThirdPersonCharacter_C|GetFMODDeath _asbp_third_person_character))
    (Default|ExecuteDeathSequence (Variables|/Game/ThirdPerson/Blueprints/BP_ThirdPersonCharacter.BP_ThirdPersonCharacter_C|GetBPC_Death%20Component _asbp_third_person_character))))

(event EventBeginPlay)

(event Collision|EventActorBeginOverlap
  (params (OtherActor :type Actor%20Object%20Reference)))

(event EventTick
  (params (DeltaSeconds :type Float%20%28single-precision%29)))

(fn ConstructionScript)

(fn SetDeathBoxManager
  (params (DeathBoxManagerReference :type BP%20Death%20Box%20Manager%20Object%20Reference))
  (Variables|Default|SetDeathBoxManagerReference DeathBoxManagerReference))