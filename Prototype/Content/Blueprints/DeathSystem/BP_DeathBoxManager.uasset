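; BP_DeathBoxManager is an actor that centralizes player death for the BP_DeathBox actors in the level.
; On BeginPlay it gathers every BP_DeathBox and registers itself as their manager.
; Its KillPlayer function plays an FMOD death sound, then casts the first player's pawn to BP_ThirdPersonCharacter and runs ExecuteDeathSequence on that character's BPC_DeathComponent.
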(event EventBeginPlay
  (bind _outactors (Actor|GetAllActorsOfClass "/Game/DeathSystem/BP_DeathBox.BP_DeathBox_C"))
  (bind _output_get (Variables|Default|SetBP_DeathBoxes _outactors))
  (for _array_element _output_get
    (Default|SetDeathBoxManager _array_element self)))

(event Collision|EventActorBeginOverlap
  (params (OtherActor :type Actor%20Object%20Reference)))

(event EventTick
  (params (DeltaSeconds :type Float%20%28single-precision%29)))

(fn ConstructionScript)

(fn KillPlayer
  (Class|FMODAudioComponent|Play (Variables|Default|GetFMODPlayerDeath))
  (bind _asbp_third_person_character (Utilities|Casting|CastToBP_ThirdPersonCharacter (Pawn|GetControlledPawn (Game|GetPlayerController (Game|GetPlayerState 0)))))
  (Default|ExecuteDeathSequence (Actor|GetComponentbyClass _asbp_third_person_character "/Game/DeathSystem/BPC_DeathComponent.BPC_DeathComponent_C")))