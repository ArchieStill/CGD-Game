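; BP_ReinforceHammer is a pickup that grants the third-person character a reinforced state.
; When the character's capsule overlaps its Sphere, it calls SetReinforced through the BPI_Hitter interface and destroys itself.
; A LaserHit event also destroys it without granting the effect.
; The Hit event is empty, with leftover reinforce and debug-print logic left disconnected.
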(event OnComponentBeginOverlap(Sphere)
  (params (OverlappedComponent :type Primitive%20Component%20Object%20Reference) (OtherActor :type Actor%20Object%20Reference) (OtherComp :type Primitive%20Component%20Object%20Reference) (OtherBodyIndex :type Integer) (bFromSweep :type Boolean) (SweepResult :type Hit%20Result%20Structure%20%28by%20ref%29))
  (bind _asbp_third_person_character (Utilities|Casting|CastToBP_ThirdPersonCharacter OtherActor))
  (if (== (Variables|/Script/Engine.Character|GetCapsuleComponent _asbp_third_person_character) OtherComp)
    (bind _asbpi_hitter (Utilities|Casting|CastToBPI_Hitter _asbp_third_person_character))
    (Default|SetReinforced _asbpi_hitter true)
    (Actor|DestroyActor)))

(event EventBeginPlay)

(event Collision|EventActorBeginOverlap
  (params (OtherActor :type Actor%20Object%20Reference)))

(event EventTick
  (params (DeltaSeconds :type Float%20%28single-precision%29)))

(event EventHit
  (params (Damage :type Float%20%28double-precision%29) (Hitter :type Actor%20Object%20Reference)))

(event EventLaserHit
  (params (Location :type Vector :default "0, 0, 0") (Type :type Laser%20Type%20Structure))
  (Actor|DestroyActor))

(fn ConstructionScript)