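; BP_Ball is a physics ball puzzle object that returns to its starting position when it falls out of the play area.
; It records the Sphere's world location on BeginPlay, then checks its height every tick against a hard-coded kill height.
; Below that height, it moves the Sphere back and zeroes its linear and angular velocity.
; GetSimulatedComponent exposes the Sphere as the simulated component.
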(event EventTick
  (params (DeltaSeconds :type Float%20%28single-precision%29))
  (bind _sphere (Variables|Default|GetSphere))
  (if (< (.Z (Math|Vector|BreakVector (Transformation|GetWorldLocation (Variables|Default|GetSphere)))) -6.5e+02)
    (Transformation|SetWorldLocation _sphere (Variables|Default|GetInitial%20Pos) false false)
    (Physics|SetPhysicsLinearVelocity _sphere "0, 0, 0" false "None")
    (Class|PrimitiveComponent|SetPhysicsAngularVelocityinDegrees _sphere "0, 0, 0" false "None")))

(event EventBeginPlay
  (Variables|Default|SetInitial%20Pos (Transformation|GetWorldLocation (Variables|Default|GetSphere))))

(fn ConstructionScript)

(fn GetSimulatedComponent
  (return (Variables|Default|GetSphere)))