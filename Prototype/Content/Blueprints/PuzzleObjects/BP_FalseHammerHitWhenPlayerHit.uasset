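; Puzzle statue "false hammer" that mirrors the player's hammer swing once activated, hitting objects and destroying a chase boulder in its trigger box.
; While active, its eyes show and its head turns toward the player; Niagara effects show the link.
; A received swing sends a timeline-driven beam from player to statue, then hits overlapping BPI_Hittable actors.
; Tick then plays swing and reset timelines and deactivates all BP_ActivateStatue actors.
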(event OnComponentBeginOverlap(Box)
  (params (OverlappedComponent :type Primitive%20Component%20Object%20Reference) (OtherActor :type Actor%20Object%20Reference) (OtherComp :type Primitive%20Component%20Object%20Reference) (OtherBodyIndex :type Integer) (bFromSweep :type Boolean) (SweepResult :type Hit%20Result%20Structure%20%28by%20ref%29))
  (bind _asbp_chase_boulder (Utilities|Casting|CastToBP_ChaseBoulder OtherActor))
  (Variables|/Game/Blueprints/BoulderChase/BP_ChaseBoulder.BP_ChaseBoulder_C|SetCanKill _asbp_chase_boulder false)
  (Variables|Default|SetBoulderInPlace true))

(event Custom|DestroyBoulder
  (if (Variables|Default|GetBoulderInPlace)
    (bind _asbp_chase_boulder (Utilities|Casting|CastToBP_ChaseBoulder (Variables|Default|GetBoulder)))
    (Transformation|SetWorldLocation (Variables|/Game/Blueprints/BoulderChase/BP_ChaseBoulder.BP_ChaseBoulder_C|GetSphere _asbp_chase_boulder) "10000.000000,1000000.000000,1000000.000000" false true)
    (Audio|Components|Audio|Play (Variables|/Game/Blueprints/BoulderChase/BP_ChaseBoulder.BP_ChaseBoulder_C|GetExplosionSFX _asbp_chase_boulder) 0.0)
    (Components|Activation|Activate (Variables|/Game/Blueprints/BoulderChase/BP_ChaseBoulder.BP_ChaseBoulder_C|GetExplosionFX _asbp_chase_boulder) false)
    (Variables|Default|SetBoulderInPlace false)))

(event Custom|ActivateHammer
  (bind _bpc_playerlinktest (Variables|Default|GetBPC_PlayerLinkTest))
  (bind _bpc_playerlinktest_2 (Variables|Default|GetBPC_PlayerLinkTest))
  (bind _returnvalue (Actor|GetActorOfClass "/Game/ThirdPerson/Blueprints/BP_ThirdPersonCharacter.BP_ThirdPersonCharacter_C"))
  (Variables|/Game/ThirdPerson/Blueprints/BP_ThirdPersonCharacter.BP_ThirdPersonCharacter_C|SetHammerConnected _returnvalue true)
  (Variables|/Game/Blueprints/BPC_PlayerLinkTest.BPC_PlayerLinkTest_C|SetFadeOut _bpc_playerlinktest_2 false)
  (Variables|/Game/Blueprints/BPC_PlayerLinkTest.BPC_PlayerLinkTest_C|SetFadeIn _bpc_playerlinktest_2 true)
  (Components|Activation|SetActive (Variables|Default|GetNiagara) true false)
  (bind _returnvalue_2 (Actor|GetActorOfClass "/Game/ThirdPerson/Blueprints/BP_ThirdPersonCharacter.BP_ThirdPersonCharacter_C"))
  (Components|Activation|SetActive (Variables|/Game/ThirdPerson/Blueprints/BP_ThirdPersonCharacter.BP_ThirdPersonCharacter_C|GetNiagara _returnvalue_2) true false)
  (Utilities|FlowControl|Delay 0.75)
  (Variables|/Game/Blueprints/BPC_PlayerLinkTest.BPC_PlayerLinkTest_C|SetFadeOut _bpc_playerlinktest true)
  (Variables|/Game/Blueprints/BPC_PlayerLinkTest.BPC_PlayerLinkTest_C|SetFadeIn _bpc_playerlinktest false))

(event Custom|Play%20False%20Hammer%20Swing%20Animation
  (bind _false_hammer_hammer (Variables|Default|GetFalse%20Hammer%20Hammer))
  (bind _relativerotation (Variables|/Script/Engine.SceneComponent|GetRelativeRotation _false_hammer_hammer))
  ;[1 1 1] temporary implementation so that the false hammer can swing the hammer down when it detects the player swinging their hammer
  (bind _newtrack_0 (Timeline|False%20Hammer%20Hit%20Animation PlayFromStart)
    (:Update
      (Transformation|SetRelativeRotation _false_hammer_hammer (Math|Rotator|MakeRotator _newtrack_0 (.pitch _relativerotation) (.yaw _relativerotation)) false false))
    (:Finished
      ;;[1 1 1] is played here because it does not work in a function
      (CallFunction|PlayFalseHammerResetAnimation))))

(event Custom|Play%20False%20Hammer%20Reset%20Animation
  (bind _false_hammer_hammer (Variables|Default|GetFalse%20Hammer%20Hammer))
  (bind _relativerotation (Variables|/Script/Engine.SceneComponent|GetRelativeRotation _false_hammer_hammer))
  ;[1 1 1] Temporary implementation so that the false hammer can reset the hammer to its initial location after swinging it
  (bind _newtrack_0 (Timeline|False%20Hammer%20Reset%20Animation PlayFromStart)
    (:Update
      (Transformation|SetRelativeRotation _false_hammer_hammer (Math|Rotator|MakeRotator _newtrack_0 (.pitch _relativerotation) (.yaw _relativerotation)) false false))))

(event Custom|Recieve%20swing
  (bind _returnvalue (Transformation|GetActorLocation))
  (bind _bpc_playerlinktest (Variables|Default|GetBPC_PlayerLinkTest))
  (bind _bpc_playerlinktest_2 (Variables|Default|GetBPC_PlayerLinkTest))
  (Components|Activation|SetActive (Variables|Default|GetNiagara) false false)
  (bind _returnvalue_2 (Actor|GetActorOfClass "/Game/ThirdPerson/Blueprints/BP_ThirdPersonCharacter.BP_ThirdPersonCharacter_C"))
  (Components|Activation|SetActive (Variables|/Game/ThirdPerson/Blueprints/BP_ThirdPersonCharacter.BP_ThirdPersonCharacter_C|GetNiagara _returnvalue_2) false false)
  (Variables|Default|SetBeam%20start (Transformation|GetActorLocation (Game|GetPlayerCharacter 0)))
  (Variables|/Game/Blueprints/BPC_PlayerLinkTest.BPC_PlayerLinkTest_C|SetFadeIn _bpc_playerlinktest_2 false)
  (Variables|/Game/Blueprints/BPC_PlayerLinkTest.BPC_PlayerLinkTest_C|SetFadeOut _bpc_playerlinktest_2 true)
  (Variables|/Game/Blueprints/BPC_PlayerLinkTest.BPC_PlayerLinkTest_C|SetFadeIn%202 _bpc_playerlinktest_2 true)
  (Variables|/Game/Blueprints/BPC_PlayerLinkTest.BPC_PlayerLinkTest_C|SetFadeOut%202 _bpc_playerlinktest_2 false)
  (bind _newtrack_0 (Timeline|signal%20line PlayFromStart)
    (:Update
      (if (> (Math|Vector|Distance(Vector) (Math|Vector|Lerp(Vector) (Variables|Default|GetBeam%20start) _returnvalue _newtrack_0) _returnvalue) (Variables|Default|GetBeamLength))
        (Default|SetBeamValues (Variables|Default|GetBPC_PlayerLinkTest) (+ (Math|Vector|Lerp(Vector) (Variables|Default|GetBeam%20start) _returnvalue _newtrack_0) (* (Math|Vector|Normalize (- (Transformation|GetActorLocation) (Math|Vector|Lerp(Vector) (Variables|Default|GetBeam%20start) _returnvalue _newtrack_0))) (Variables|Default|GetBeamLength))) (Math|Vector|Lerp(Vector) (Variables|Default|GetBeam%20start) _returnvalue _newtrack_0))
        (else
          (Default|SetBeamValues (Variables|Default|GetBPC_PlayerLinkTest) (Math|Vector|Lerp(Vector) (Variables|Default|GetBeam%20start) _returnvalue _newtrack_0) (Transformation|GetActorLocation)))))
    (:Finished
      (Variables|/Game/Blueprints/BPC_PlayerLinkTest.BPC_PlayerLinkTest_C|SetFadeIn%202 _bpc_playerlinktest false)
      (Variables|/Game/Blueprints/BPC_PlayerLinkTest.BPC_PlayerLinkTest_C|SetFadeOut%202 _bpc_playerlinktest true)
      (Utilities|FlowControl|Delay 0.0)
      (Variables|Default|Sethit true)
      (for _array_element (Collision|GetOverlappingActors (Variables|Default|GetBox) 0 :!class /Script/Engine.PrimitiveComponent)
        (bind _asbpi_hittable (Utilities|Casting|CastToBPI_Hittable _array_element))
        (Default|Hit _asbpi_hittable 0.0 self)
        (Game|Feedback|ClientPlayForceFeedback (Game|GetPlayerController 0) "/Game/Blueprints/Rumble/Boulder/FFE_Rumble_DestroyBoulder.FFE_Rumble_DestroyBoulder" "None" false false false)))))

(event EventBeginPlay
  ;[1 1 1] Hide the eyes which show linkage to the player
  (Rendering|SetVisibility (Variables|Default|GetFalse%20Hammer%20Eyes) false false)
  ;[1 1 1] Set a variable which stores the initial head world rotation, this is used to return the head to its default position when not active
  (Variables|Default|SetInitial%20False%20Hammer%20Head%20World%20Rotation (Transformation|GetWorldRotation (Variables|Default|GetFalse%20Hammer%20Head)))
  ;[1 1 1] Set a variable which stores the initial head relative rotation. This is used to remove rotations made in the viewport when calculating the rotation to face the player
  (Variables|Default|SetInitial%20False%20Hammer%20Head%20Relative%20Rotation (Variables|/Script/Engine.SceneComponent|GetRelativeRotation (Variables|Default|GetFalse%20Hammer%20Head)))
  (Components|Activation|SetActive (Variables|Default|GetNiagara) false false))

(event EventTick
  (params (DeltaSeconds :type Float%20%28single-precision%29))
  (if (Variables|Default|GetActive)
    ;[1 1 1] Activate the false hammer's eyes to show it's watching the player
    (Rendering|SetVisibility (Variables|Default|GetFalse%20Hammer%20Eyes) true false)
    ;[1 1 1] Function which makes the head of the false hammer look at the player
    (CallFunction|LookatPlayer DeltaSeconds)
    (if (Variables|Default|Gethit)
      ;[1 1 1] Plays two customiseable animations, one for the down swing of the hammer then one for the reset back to its original position
      (CallFunction|PlayFalseHammerSwingAnimation)
      (Variables|Default|SetActive false)
      ;[1 1 1] De activate the eyes after the player has swung the hammer
      (Rendering|SetVisibility (Variables|Default|GetFalse%20Hammer%20Eyes) false false)
      (bind _outactors (Actor|GetAllActorsOfClass "/Game/Blueprints/PuzzleObjects/BP_ActivateStatue.BP_ActivateStatue_C"))
      (for _array_element _outactors
        (Default|Deactivate _array_element)
        (if (Variables|Default|GetBoulderInPlace)
          (CallFunction|DestroyBoulder))
        (Variables|Default|Sethit false)))
    (else
      ;[1 1 1] Set the lcoation of the head to its original position if the false hammer is not active, interping for smooth transition between two rotated position
      (Transformation|SetWorldRotation (Variables|Default|GetFalse%20Hammer%20Head) (Class|KismetMathLibrary|RInterptoConstant (Transformation|GetWorldRotation (Variables|Default|GetFalse%20Hammer%20Head)) (Variables|Default|GetInitial%20False%20Hammer%20Head%20World%20Rotation) DeltaSeconds (Variables|Default|GetFalse%20Hammer%20Head%20Rotation%20Speed)) false false))))

(fn ConstructionScript)

(fn HitStuff
  (if (Variables|Default|GetActive)
    (CallFunction|RecieveSwing)))

(fn LookatPlayer
  (params (Delta%20Time :type Float%20%28double-precision%29))
  (bind _false_hammer_head (Variables|Default|GetFalse%20Hammer%20Head))
  (bind _returnvalue (Transformation|GetWorldRotation _false_hammer_head))
  ;[1 1 1] Need some sort of variable which references the player, this bit's a bit messy
  (bind _asbp_third_person_character (Utilities|Casting|CastToBP_ThirdPersonCharacter (Game|GetPlayerCharacter 0)))
  (Transformation|SetWorldRotation (Variables|Default|GetFalse%20Hammer%20Head) (Class|KismetMathLibrary|RInterptoConstant (Math|Rotator|MakeRotator (.roll _returnvalue) (.pitch _returnvalue) (.yaw _returnvalue)) (Math|Rotator|MakeRotator (.roll _returnvalue) (.pitch _returnvalue) (- (.yaw (Math|Rotator|FindLookatRotation (Transformation|GetWorldLocation (Variables|Default|GetFalse%20Hammer%20Head)) (Transformation|GetWorldLocation (Variables|/Script/Engine.Character|GetMesh _asbp_third_person_character)))) (.yaw (Variables|Default|GetInitial%20False%20Hammer%20Head%20Relative%20Rotation)))) Delta%20Time (Variables|Default|GetFalse%20Hammer%20Head%20Rotation%20Speed)) false false))