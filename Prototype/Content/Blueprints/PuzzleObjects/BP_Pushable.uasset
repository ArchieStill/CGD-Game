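; Pushable puzzle block that, when hit, slides away from the player along the dominant world X or Y axis until blocked.
; HitEvent box-traces for the stopping point and derives a travel timer from Speed, then Tick moves the cube and snaps it there.
; Tick also fakes gravity with traces and teleports.
; Activate returns the cube to the actor's location, and an optional Child attaches to it on BeginPlay.
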(event Custom|Hit%20Event
  (params (Damage :type Float%20%28double-precision%29))
  (bind _returnvalue (Game|GetPlayerCharacter 0))
  (bind _cube (Variables|Default|GetCube))
  (bind _cube_2 (Variables|Default|GetCube))
  (bind _returnvalue_2 (Transformation|GetActorLocation _returnvalue))
  (bind _returnvalue_3 (Transformation|GetWorldLocation _cube))
  (bind _returnvalue_4 (Transformation|GetWorldLocation _cube_2))
  (bind _returnvalue_5 (- _returnvalue_3 _returnvalue_2))
  (bind _returnvalue_6 (Math|Vector|VectorGetAbs _returnvalue_5))
  ;[1 1 1] Sets direction and destination for the block based on the players position when this was hit and how far in that direction it can travel
  (if (not (Variables|Default|Getmoving))
    (Variables|Default|Setmoving true)
    (if (> (.x _returnvalue_6) (.y _returnvalue_6))
      (if (> (.X (Math|Vector|BreakVector _returnvalue_5)) 0.0)
        (Variables|Default|SetDirection "1.000000,0.000000,0.000000")
        (else
          (Variables|Default|SetDirection "-1.000000,0.000000,0.000000")))
      (elif (> (.Y (Math|Vector|BreakVector _returnvalue_5)) 0.0)
        (Variables|Default|SetDirection "0.000000,1.000000,0.000000")
        (else
          (Variables|Default|SetDirection "0.000000,-1.000000,0.000000"))))
    (Variables|Default|Setmoving true)
    (bind _returnvalue_7 (Actor|GetActorOfClass "/Game/Models/Character/TempVenturerAnimatedModel.TempVenturerAnimatedModel_C"))
    (bind _returnvalue_8 (Actor|GetActorOfClass "/Game/ThirdPerson/Blueprints/TrapActivationBox.TrapActivationBox_C"))
    (bind _outhit (Class|KismetSystemLibrary|BoxTraceSingleforObjects (+ _returnvalue_4 (Variables|Default|GetDirection)) (+ _returnvalue_4 (* (Variables|Default|GetDirection) 1e+05)) (- (* (Transformation|GetActorScale3D) 5e+01) (* (Math|Vector|MakeVector (Math|Float|Absolute(Float) (.y (Variables|Default|GetDirection))) (Math|Float|Absolute(Float) (.x (Variables|Default|GetDirection))) 1.0) 2.0)) "0, 0, 0" (Utilities|Array|MakeArray "ObjectTypeQuery1" "ObjectTypeQuery2") false (Utilities|Array|MakeArray (Game|GetPlayerCharacter 0) _returnvalue_7 _returnvalue_8) "ForDuration" true))
    (if (> (.Distance (Collision|BreakHitResult _outhit)) 2.0)
      (Variables|Default|SetDesiredPos (.Location (Collision|BreakHitResult _outhit)))
      (Variables|Default|SetmoveTimer (/ (.Distance (Collision|BreakHitResult _outhit)) (Variables|Default|Getspeed)))
      (else
        (Variables|Default|Setmoving false)))))

(event EventBeginPlay
  (if (Variables|Default|Getdisablephysics)
    (Physics|SetSimulatePhysics (Variables|Default|GetCube) false))
  (if (Utilities|IsValid (Variables|Default|Getchild))
    (Transformation|AttachComponentToComponent (Variables|Default|Getchild) (Variables|Default|GetCube) "None" "KeepWorld" "KeepWorld" "KeepWorld" true)))

(event Collision|EventActorBeginOverlap
  (params (OtherActor :type Actor%20Object%20Reference)))

(event EventActivate
  ;[1 1 1] Resets cube position
  (Transformation|SetWorldLocation (Variables|Default|GetCube) (Transformation|GetActorLocation) false false))

(event EventTick
  (params (DeltaSeconds :type Float%20%28single-precision%29))
  (bind _returnvalue (Transformation|GetActorScale3D))
  (bind _returnvalue_2 (Game|GetPlayerCharacter 0))
  (bind _cube (Variables|Default|GetCube))
  (bind _cube_2 (Variables|Default|GetCube))
  (bind _gravity (Variables|Default|Getgravity))
  (bind _cube_3 (Variables|Default|GetCube))
  (bind _returnvalue_3 (Transformation|GetWorldLocation _cube_3))
  (bind _returnvalue_4 (Transformation|GetWorldLocation _cube))
  (bind _returnvalue_5 (* _returnvalue 5e+01))
  (bind _returnvalue_6 (* (Math|Vector|MakeVector 0.0 0.0 _gravity) DeltaSeconds))
  (bind _returnvalue_7 (+ _returnvalue_4 _returnvalue_6))
  ;[1 1 1] Moves the cube along in its direction and moves it down with gravity
  (bind _returnvalue_8 (Actor|GetActorOfClass "/Game/Models/Character/TempVenturerAnimatedModel.TempVenturerAnimatedModel_C"))
  (bind _returnvalue_9 (Actor|GetActorOfClass "/Game/ThirdPerson/Blueprints/TrapActivationBox.TrapActivationBox_C"))
  (bind _outhit (Collision|LineTraceForObjects _returnvalue_3 (- _returnvalue_3 (Math|Vector|MakeVector 0.0 0.0 (* (.z (Transformation|GetActorScale3D)) 5e+01))) (Utilities|Array|MakeArray "ObjectTypeQuery1" "ObjectTypeQuery2") false (Utilities|Array|MakeArray _returnvalue_8 _returnvalue_9 _returnvalue_2) "None"))
  (if (.bBlockingHit (Collision|BreakHitResult _outhit))
    (Transformation|SetWorldLocation (Variables|Default|GetCube) (+ (Transformation|GetWorldLocation (Variables|Default|GetCube)) (Math|Vector|MakeVector 0.0 0.0 (- (* (.z (Transformation|GetActorScale3D)) 5e+01) (.Distance (Collision|BreakHitResult _outhit))))) false true))
  (bind _outhit_2 (Class|KismetSystemLibrary|BoxTraceSingleforObjects _returnvalue_4 _returnvalue_7 (Math|Vector|MakeVector (- (.x _returnvalue_5) 2.0) (- (.y _returnvalue_5) 2.0) (.z _returnvalue_5)) "0, 0, 0" (Utilities|Array|MakeArray "ObjectTypeQuery1" "ObjectTypeQuery2") false (Utilities|Array|MakeArray (Variables|Default|Getchild) _returnvalue_8 _returnvalue_9 _returnvalue_2) "ForOneFrame" true))
  (if (.bBlockingHit (Collision|BreakHitResult _outhit_2))
    (Transformation|SetWorldLocation (Variables|Default|GetCube) (.Location (Collision|BreakHitResult _outhit_2)) false true)
    (else
      (Transformation|SetWorldLocation (Variables|Default|GetCube) _returnvalue_7 false true)))
  (bind _returnvalue_10 (Physics|GetPhysicsLinearVelocity _cube_2 "None"))
  (if (> (.z _returnvalue_10) 0.0)
    (Physics|SetPhysicsLinearVelocity _cube_2 (Math|Vector|MakeVector (.x _returnvalue_10) (.y _returnvalue_10) 0.0) false "None"))
  (if (Variables|Default|Getmoving)
    (bind _output_get (Variables|Default|SetmoveTimer (- (Variables|Default|GetmoveTimer) DeltaSeconds)))
    (if (< _output_get 0.0)
      (Transformation|SetWorldLocation (Variables|Default|GetCube) (Variables|Default|GetDesiredPos) false true)
      (Variables|Default|Setmoving false)
      (else
        (Transformation|SetWorldLocation (Variables|Default|GetCube) (+ (Transformation|GetWorldLocation (Variables|Default|GetCube)) (* (Variables|Default|GetDirection) DeltaSeconds (Variables|Default|Getspeed))) false true)))))

(fn ConstructionScript)

(fn Hit
  (params (Damage :type Float%20%28double-precision%29) (Hitter :type Actor%20Object%20Reference))
  (CallFunction|HitEvent 0.0)
  (return))