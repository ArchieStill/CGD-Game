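; Guardian demo puzzle actor that projects a laser-like static mesh toward a Target actor and destroys itself on its Hit event.
; Each Tick rotates the mesh with LookAt along its Z axis, resets its thin cross-section, then stretches Z by the distance to the target.
; The beam length comes straight from the target's location, with no trace for blocking hits despite the inline note.
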(event EventTick
  (params (DeltaSeconds :type Float%20%28single-precision%29))
  (bind _staticmesh (Variables|Default|GetStaticMesh))
  (bind _staticmesh_2 (Variables|Default|GetStaticMesh))
  (bind _target (Variables|Default|Gettarget))
  (bind _staticmesh_3 (Variables|Default|GetStaticMesh))
  (bind _returnvalue (Transformation|GetWorldScale _staticmesh_2))
  (bind _rootcomponent (Variables|/Script/Engine.Actor|GetRootComponent _target))
  (bind (_x _y) (Math|Vector|BreakVector _returnvalue))
  (bind _returnvalue_2 (Transformation|GetWorldLocation _rootcomponent))
  (Transformation|SetWorldTransform _staticmesh_3 (Class|KismetAnimationLibrary|Lookat (Transformation|GetWorldTransform _staticmesh) _returnvalue_2 "0.000000,0.000000,1.000000" false "0, 0, 0" 0.0) false false)
  (Transformation|SetWorldScale3D _staticmesh_3 "0.200000,0.200000,1.000000")
  ;[1 1 1] Scales the laser to reach the blocking hit
  (Transformation|SetWorldScale3D _staticmesh_2 (Math|Vector|MakeVector _x _y (/ (Math|Vector|Distance(Vector) (Transformation|GetWorldLocation _staticmesh) _returnvalue_2) 1e+02))))

(event EventHit
  (params (Damage :type Float%20%28double-precision%29) (Hitter :type Actor%20Object%20Reference))
  (Actor|DestroyActor))

(fn ConstructionScript)