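; BP_Switch is a puzzle switch that toggles a list of linked objects on and off when hit.
; Each hit, while CanUse is true, alternately calls Activate or Deactivate on ObjectsToActivate through BPI_Activateable, then a timeline presses the button top down and back up.
; Tick runs a cooldown timer, but nothing here clears CanUse, so it never blocks hits.
; Older button timelines and red/blue material swaps remain unconnected.
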(event EventBeginPlay
  ;[1 1 1] Sets Initial height
  (Variables|Default|Setstart%20height (.Z (Math|Vector|BreakVector (Transformation|GetWorldLocation (Variables|Default|GetButton_Square_Top)))))
  (Variables|Default|Settimer (Variables|Default|Getcooldown)))

(event EventHit
  (params (Damage :type Float%20%28double-precision%29) (Hitter :type Actor%20Object%20Reference))
  (bind _button_square_top (Variables|Default|GetButton_Square_Top))
  (bind _returnvalue (Transformation|GetWorldLocation _button_square_top))
  (bind (_x _y) (Math|Vector|BreakVector _returnvalue))
  ;[1 1 1] Activates "object to activate" if inactive
  (if (Variables|Default|Getcan%20use)
    (if (Variables|Default|Getactive)
      (for _array_element (Variables|Default|Getobjects%20to%20activate)
        (bind _asbpi_activateable (Utilities|Casting|CastToBPI_Activateable _array_element)
          (:then
            (Default|Deactivate _asbpi_activateable))
          (:CastFailed
            (Development|PrintString "cast failed"))))
      (Variables|Default|Setactive false)
      ;[1 1 1] Pushes the button down/up
      (bind _height (Timeline|Timeline_2 Play)
        (:Update
          (Transformation|SetWorldLocation (Variables|Default|GetButton_Square_Top) (Math|Vector|MakeVector _x _y (+ (* (Variables|Default|Getmove%20amount) _height) (Variables|Default|Getstart%20height))) false false))
        (:Finished
          (if (> _height 0.0)
            (Timeline|Timeline_2 Reverse))))
      (else
        (for _array_element_2 (Variables|Default|Getobjects%20to%20activate)
          (bind _asbpi_activateable_2 (Utilities|Casting|CastToBPI_Activateable _array_element_2)
            (:then
              (Default|Activate _asbpi_activateable_2))
            (:CastFailed
              (Development|PrintString "cast failed"))))
        (Variables|Default|Setactive true)
        (Timeline|Timeline_2 Play)))))

(event EventTick
  (params (DeltaSeconds :type Float%20%28single-precision%29))
  (if (Variables|Default|Getcan%20use)
    (bind _output_get (Variables|Default|Settimer (- (stale _output_get) DeltaSeconds)))
    (if (< _output_get 0.0)
      (Variables|Default|Setcan%20use true)
      (Variables|Default|Settimer (Variables|Default|Getcooldown)))))

(fn ConstructionScript)