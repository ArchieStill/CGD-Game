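; Boss trap door puzzle object that opens when the third-person character steps on it.
; A box overlap filtered to the player's capsule component sets both cube meshes to ignore all collision channels.
; One tick later it snaps two arrow components to opposite fixed world rotations, with no animation or closing logic.
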(event OnComponentBeginOverlap(Box)
  (params (OverlappedComponent :type Primitive%20Component%20Object%20Reference) (OtherActor :type Actor%20Object%20Reference) (OtherComp :type Primitive%20Component%20Object%20Reference) (OtherBodyIndex :type Integer) (bFromSweep :type Boolean) (SweepResult :type Hit%20Result%20Structure%20%28by%20ref%29))
  ;[1 1 1] Opens the trap door when stepped on
  (bind _asbp_third_person_character (Utilities|Casting|CastToBP_ThirdPersonCharacter OtherActor))
  (if (== (Variables|/Script/Engine.Character|GetCapsuleComponent _asbp_third_person_character) OtherComp)
    (Collision|SetCollisionResponsetoAllChannels (Variables|Default|GetCube1) "ECR_Ignore")
    (Collision|SetCollisionResponsetoAllChannels (Variables|Default|GetCube) "ECR_Ignore")
    (Utilities|FlowControl|DelayUntilNextTick)
    (Transformation|SetWorldRotation (Variables|Default|GetArrow1) "-90.000000,0.000000,0.000000" false false)
    (Transformation|SetWorldRotation (Variables|Default|GetArrow) "90.000000,0.000000,0.000000" false false)))

(event EventBeginPlay)

(event Collision|EventActorBeginOverlap
  (params (OtherActor :type Actor%20Object%20Reference)))

(event EventTick
  (params (DeltaSeconds :type Float%20%28single-precision%29)))

(fn ConstructionScript)