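; BP_BlueCrystalBumper is a blue puzzle platform that moves vertically when activated and returns when deactivated.
; An Active flag guards a timeline, played or reversed, that offsets Z from the height stored at BeginPlay.
; When the third-person character leaves the Box, its upward velocity is capped.
; Show, Hide and PartiallyHide events switch the Platform's visibility and translucent blue materials.
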(event OnComponentEndOverlap(Box)
  (params (OverlappedComponent :type Primitive%20Component%20Object%20Reference) (OtherActor :type Actor%20Object%20Reference) (OtherComp :type Primitive%20Component%20Object%20Reference) (OtherBodyIndex :type Integer))
  (bind _asbp_third_person_character (Utilities|Casting|CastToBP_ThirdPersonCharacter OtherActor))
  (if (> (.Z (Math|Vector|BreakVector (Variables|/Script/Engine.MovementComponent|GetVelocity (Variables|/Script/Engine.Character|GetCharacterMovement _asbp_third_person_character)))) 1.5e+03)
    (Variables|/Script/Engine.MovementComponent|SetVelocity (Variables|/Script/Engine.Character|GetCharacterMovement _asbp_third_person_character) (Math|Vector|MakeVector (.X (Math|Vector|BreakVector (Variables|/Script/Engine.MovementComponent|GetVelocity (Variables|/Script/Engine.Character|GetCharacterMovement _asbp_third_person_character)))) (.Y (Math|Vector|BreakVector (Variables|/Script/Engine.MovementComponent|GetVelocity (Variables|/Script/Engine.Character|GetCharacterMovement _asbp_third_person_character)))) 1.5e+03))))

(event EventBeginPlay
  ;[1 1 1] Sets doors initail height
  (Variables|Default|Setstart%20height (.Z (Math|Vector|BreakVector (Transformation|GetActorLocation)))))

(event EventShow
  (bind _platform (Variables|Default|Getplatform))
  (Rendering|SetVisibility _platform true false)
  (Rendering|Material|SetMaterial _platform 0 "/Game/Materials/M_TranslucentBlue.M_TranslucentBlue"))

(event EventHide
  (Rendering|SetVisibility (Variables|Default|Getplatform) false false))

(event EventPartiallyHide
  (bind _platform (Variables|Default|Getplatform))
  (Rendering|SetVisibility _platform true false)
  (Rendering|Material|SetMaterial _platform 0 "/Game/Materials/MI_Blue_Transparent_2.MI_Blue_Transparent_2"))

(event EventActivate
  (bind _returnvalue (Transformation|GetActorLocation))
  (bind (_x _y) (Math|Vector|BreakVector _returnvalue))
  ;[1 1 1] Opens the door
  (if (not (Variables|Default|Getactive))
    (Variables|Default|Setactive true)
    ;[1 1 1] Handles the door movements
    (bind _height (Timeline|Timeline Play)
      (:Update
        (Transformation|SetActorLocation (Math|Vector|MakeVector _x _y (+ (* (Variables|Default|GetMax%20Move%20Distance) _height) (Variables|Default|Getstart%20height))) false false)))))

(event EventDeactivate
  (bind _returnvalue (Transformation|GetActorLocation))
  (bind (_x _y) (Math|Vector|BreakVector _returnvalue))
  ;[1 1 1] Closes the door
  (if (Variables|Default|Getactive)
    (Variables|Default|Setactive false)
    ;[1 1 1] Handles the door movements
    (bind _height (Timeline|Timeline Reverse)
      (:Update
        (Transformation|SetActorLocation (Math|Vector|MakeVector _x _y (+ (* (Variables|Default|GetMax%20Move%20Distance) _height) (Variables|Default|Getstart%20height))) false false)))))

(fn ConstructionScript)