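; Puzzle button that, when hit, temporarily activates its linked objects through BPI_Activateable.
; A hit ignored while active otherwise starts FMOD cog audio and a Timeline that moves the button top's Z from its starting height.
; Tick counts down the active time, then deactivates the linked objects and reverses the Timeline to return the button.
; An older offset-based Timeline remains unconnected.
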(event Custom|Hit%20Event
  (params (Damage :type Float%20%28double-precision%29))
  (bind _button_round_top (Variables|Default|GetButton_Round_Top))
  (bind _returnvalue (Transformation|GetWorldLocation _button_round_top))
  (bind (_x _y) (Math|Vector|BreakVector _returnvalue))
  ;[1 1 1] Activates "object to activate" if inactive
  (if (not (Variables|Default|Getactive))
    (Class|FMODAudioComponent|Play (Variables|Default|GetFMODCogs))
    (for _array_element (Variables|Default|Getobjects%20to%20activate)
      (bind _asbpi_activateable (Utilities|Casting|CastToBPI_Activateable _array_element)
        (:then
          (Default|Activate _asbpi_activateable))
        (:CastFailed
          (Development|PrintString "cast failed"))))
    (Variables|Default|Setactive true)
    (Variables|Default|Setactive%20timer (Variables|Default|Getactive%20time))
    ;[1 1 1] Pushes the button down/up
    (bind _height (Timeline|Timeline Play)
      (:Update
        (Transformation|SetWorldLocation (Variables|Default|GetButton_Round_Top) (Math|Vector|MakeVector _x _y (+ (* (Variables|Default|Getmove%20amount) _height) (Variables|Default|Getstart%20height))) false false))
      (:Finished
        (if (not (== _height 0.0))
          (Class|FMODAudioComponent|Stop (Variables|Default|GetFMODCogs)))))))

(event EventBeginPlay
  ;[1 1 1] Sets Initial height
  (Variables|Default|Setstart%20height (.Z (Math|Vector|BreakVector (Transformation|GetWorldLocation (Variables|Default|GetButton_Round_Top))))))

(event EventTick
  (params (DeltaSeconds :type Float%20%28single-precision%29))
  (bind _button_round_top (Variables|Default|GetButton_Round_Top))
  (bind _returnvalue (Transformation|GetWorldLocation _button_round_top))
  (bind (_x _y) (Math|Vector|BreakVector _returnvalue))
  ;[1 1 1] Deactivates "object to activate" after a set time
  (if (Variables|Default|Getactive)
    (bind _output_get (Variables|Default|Setactive%20timer (- (Variables|Default|Getactive%20timer) DeltaSeconds)))
    (if (< _output_get 0.0)
      (Variables|Default|Setactive false)
      (for _array_element (Variables|Default|Getobjects%20to%20activate)
        (bind _asbpi_activateable (Utilities|Casting|CastToBPI_Activateable _array_element))
        (Default|Deactivate _asbpi_activateable))
      ;[1 1 1] Pushes the button down/up
      (bind _height (Timeline|Timeline Reverse)
        (:Update
          (Transformation|SetWorldLocation (Variables|Default|GetButton_Round_Top) (Math|Vector|MakeVector _x _y (+ (* (Variables|Default|Getmove%20amount) _height) (Variables|Default|Getstart%20height))) false false))
        (:Finished
          (if (not (== _height 0.0))
            (Class|FMODAudioComponent|Stop (Variables|Default|GetFMODCogs))))))))

(fn ConstructionScript)

(fn Hit
  (params (Damage :type Float%20%28double-precision%29) (Hitter :type Actor%20Object%20Reference))
  (CallFunction|HitEvent 0.0)
  (return))