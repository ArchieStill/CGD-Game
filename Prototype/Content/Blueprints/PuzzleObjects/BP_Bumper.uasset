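; BP_Bumper is a puzzle door or platform that moves vertically from its start height by MaxMoveDistance when activated and returns when deactivated.
; Activate and Deactivate play or reverse one of two timelines, chosen by Slow, with FMOD cog sounds.
; They toggle the Killbox active for downward travel, and its overlap triggers the character's death sequence.
; Leaving the Box clamps the character's upward velocity to jump speed.
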(event OnComponentEndOverlap(Box)
  (params (OverlappedComponent :type Primitive%20Component%20Object%20Reference) (OtherActor :type Actor%20Object%20Reference) (OtherComp :type Primitive%20Component%20Object%20Reference) (OtherBodyIndex :type Integer))
  (bind _asbp_third_person_character (Utilities|Casting|CastToBP_ThirdPersonCharacter OtherActor))
  (if (> (.Z (Math|Vector|BreakVector (Variables|/Script/Engine.MovementComponent|GetVelocity (Variables|/Script/Engine.Character|GetCharacterMovement _asbp_third_person_character)))) (Variables|/Script/Engine.CharacterMovementComponent|GetJumpZVelocity (Variables|/Script/Engine.Character|GetCharacterMovement _asbp_third_person_character)))
    (Variables|/Script/Engine.MovementComponent|SetVelocity (Variables|/Script/Engine.Character|GetCharacterMovement _asbp_third_person_character) (Math|Vector|MakeVector (.X (Math|Vector|BreakVector (Variables|/Script/Engine.MovementComponent|GetVelocity (Variables|/Script/Engine.Character|GetCharacterMovement _asbp_third_person_character)))) (.Y (Math|Vector|BreakVector (Variables|/Script/Engine.MovementComponent|GetVelocity (Variables|/Script/Engine.Character|GetCharacterMovement _asbp_third_person_character)))) (Variables|/Script/Engine.CharacterMovementComponent|GetJumpZVelocity (Variables|/Script/Engine.Character|GetCharacterMovement _asbp_third_person_character))))))

(event OnComponentBeginOverlap(killbox)
  (params (OverlappedComponent :type Primitive%20Component%20Object%20Reference) (OtherActor :type Actor%20Object%20Reference) (OtherComp :type Primitive%20Component%20Object%20Reference) (OtherBodyIndex :type Integer) (bFromSweep :type Boolean) (SweepResult :type Hit%20Result%20Structure%20%28by%20ref%29))
  (bind _asbp_third_person_character (Utilities|Casting|CastToBP_ThirdPersonCharacter OtherActor))
  (if (== OtherComp (Variables|/Script/Engine.Character|GetCapsuleComponent _asbp_third_person_character))
    (Default|ExecuteDeathSequence (Actor|GetComponentbyClass _asbp_third_person_character "/Game/Blueprints/DeathSystem/BPC_DeathComponent.BPC_DeathComponent_C"))))

(event Custom|PlayCogs
  (Class|FMODAudioComponent|Play (Variables|Default|GetFMODCogs))
  (Utilities|FlowControl|Delay 3.0)
  (Class|FMODAudioComponent|Stop (Variables|Default|GetFMODCogs)))

(event EventBeginPlay
  ;[1 1 1] Sets doors initail height
  (Variables|Default|Setstart%20height (.Z (Math|Vector|BreakVector (Transformation|GetActorLocation)))))

(event EventActivate
  (bind _returnvalue (Transformation|GetActorLocation))
  (bind _returnvalue_2 (Transformation|GetActorLocation))
  (bind _killbox (Variables|Default|Getkillbox))
  (bind (_x _y) (Math|Vector|BreakVector _returnvalue))
  (bind (_x_2 _y_2) (Math|Vector|BreakVector _returnvalue_2))
  ;[1 1 1] Opens the door
  (if (not (Variables|Default|Getactive))
    (CallFunction|PlayCogs)
    (if (> (Variables|Default|GetMax%20Move%20Distance) 0.0)
      (Components|Activation|SetActive _killbox false false)
      (else
        (Components|Activation|SetActive _killbox true false)))
    (Variables|Default|Setactive true)
    (if (Variables|Default|Getslow)
      (bind _height (Timeline|Timeline_0 Play)
        (:Update
          (Transformation|SetActorLocation (Math|Vector|MakeVector _x_2 _y_2 (+ (* (Variables|Default|GetMax%20Move%20Distance) _height) (Variables|Default|Getstart%20height))) false false))
        (:Finished
          (Class|FMODAudioComponent|Stop (Variables|Default|GetFMODCogs))))
      (else
        ;[1 1 1] Handles the door movements
        (bind _height_2 (Timeline|Timeline Play)
          (:Update
            (Transformation|SetActorLocation (Math|Vector|MakeVector _x _y (+ (* (Variables|Default|GetMax%20Move%20Distance) _height_2) (Variables|Default|Getstart%20height))) false false)))))))

(event EventDeactivate
  (bind _returnvalue (Transformation|GetActorLocation))
  (bind _returnvalue_2 (Transformation|GetActorLocation))
  (bind _killbox (Variables|Default|Getkillbox))
  (bind (_x _y) (Math|Vector|BreakVector _returnvalue))
  (bind (_x_2 _y_2) (Math|Vector|BreakVector _returnvalue_2))
  ;[1 1 1] Closes the door
  (if (Variables|Default|Getactive)
    (CallFunction|PlayCogs)
    (if (> (Variables|Default|GetMax%20Move%20Distance) 0.0)
      (Components|Activation|SetActive _killbox true false)
      (else
        (Components|Activation|SetActive _killbox false false)))
    (Variables|Default|Setactive false)
    (if (Variables|Default|Getslow)
      (bind _height (Timeline|Timeline_0 Reverse)
        (:Update
          (Transformation|SetActorLocation (Math|Vector|MakeVector _x_2 _y_2 (+ (* (Variables|Default|GetMax%20Move%20Distance) _height) (Variables|Default|Getstart%20height))) false false))
        (:Finished
          (Class|FMODAudioComponent|Stop (Variables|Default|GetFMODCogs))))
      (else
        ;[1 1 1] Handles the door movements
        (bind _height_2 (Timeline|Timeline Reverse)
          (:Update
            (Transformation|SetActorLocation (Math|Vector|MakeVector _x _y (+ (* (Variables|Default|GetMax%20Move%20Distance) _height_2) (Variables|Default|Getstart%20height))) false false)))))))

(fn ConstructionScript)