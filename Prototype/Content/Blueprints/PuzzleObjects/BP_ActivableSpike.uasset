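; Activatable floor spike trap that kills the player character or breaks blockades caught by it.
; Activate plays audio and Niagara effects, then after a short delay opens a brief CanSpike damage window.
; Tick drives a timeline that moves the spikes vertically, restarting it while idle and clearing activation when it finishes.
; Hitbox begin-overlaps trigger the death component or blockade break only within that window, plus a one-time smash sound on any overlap.
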(event OnComponentBeginOverlap(HitBox)
  (params (OverlappedComponent :type Primitive%20Component%20Object%20Reference) (OtherActor :type Actor%20Object%20Reference) (OtherComp :type Primitive%20Component%20Object%20Reference) (OtherBodyIndex :type Integer) (bFromSweep :type Boolean) (SweepResult :type Hit%20Result%20Structure%20%28by%20ref%29))
  ;[1 1 1] Player/Blockade Overlap
  (CallFunction|HitObject OtherActor OtherComp)
  (if (not (Variables|Default|GetHasPlayed))
    (Class|FMODAudioComponent|Play (Variables|Default|GetFMODBoulderSmash))
    (Variables|Default|SetHasPlayed true)))

(event EventActivate
  ;[1 1 1] Floor Trap Activate
  (if (not (Variables|Default|GetFloorTrapActivated))
    (Variables|Default|SetFloorTrapActivated true)
    ;[1 1 1] Play Audio
    (Class|FMODAudioComponent|Play (Variables|Default|GetFMODSpike))
    ;[1 1 1] Particle System
    (AddComponent|AddNiagaraComponent false (Math|Transform|MakeTransform "0, 0, 0" "0, 0, 0" "0.100000,0.100000,0.100000"))
    ;[1 1 1] Delay
    (Utilities|FlowControl|Delay 0.5)
    (Variables|Default|Setcan%20spike true)
    (Utilities|FlowControl|Delay 0.1)
    (Variables|Default|Setcan%20spike false)
    (Class|FMODAudioComponent|Stop (Variables|Default|GetFMODSpike))))

(event EventTick
  (params (DeltaSeconds :type Float%20%28single-precision%29))
  ;[1 1 1] Spear Movement
  (if (Variables|Default|GetFloorTrapActivated)
    (bind _movement (Timeline|Spear_Movement Play)
      (:Update
        (Transformation|SetRelativeLocation (Variables|Default|GetSpikes) (Math|Vector|MakeVector 0.0 0.0 _movement) false false))
      (:Finished
        (Variables|Default|SetFloorTrapActivated false)))
    (else
      (Timeline|Spear_Movement PlayFromStart))))

(fn ConstructionScript
  (|CallParentFunction))

(fn HitObject
  (params (hit_actor :type Actor%20Object%20Reference) (hit_component :type Primitive%20Component%20Object%20Reference))
  (if (Variables|Default|Getcan%20spike)
    (bind _asbp_third_person_character (Utilities|Casting|CastToBP_ThirdPersonCharacter hit_actor)
      (:then
        (if (== hit_component (Variables|/Script/Engine.Character|GetCapsuleComponent _asbp_third_person_character))
          (Default|ExecuteDeathSequence (Actor|GetComponentbyClass _asbp_third_person_character "/Game/Blueprints/DeathSystem/BPC_DeathComponent.BPC_DeathComponent_C"))))
      (:CastFailed
        (bind _asbp_blockade (Utilities|Casting|CastToBP_Blockade hit_actor))
        (Default|Break _asbp_blockade)))))