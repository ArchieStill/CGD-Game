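; BP_CodeLight is a colored indicator light for a code button puzzle that switches between unlit and lit looks.
; A LightCol enum of red, blue, green or yellow picks the material pair applied to LightMesh.
; Activate sets the lit material, while BeginPlay and Deactivate share one switch that sets the unlit material.
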(event EventBeginPlay
  (bind _lightmesh (Variables|Default|GetLightMesh))
  (switch Utilities|FlowControl|Switch|SwitchonLightColoursEnum (Variables|Default|GetLightCol)
    (:NewEnumerator0
      (Rendering|Material|SetMaterial _lightmesh 0 "/Game/Models/CodeButtons/CB_Red.CB_Red"))
    (:NewEnumerator1
      (Rendering|Material|SetMaterial _lightmesh 0 "/Game/Models/CodeButtons/CB_Blue.CB_Blue"))
    (:NewEnumerator2
      (Rendering|Material|SetMaterial _lightmesh 0 "/Game/Models/CodeButtons/CB_Green.CB_Green"))
    (:NewEnumerator3
      (Rendering|Material|SetMaterial _lightmesh 0 "/Game/Models/CodeButtons/CB_Yellow.CB_Yellow"))))

(event EventActivate
  (bind _lightmesh (Variables|Default|GetLightMesh))
  (switch Utilities|FlowControl|Switch|SwitchonLightColoursEnum (Variables|Default|GetLightCol)
    (:NewEnumerator0
      (Rendering|Material|SetMaterial _lightmesh 0 "/Game/Models/CodeButtons/CB_RedOn.CB_RedOn"))
    (:NewEnumerator1
      (Rendering|Material|SetMaterial _lightmesh 0 "/Game/Models/CodeButtons/CB_BlueOn.CB_BlueOn"))
    (:NewEnumerator2
      (Rendering|Material|SetMaterial _lightmesh 0 "/Game/Models/CodeButtons/CB_GreenOn.CB_GreenOn"))
    (:NewEnumerator3
      (Rendering|Material|SetMaterial _lightmesh 0 "/Game/Models/CodeButtons/CB_YellowOn.CB_YellowOn"))))

(event EventDeactivate
  (bind _lightmesh (Variables|Default|GetLightMesh))
  (switch Utilities|FlowControl|Switch|SwitchonLightColoursEnum (Variables|Default|GetLightCol)
    (:NewEnumerator0
      (Rendering|Material|SetMaterial _lightmesh 0 "/Game/Models/CodeButtons/CB_Red.CB_Red"))
    (:NewEnumerator1
      (Rendering|Material|SetMaterial _lightmesh 0 "/Game/Models/CodeButtons/CB_Blue.CB_Blue"))
    (:NewEnumerator2
      (Rendering|Material|SetMaterial _lightmesh 0 "/Game/Models/CodeButtons/CB_Green.CB_Green"))
    (:NewEnumerator3
      (Rendering|Material|SetMaterial _lightmesh 0 "/Game/Models/CodeButtons/CB_Yellow.CB_Yellow"))))

(fn ConstructionScript)