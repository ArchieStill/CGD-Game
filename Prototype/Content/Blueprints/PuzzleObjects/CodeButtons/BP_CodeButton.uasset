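; BP_CodeButton is a colored puzzle button that moves when hit and resets after a set time.
; BeginPlay records the starting height and picks the red, blue, green or yellow mesh.
; A hit starts cog audio, a countdown and a Timeline that offsets the mesh's Z.
; When Tick's countdown expires, it calls Deactivate on linked objects through BPI_Activateable and reverses the Timeline; this file never activates them.
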(event EventTick
  (params (DeltaSeconds :type Float%20%28single-precision%29))
  (bind _buttonmain (Variables|Default|GetButtonMain))
  (bind _returnvalue (Transformation|GetWorldLocation _buttonmain))
  (bind (_x _y) (Math|Vector|BreakVector _returnvalue))
  ;[1 1 1] Deactivates "object to activate" after a set time
  (if (Variables|Default|Getactive)
    (bind _output_get (Variables|Default|SetActiveTimer (- (Variables|Default|GetActiveTimer) DeltaSeconds)))
    (if (< _output_get 0.0)
      (Variables|Default|Setactive false)
      (for _array_element (Variables|Default|GetObjectsToActivate)
        (bind _asbpi_activateable (Utilities|Casting|CastToBPI_Activateable _array_element))
        (Default|Deactivate _asbpi_activateable))
      (bind _height (Timeline|Timeline Reverse)
        (:Update
          (Transformation|SetWorldLocation (Variables|Default|GetButtonMain) (Math|Vector|MakeVector _x _y (+ (* (Variables|Default|GetMoveAmount) _height) (Variables|Default|GetStartHeight))) false false))
        (:Finished
          (if (not (== _height 0.0))
            (Class|FMODAudioComponent|Stop (Variables|Default|GetFMODCogs))))))))

(event EventHit
  (params (Damage :type Float%20%28double-precision%29) (Hitter :type Actor%20Object%20Reference))
  (bind _buttonmain (Variables|Default|GetButtonMain))
  (bind _returnvalue (Transformation|GetWorldLocation _buttonmain))
  (bind (_x _y) (Math|Vector|BreakVector _returnvalue))
  ;[1 1 1] Activates button when hit
  (if (not (Variables|Default|Getactive))
    (Class|FMODAudioComponent|Play (Variables|Default|GetFMODCogs))
    (Variables|Default|Setactive true)
    (Variables|Default|SetActiveTimer (Variables|Default|GetActiveTime))
    (bind _height (Timeline|Timeline Play)
      (:Update
        (Transformation|SetWorldLocation (Variables|Default|GetButtonMain) (Math|Vector|MakeVector _x _y (+ (* (Variables|Default|GetMoveAmount) _height) (Variables|Default|GetStartHeight))) false false))
      (:Finished
        (if (not (== _height 0.0))
          (Class|FMODAudioComponent|Stop (Variables|Default|GetFMODCogs)))))))

(event EventBeginPlay
  (bind _buttonmain (Variables|Default|GetButtonMain))
  (Variables|Default|SetStartHeight (.Z (Math|Vector|BreakVector (Transformation|GetWorldLocation (Variables|Default|GetButtonMain)))))
  (switch Utilities|FlowControl|Switch|SwitchonLightColoursEnum (Variables|Default|GetButtonCol)
    (:NewEnumerator0
      (Components|StaticMesh|SetStaticMesh _buttonmain "/Game/Models/CodeButtons/ButtonRed.ButtonRed"))
    (:NewEnumerator1
      (Components|StaticMesh|SetStaticMesh _buttonmain "/Game/Models/CodeButtons/ButtonBlue.ButtonBlue"))
    (:NewEnumerator2
      (Components|StaticMesh|SetStaticMesh _buttonmain "/Game/Models/CodeButtons/ButtonGreen.ButtonGreen"))
    (:NewEnumerator3
      (Components|StaticMesh|SetStaticMesh _buttonmain "/Game/Models/CodeButtons/ButtonYellow.ButtonYellow"))))

(fn ConstructionScript)