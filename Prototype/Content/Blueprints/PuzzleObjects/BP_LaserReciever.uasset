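; BP_LaserReciever is a puzzle object that keeps a linked object activated while a laser hits it.
; LaserHit resets a frame counter and, if inactive, activates ObjectToActivate through the BPI_Activateable interface.
; Tick increments the counter while active and deactivates the object once LifetimeFrames pass without a hit, so laser input must be continually refreshed.
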(event EventTick
  (params (DeltaSeconds :type Float%20%28single-precision%29))
  (if (Variables|Default|Getactive)
    ;[1 1 1] If receiver goes a frame without recieving input, deactivate
    (bind _output_get (Variables|Default|Setlifetime%20frames%20counter (+ (Variables|Default|Getlifetime%20frames%20counter) 1)))
    (if (>= _output_get (Variables|Default|Getlifetime%20frames))
      (Variables|Default|Setactive false)
      (bind _asbpi_activateable (Utilities|Casting|CastToBPI_Activateable (Variables|Default|Getobject%20to%20activate)))
      (Default|Deactivate _asbpi_activateable))))

(event EventLaserHit
  (params (Location :type Vector :default "0, 0, 0") (Type :type Laser%20Type%20Structure))
  ;[1 1 1] Keeps the "object to activate" activated while still receiving laser input
  (if (Variables|Default|GetActive)
    _
    (else
      (bind _asbpi_activateable (Utilities|Casting|CastToBPI_Activateable (Variables|Default|Getobject%20to%20activate))
        (:then
          (Default|Activate _asbpi_activateable))
        (:CastFailed
          (Development|PrintString "cast failed")))
      (Variables|Default|Setactive true)))
  (Variables|Default|Setlifetime%20frames%20counter 0))

(fn ConstructionScript)