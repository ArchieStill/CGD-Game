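; Puzzle laser beam that kills the player character on contact and triggers laser-interactable objects.
; Each tick while active, it sphere-traces along its arrow and stretches the mesh to the hit, passing hit location and laser type to BPI_LaserInteractable actors.
; Non-self-sustaining lasers switch off after a set number of frames unless SetActive refreshes them.
; Laser type defaults from a data table and sets the beam material.
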(event EventBeginPlay
  ;[1 1 1] Sets the laser type to default so theres no error if a type isn't set
  (bind _returnvalue (Utilities|GetDataTableRow "/Game/LaserTypesTable.LaserTypesTable" "Default")
    (:then
      (CallFunction|SetLaserType _returnvalue))))

(event EventTick
  (params (DeltaSeconds :type Float%20%28single-precision%29))
  (bind _returnvalue (Transformation|GetActorLocation))
  (bind _staticmesh (Variables|Default|GetStaticMesh))
  (bind _staticmesh_2 (Variables|Default|GetStaticMesh))
  (bind _returnvalue_2 (Transformation|GetWorldScale _staticmesh))
  (bind _returnvalue_3 (Transformation|GetWorldScale _staticmesh_2))
  (bind (_x _y) (Math|Vector|BreakVector _returnvalue_2))
  (bind (_x_2 _y_2) (Math|Vector|BreakVector _returnvalue_3))
  (CallFunction|CheckLifetime)
  ;[1 1 1] Ray traces from the lasers position to a very far away distance
  (if (Variables|Default|GetActive)
    (bind (_outhit _returnvalue_4) (Collision|SphereTraceByChannel _returnvalue (+ _returnvalue (* (Math|Vector|GetForwardVector (Variables|Default|GetArrow)) 1e+05)) 5e+01 "TraceTypeQuery3" false (Variables|Default|Getignore%20actors) "None"))
    (bind _output_get (Variables|Default|SetBlockingHit _returnvalue_4))
    (if _output_get
      ;[1 1 1] Scales the laser to reach the blocking hit
      (Transformation|SetWorldScale3D _staticmesh_2 (Math|Vector|MakeVector _x_2 _y_2 (/ (.Distance (Collision|BreakHitResult _outhit)) 1e+02)))
      (bind _asbp_third_person_character (Utilities|Casting|CastToBP_ThirdPersonCharacter (.HitActor (Collision|BreakHitResult _outhit)))
        (:then
          (Default|ExecuteDeathSequence (Variables|/Game/ThirdPerson/Blueprints/BP_ThirdPersonCharacter.BP_ThirdPersonCharacter_C|GetBPC_Death%20Component _asbp_third_person_character)))
        (:CastFailed
          ;[1 1 1] Calls laser hit if the object the laser is touching has BPI_LaserInteractable
          (bind _asbpi_laser_interactable (Utilities|Casting|CastToBPI_LaserInteractable (.HitActor (Collision|BreakHitResult _outhit))))
          (Default|LaserHit _asbpi_laser_interactable (.Location (Collision|BreakHitResult _outhit)) (Variables|Default|GetLaserType))))
      (else
        ;[1 1 1] Sets the laser to maximum scale if it hits nothing
        (Transformation|SetWorldScale3D _staticmesh (Math|Vector|MakeVector _x _y 1e+03))))))

(fn ConstructionScript)

(fn SetActive
  (params (New%20Active :type Boolean))
  ;[1 1 1] Activates/Deactivates the laser
  (bind _output_get (Variables|Default|SetActive New%20Active))
  (if _output_get
    (Variables|Default|SetLifetimeFramesCounter 0))
  (Development|SetHiddeninGame (Variables|Default|GetStaticMesh) (not _output_get) false))

(fn CheckLifetime
  ;[1 1 1] Self sustaining lasers can stay active without input from another laser / source
  (if (not (Variables|Default|GetSelfSustaining))
    (if (Variables|Default|GetActive)
      ;[1 1 1] If laser goes a frame without recieving input, deactivate
      (bind _output_get (Variables|Default|SetLifetimeFramesCounter (+ (Variables|Default|GetLifetimeFramesCounter) 1)))
      (if (>= _output_get (Variables|Default|GetLifetimeFrames))
        (CallFunction|SetActive false)))))

(fn SetLaserType
  (params (Type :type Laser%20Type%20Structure))
  (bind _output_get (Variables|Default|SetLaserType Type))
  (Rendering|Material|SetMaterial (Variables|Default|GetStaticMesh) 0 (.Mat (Utilities|Struct|BreakLaserType _output_get))))

(fn AddActortoIgnore
  (params (actor :type Actor%20Object%20Reference))
  (Utilities|Array|Add (Variables|Default|Getignore%20actors) actor))