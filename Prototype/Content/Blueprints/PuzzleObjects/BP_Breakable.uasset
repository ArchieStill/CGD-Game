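; BP_Breakable is a puzzle object that breaks when hit, with an optional hit prompt hidden at BeginPlay unless InputPrompt is set.
; Hit breaks it immediately unless it is Reinforced, in which case the Hitter must report being reinforced through BPI_Hitter.
; Breaking scales the Cube to zero and hides the prompt instead of destroying the actor, and Damage is unused.
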(event EventBeginPlay
  (if (not (Variables|Default|Getinput%20prompt))
    (Rendering|SetVisibility (Variables|Default|GetHitPrompt) false false)))

(fn ConstructionScript)

(fn Hit
  (params (Damage :type Float%20%28double-precision%29) (Hitter :type Actor%20Object%20Reference))
  (if (Variables|Default|GetReinforced)
    (bind _asbpi_hitter (Utilities|Casting|CastToBPI_Hitter Hitter))
    (bind _value (Default|GetReinforced _asbpi_hitter))
    (if _value
      (Transformation|SetWorldScale3D (Variables|Default|GetCube) "0, 0, 0" :!label _label)
      (Rendering|SetVisibility (Variables|Default|GetHitPrompt) false false))
    (else
      (goto _label))))