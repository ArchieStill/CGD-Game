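; Orange crystal platform that switches between a solid-looking shown state and a transparent hidden state.
; Show applies the orange crystal material to the Platform component and sets its collision to query-only.
; Hide swaps in the transparent orange material instance and disables collision.
; The graph contains no movement logic and no callers for either event.
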(event EventBeginPlay
  (|CallParentFunction) ; This node is disabled and will not be called.\nDrag off pins to build functionality.
)

(event Collision|EventActorBeginOverlap
  (params (OtherActor :type Actor%20Object%20Reference))
  (|CallParentFunction OtherActor) ; This node is disabled and will not be called.\nDrag off pins to build functionality.
)

(event EventTick
  (params (DeltaSeconds :type Float%20%28single-precision%29))
  (|CallParentFunction DeltaSeconds) ; This node is disabled and will not be called.\nDrag off pins to build functionality.
)

(event EventShow
  (params (crystal_id :type Integer))
  (bind _platform (Variables|Default|Getplatform))
  (Rendering|Material|SetMaterial _platform 0 "/Game/Models/Crystal/M_CrystalOrange.M_CrystalOrange")
  (Collision|SetCollisionEnabled _platform "QueryOnly"))

(event EventHide
  (params (crystal_id :type Integer))
  (bind _platform (Variables|Default|Getplatform))
  (Rendering|Material|SetMaterial _platform 0 "/Game/Materials/MI_Orange_Transparent.MI_Orange_Transparent")
  (Collision|SetCollisionEnabled _platform "NoCollision"))

(fn ConstructionScript
  (|CallParentFunction))