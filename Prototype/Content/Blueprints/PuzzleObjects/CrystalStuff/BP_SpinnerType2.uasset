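; BP_SpinnerType2 is a crystal puzzle object whose blue cylinder segment switches between shown, partially hidden and hidden through three events.
; Show and PartiallyHide make the segment visible with different blue materials and play the FMOD activate or deactivate sound.
; IsLit and IsFlashing keep those sounds from replaying until Hide turns the segment invisible and clears both flags.
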(event EventBeginPlay
  (|CallParentFunction) ; This node is disabled and will not be called.\nDrag off pins to build functionality.
)

(event Collision|EventActorBeginOverlap
  (params (OtherActor :type Actor%20Object%20Reference))
  (|CallParentFunction OtherActor) ; This node is disabled and will not be called.\nDrag off pins to build functionality.
)

(event EventHide
  (Rendering|SetVisibility (Variables|Default|Getblue_cylinder_removed_segment) false false)
  (Variables|Default|SetIsFlashing false)
  (Variables|Default|SetIsLit false))

(event EventShow
  (bind _blue_cylinder_removed_segment (Variables|Default|Getblue_cylinder_removed_segment))
  (Rendering|SetVisibility _blue_cylinder_removed_segment true false)
  (Rendering|Material|SetMaterial _blue_cylinder_removed_segment 0 "/Game/Materials/M_TranslucentBlue.M_TranslucentBlue")
  (if (not (Variables|Default|GetIsLit))
    (Class|FMODAudioComponent|Play (Variables|Default|GetFMODActivateBlueCrystal))
    (Variables|Default|SetIsLit true)))

(event EventTick
  (params (DeltaSeconds :type Float%20%28single-precision%29))
  (|CallParentFunction DeltaSeconds) ; This node is disabled and will not be called.\nDrag off pins to build functionality.
)

(event EventPartiallyHide
  (bind _blue_cylinder_removed_segment (Variables|Default|Getblue_cylinder_removed_segment))
  (Rendering|SetVisibility _blue_cylinder_removed_segment true false)
  (Rendering|Material|SetMaterial _blue_cylinder_removed_segment 0 "/Game/Materials/MI_Blue_Transparent_2.MI_Blue_Transparent_2")
  (if (not (Variables|Default|GetIsFlashing))
    (Class|FMODAudioComponent|Play (Variables|Default|GetFMODDeactivatecrystal))
    (Variables|Default|SetIsFlashing true)))

(fn ConstructionScript
  (|CallParentFunction))