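; BP_RisingWater is a rising water hazard that kills the player on contact and extinguishes torches it reaches.
; Once activated, Tick moves it up at a steady rate, or at a sudden-rise rate until it reaches a target height, which becomes the new reset point.
; Player overlap runs the death component's sequence and resets the water, jumping to the target height if mid-surge.
; Ending a surge or resetting clears the FMOD "Explosion" parameter.
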(event OnComponentBeginOverlap(hitbox)
  (params (OverlappedComponent :type Primitive%20Component%20Object%20Reference) (OtherActor :type Actor%20Object%20Reference) (OtherComp :type Primitive%20Component%20Object%20Reference) (OtherBodyIndex :type Integer) (bFromSweep :type Boolean) (SweepResult :type Hit%20Result%20Structure%20%28by%20ref%29))
  (if (Utilities|ClassIsChildOf (Utilities|GetClass OtherActor) "/Game/ThirdPerson/Blueprints/BP_ThirdPersonCharacter.BP_ThirdPersonCharacter_C")
    (Default|ExecuteDeathSequence (Actor|GetComponentbyClass OtherActor "/Game/Blueprints/DeathSystem/BPC_DeathComponent.BPC_DeathComponent_C"))
    (CallFunction|ResetWater)
    (elif (Components|ComponentHasTag OtherComp "WaterExtinguishPoint")
      (bind _asbp_room_torch (Utilities|Casting|CastToBP_RoomTorch OtherActor)
        (:then
          (Default|Extinguish _asbp_room_torch))
        (:CastFailed
          (bind _asbp_big_torch (Utilities|Casting|CastToBP_BigTorch OtherActor))
          (Default|Extinguish _asbp_big_torch))))))

(event EventBeginPlay
  (Variables|Default|Setreset_position (Transformation|GetActorLocation)))

(event EventTick
  (params (DeltaSeconds :type Float%20%28single-precision%29))
  (bind _returnvalue (Transformation|GetActorLocation))
  (bind _sudden_rise_target_height (Variables|Default|Getsudden_rise_target_height))
  (if (Variables|Default|Getactive)
    (if (Variables|Default|Getsudden_rising)
      (Transformation|AddActorWorldOffset (Math|Vector|MakeVector 0.0 0.0 (* (Variables|Default|Getrise_rate_sudden) DeltaSeconds)))
      (Math|Float|CompareFloat (.z _returnvalue) _sudden_rise_target_height
        (:>
          (Transformation|SetActorLocation (Math|Vector|MakeVector (.x _returnvalue) (.y _returnvalue) _sudden_rise_target_height) false false))
        (:==
          _))
      (Variables|Default|Setsudden_rising false)
      (Variables|Default|Setreset_position (Transformation|GetActorLocation))
      (Class|FMODAudioComponent|SetParameter (Variables|Default|GetFMODRushingWater) "Explosion" 0.0)
      (else
        (Transformation|AddActorWorldOffset (Math|Vector|MakeVector 0.0 0.0 (* (Variables|Default|Getrise_rate) DeltaSeconds)))))))

(event EventActivate
  (Variables|Default|Setactive true))

(fn ConstructionScript)

(fn ResetWater
  (bind _returnvalue (Transformation|GetActorLocation))
  (Variables|Default|Setactive false)
  (if (Variables|Default|Getsudden_rising)
    (bind _output_get (Variables|Default|Setreset_position (Math|Vector|MakeVector (.x _returnvalue) (.y _returnvalue) (Variables|Default|Getsudden_rise_target_height)))))
  (Transformation|SetActorLocation _output_get false false)
  (Class|FMODAudioComponent|SetParameter (Variables|Default|GetFMODRushingWater) "Explosion" 0.0))

(fn SuddenRise
  (Variables|Default|Setactive true)
  (Variables|Default|Setsudden_rising true))

(fn StopRise)