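; Puzzle door that opens by destroying itself when the third-person character reaches it holding both the red and blue keys.
; On trigger overlap, it prints both key flags and reveals a group of four key components for each key held.
; With both keys held, it clears the character's keys and removes the door actor immediately.
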(event OnComponentBeginOverlap(trigger)
  (params (OverlappedComponent :type Primitive%20Component%20Object%20Reference) (OtherActor :type Actor%20Object%20Reference) (OtherComp :type Primitive%20Component%20Object%20Reference) (OtherBodyIndex :type Integer) (bFromSweep :type Boolean) (SweepResult :type Hit%20Result%20Structure%20%28by%20ref%29))
  (bind _asbp_third_person_character (Utilities|Casting|CastToBP_ThirdPersonCharacter OtherActor))
  (Development|PrintText (Utilities|Text|ToText(Boolean) (Variables|/Game/ThirdPerson/Blueprints/BP_ThirdPersonCharacter.BP_ThirdPersonCharacter_C|Gethas_red_key _asbp_third_person_character)))
  (Development|PrintText (Utilities|Text|ToText(Boolean) (Variables|/Game/ThirdPerson/Blueprints/BP_ThirdPersonCharacter.BP_ThirdPersonCharacter_C|Gethas_blue_key _asbp_third_person_character)))
  (if (Variables|/Game/ThirdPerson/Blueprints/BP_ThirdPersonCharacter.BP_ThirdPersonCharacter_C|Gethas_red_key _asbp_third_person_character)
    (Rendering|SetVisibility (Variables|Default|Getkey_004) true false))
  (if (Variables|/Game/ThirdPerson/Blueprints/BP_ThirdPersonCharacter.BP_ThirdPersonCharacter_C|Gethas_blue_key _asbp_third_person_character)
    (Rendering|SetVisibility (Variables|Default|Getkey_007) true false)
    (if (and (Variables|/Game/ThirdPerson/Blueprints/BP_ThirdPersonCharacter.BP_ThirdPersonCharacter_C|Gethas_red_key _asbp_third_person_character) (Variables|/Game/ThirdPerson/Blueprints/BP_ThirdPersonCharacter.BP_ThirdPersonCharacter_C|Gethas_blue_key _asbp_third_person_character))
      (Default|ClearKeys _asbp_third_person_character)
      (Actor|DestroyActor))))

(event EventBeginPlay)

(event Collision|EventActorBeginOverlap
  (params (OtherActor :type Actor%20Object%20Reference)))

(event EventTick
  (params (DeltaSeconds :type Float%20%28single-precision%29)))

(fn ConstructionScript)