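; A puzzle door that opens when the player character carries all four keys: red, blue, green and yellow.
; Overlapping the trigger reveals the door's key meshes for each color the character holds.
; With all four, it clears the character's keys and opens by hiding the door and keys and disabling collision.
; ResetDoor restores the closed state, though nothing in this graph calls it.
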(event OnComponentBeginOverlap(trigger)
  (params (OverlappedComponent :type Primitive%20Component%20Object%20Reference) (OtherActor :type Actor%20Object%20Reference) (OtherComp :type Primitive%20Component%20Object%20Reference) (OtherBodyIndex :type Integer) (bFromSweep :type Boolean) (SweepResult :type Hit%20Result%20Structure%20%28by%20ref%29))
  (bind _asbp_third_person_character (Utilities|Casting|CastToBP_ThirdPersonCharacter OtherActor))
  (if (Variables|/Game/ThirdPerson/Blueprints/BP_ThirdPersonCharacter.BP_ThirdPersonCharacter_C|GetHasRedKey _asbp_third_person_character)
    (Rendering|SetVisibility (Variables|Default|Getred_key_004) true false))
  (if (Variables|/Game/ThirdPerson/Blueprints/BP_ThirdPersonCharacter.BP_ThirdPersonCharacter_C|GetHasBlueKey _asbp_third_person_character)
    (Rendering|SetVisibility (Variables|Default|Getblue_key_003) true false))
  (if (Variables|/Game/ThirdPerson/Blueprints/BP_ThirdPersonCharacter.BP_ThirdPersonCharacter_C|GetHasGreenKey _asbp_third_person_character)
    (Rendering|SetVisibility (Variables|Default|Getgreen_key_001) true false))
  (if (Variables|/Game/ThirdPerson/Blueprints/BP_ThirdPersonCharacter.BP_ThirdPersonCharacter_C|GetHasKey _asbp_third_person_character)
    (Rendering|SetVisibility (Variables|Default|Getyellow_key_002) true false)
    (if (Math|Boolean|ANDBoolean (Variables|/Game/ThirdPerson/Blueprints/BP_ThirdPersonCharacter.BP_ThirdPersonCharacter_C|GetHasRedKey _asbp_third_person_character) (Variables|/Game/ThirdPerson/Blueprints/BP_ThirdPersonCharacter.BP_ThirdPersonCharacter_C|GetHasBlueKey _asbp_third_person_character) (Variables|/Game/ThirdPerson/Blueprints/BP_ThirdPersonCharacter.BP_ThirdPersonCharacter_C|GetHasGreenKey _asbp_third_person_character) (Variables|/Game/ThirdPerson/Blueprints/BP_ThirdPersonCharacter.BP_ThirdPersonCharacter_C|GetHasKey _asbp_third_person_character))
      (Default|ClearKeys _asbp_third_person_character)
      (CallFunction|OpenDoor))))

(fn ConstructionScript)

(fn ResetDoor
  (bind _door (Variables|Default|Getdoor))
  ;[1 1 1] Hide keys that are visibly in the door
  (Rendering|SetVisibility (Variables|Default|Getred_key_003) false false)
  (Rendering|SetVisibility _door true false)
  (Collision|SetCollisionEnabled _door "QueryAndPhysics")
  (Collision|SetCollisionEnabled (Variables|Default|Gettrigger) "QueryOnly"))

(fn OpenDoor
  ;[1 1 1] Make door invisible and disable collisions
  (Rendering|SetVisibility (Variables|Default|Getred_key_004) false false)
  (Collision|SetCollisionEnabled (Variables|Default|Getdoor) "NoCollision"))