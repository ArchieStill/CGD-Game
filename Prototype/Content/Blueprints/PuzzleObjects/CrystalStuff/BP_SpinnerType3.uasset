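; BP_SpinnerType3 is a crystal puzzle object made of three block meshes with switchable visibility states.
; Show makes the blocks visible with a translucent blue material, PartiallyHide swaps in a transparent blue material instance, and Hide turns them invisible.
; It contains no spinning or trigger logic of its own, as BeginPlay, overlap and Tick are disabled stubs and the construction script only calls its parent.
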(event EventBeginPlay
  (|CallParentFunction) ; This node is disabled and will not be called.\nDrag off pins to build functionality.
)

(event Collision|EventActorBeginOverlap
  (params (OtherActor :type Actor%20Object%20Reference))
  (|CallParentFunction OtherActor) ; This node is disabled and will not be called.\nDrag off pins to build functionality.
)

(event EventHide
  (Rendering|SetVisibility (Variables|Default|Getblock_001) false false))

(event EventShow
  (bind _block_001 (Variables|Default|Getblock_001))
  (Rendering|SetVisibility _block_001 true false)
  (Rendering|Material|SetMaterial _block_001 0 "/Game/Materials/M_TranslucentBlue.M_TranslucentBlue"))

(event EventTick
  (params (DeltaSeconds :type Float%20%28single-precision%29))
  (|CallParentFunction DeltaSeconds) ; This node is disabled and will not be called.\nDrag off pins to build functionality.
)

(event EventPartiallyHide
  (bind _block_001 (Variables|Default|Getblock_001))
  (Rendering|SetVisibility _block_001 true false)
  (Rendering|Material|SetMaterial _block_001 0 "/Game/Materials/MI_Blue_Transparent_2.MI_Blue_Transparent_2"))

(fn ConstructionScript
  (|CallParentFunction))