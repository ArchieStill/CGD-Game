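; Blue crystal puzzle platform that lights up, flashes and hides on crystal events, and can slide along the Y axis.
; Show records a positive crystal ID, reveals the mesh with a maze or lit material and plays activation audio once.
; PartiallyHide turns it transparent with deactivation audio and Hide makes it invisible, both only for the recorded ID.
; Tick applies swept left/right movement, and overlapping KillBox teleports it to MovePlat's location.
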(event Collision|EventActorBeginOverlap
  (params (OtherActor :type Actor%20Object%20Reference))
  (if (== OtherActor (Variables|Default|GetKillBox))
    (Transformation|SetActorLocation (Transformation|GetActorLocation (Variables|Default|GetMovePlat)) false false)))

(event EventTick
  (params (DeltaSeconds :type Float%20%28single-precision%29))
  (bind _returnvalue (Transformation|GetActorLocation))
  (bind _returnvalue_2 (Transformation|GetActorLocation))
  (bind (_x _y _z) (Math|Vector|BreakVector _returnvalue))
  (bind (_x_2 _y_2 _z_2) (Math|Vector|BreakVector _returnvalue_2))
  (if (Variables|Default|GetMovingLeft)
    (Transformation|SetActorLocation (Math|Vector|MakeVector _x (- _y 5.0) _z) true false)
    (elif (Variables|Default|GetMovingRight)
      (Transformation|SetActorLocation (Math|Vector|MakeVector _x_2 (+ _y_2 5.0) _z_2) true false))))

(event EventShow
  (params (crystal_id :type Integer))
  (bind _platform (Variables|Default|Getplatform))
  (if (> crystal_id 0)
    (Variables|Default|Setcrystal_id_to_hide_this crystal_id))
  (Rendering|SetVisibility _platform true false)
  (if (Variables|Default|GetIsMaze)
    (Rendering|Material|SetMaterial _platform 0 "/Game/Materials/MI_MazeBlue.MI_MazeBlue")
    (else
      (Rendering|Material|SetMaterial _platform 0 "/Game/Materials/Crystal/M_CrystalLit.M_CrystalLit")))
  (if (not (Variables|Default|GetIsLit))
    (Class|FMODAudioComponent|Play (Variables|Default|GetFMODActivateBlueCrystal))
    (Variables|Default|SetIsLit true)))

(event EventPartiallyHide
  (params (crystal_id :type Integer))
  (bind _platform (Variables|Default|Getplatform))
  (Math|Integer|CompareInt crystal_id (Variables|Default|Getcrystal_id_to_hide_this)
    (:==
      (Rendering|SetVisibility _platform true false)
      (Rendering|Material|SetMaterial _platform 0 "/Game/Materials/MI_Blue_Transparent_2.MI_Blue_Transparent_2")
      (if (not (Variables|Default|GetIsFlashing))
        (Class|FMODAudioComponent|Play (Variables|Default|GetFMODDeactivatecrystal))
        (Variables|Default|SetIsFlashing true)))))

(event EventHide
  (params (crystal_id :type Integer))
  (Math|Integer|CompareInt crystal_id (Variables|Default|Getcrystal_id_to_hide_this)
    (:==
      (Rendering|SetVisibility (Variables|Default|Getplatform) false false)
      (Variables|Default|SetIsLit false)
      (Variables|Default|SetIsFlashing false))))

(fn ConstructionScript)