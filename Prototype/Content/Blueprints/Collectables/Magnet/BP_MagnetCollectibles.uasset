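; BP_MagnetCollectibles is a collectible actor that homes in on the player once the player pawn overlaps its HomingArea.
; It first lerps away along the player's forward direction toward a computed push-away point, using the HomeAwayFromPlayer timeline.
; The HomeToPlayer timeline then lerps it toward the player's live location, started when the push finishes or by a short delay that cuts it off.
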(event OnComponentBeginOverlap(HomingArea)
  (params (OverlappedComponent :type Primitive%20Component%20Object%20Reference) (OtherActor :type Actor%20Object%20Reference) (OtherComp :type Primitive%20Component%20Object%20Reference) (OtherBodyIndex :type Integer) (bFromSweep :type Boolean) (SweepResult :type Hit%20Result%20Structure%20%28by%20ref%29))
  (bind _returnvalue (Game|Player|GetPlayerPawn 0))
  (if (== OtherActor _returnvalue)
    (Variables|Default|SetPush%20Away%20Location (+ (Transformation|GetActorLocation) (* (Math|Vector|GetForwardVector (Transformation|GetActorRotation _returnvalue)) 225.0)))
    (Utilities|FlowControl|Sequence
      (:then_0
        (bind _value (Timeline|Home%20Away%20From%20Player PlayFromStart)
          (:Update
            (Transformation|SetActorLocation (Math|Vector|Lerp(Vector) (Transformation|GetActorLocation) (Variables|Default|GetPush%20Away%20Location) _value) false false))
          (:Finished
            (bind _value_2 (Timeline|Home%20To%20Player PlayFromStart)
              (:Update
                (Transformation|SetActorLocation (Math|Vector|Lerp(Vector) (Transformation|GetActorLocation) (Transformation|GetActorLocation (Game|Player|GetPlayerPawn 0)) _value_2) false false))))))
      (:then_1
        (Utilities|FlowControl|Delay 0.4)
        (Audio|Components|Audio|Stop (Variables|Default|GetHome%20Away%20From%20Player))
        (Timeline|Home%20To%20Player PlayFromStart)))))

(event EventBeginPlay)

(event Collision|EventActorBeginOverlap
  (params (OtherActor :type Actor%20Object%20Reference)))

(event EventTick
  (params (DeltaSeconds :type Float%20%28single-precision%29)))

(fn ConstructionScript)