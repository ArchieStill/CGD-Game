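; Collectable item, configured by the pot that gives it a type, that adds its value to the player's coins.
; SetItemType finds the matching enum row in DT_Items and applies its mesh, material and score value.
; The mesh spins every tick; the first overlap by any actor adds the value to GI_PlayerData, plays an FMOD sound and destroys the item.
; Sine-based bobbing is present but its call is disconnected.
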(event OnComponentBeginOverlap(ItemCollectCollision)
  (params (OverlappedComponent :type Primitive%20Component%20Object%20Reference) (OtherActor :type Actor%20Object%20Reference) (OtherComp :type Primitive%20Component%20Object%20Reference) (OtherBodyIndex :type Integer) (bFromSweep :type Boolean) (SweepResult :type Hit%20Result%20Structure%20%28by%20ref%29))
  (if (not (Variables|Default|GetPlayerCollected))
    (Variables|Default|SetPlayerCollected true)
    ;[1 1 1] Gets playerdata implementation and adds the given score of the item dependant on the data table value set for it
    (bind _asgi_player_data (Utilities|Casting|CastToGI_PlayerData (Game|GetGameInstance)))
    (Variables|/Game/Blueprints/GI_PlayerData.GI_PlayerData_C|Setcoins _asgi_player_data (+ (Variables|Default|GetScore%20Value) (Variables|/Game/Blueprints/GI_PlayerData.GI_PlayerData_C|Getcoins _asgi_player_data)))
    (Class|FMODAudioComponent|Play (Variables|Default|GetFMOD%20coin%20pickup))
    (Actor|DestroyActor)))

(event EventBeginPlay
  ;[1 1 1] initialise the relative starting location of the item for the bobbing movement
  (Variables|Default|SetStarting%20bob%20Height (.z (Variables|/Script/Engine.SceneComponent|GetRelativeLocation (Variables|Default|GetItemMesh)))))

(event Collision|EventActorBeginOverlap
  (params (OtherActor :type Actor%20Object%20Reference)))

(event EventTick
  (params (DeltaSeconds :type Float%20%28single-precision%29))
  (Transformation|AddLocalRotation (Variables|Default|GetItemMesh) "0.000000,5.000000,0.000000" false false))

(fn ConstructionScript)

(fn SetItemType
  (params (Item%20Type :type ItemEnum%20Enum :default "NewEnumerator0"))
  (Variables|Default|SetItem%20Type Item%20Type)
  (CallFunction|FindItemDataRowName))

(fn FindItemDataRowName
  ;[1 0.5686 0.02353] For each item in the data table row, get the enum and compare it against the one given to the actor by the pot, if they are the same, set some variables in the actor to reflect that item's nature
  (bind _outrownames (DataTable|GetDataTableRowNames "/Game/Blueprints/Collectables/Pots++/DT_Items.DT_Items"))
  (bind _array_element (Utilities|Array|ForEachLoopwithBreak _outrownames :!label _label)
    (:LoopBody
      (bind _returnvalue (Utilities|GetDataTableRow "/Game/Blueprints/Collectables/Pots++/DT_Items.DT_Items" _array_element)
        (:then
          (if (Utilities|Enum|Equal(Enum) (.itemassignedenum _returnvalue) (Variables|Default|GetItem%20Type))
            (Components|StaticMesh|SetStaticMesh (Variables|Default|GetItemMesh) (.itemmodel _returnvalue))
            (Rendering|Material|SetMaterial (Variables|Default|GetItemMesh) 0 (Rendering|Material|GetMaterial (.itemmodel _returnvalue) 0))
            ;[1 0.5686 0.02353] Score is assigned to a working variable so it is easier to retrieve when working with values later
            (Variables|Default|SetScore%20Value (.scorevalue _returnvalue))
            (goto _label Break)))))))

(fn ShouldItemBob
  (params (Toggle :type Boolean))
  (Variables|Default|SetShouldItemBob Toggle))