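; Breakable tutorial pot that can drop a gold coin when hit and hides its hit prompt once smashed.
; Hit optionally spawns an auto-collected coin above the pot with an upward impulse, then Smash plays FX and FMOD audio.
; A chase boulder overlap also smashes it, without a coin.
; Smashing zero-scales the mesh, ignores pawns and shifts the boulder trigger far upward instead of destroying anything, so Reset can restore it.
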(event OnComponentBeginOverlap(BoulderCollision)
  (params (OverlappedComponent :type Primitive%20Component%20Object%20Reference) (OtherActor :type Actor%20Object%20Reference) (OtherComp :type Primitive%20Component%20Object%20Reference) (OtherBodyIndex :type Integer) (bFromSweep :type Boolean) (SweepResult :type Hit%20Result%20Structure%20%28by%20ref%29))
  (Utilities|Casting|CastToBP_ChaseBoulder OtherActor)
  (CallFunction|Smash))

(event Custom|Smash
  (bind _bouldercollision (Variables|Default|GetBoulderCollision))
  (bind _potmesh (Variables|Default|GetPotMesh))
  (Utilities|FlowControl|Delay 0.0)
  (Collision|SetCollisionResponsetoChannel _potmesh "ECC_Pawn" "ECR_Ignore")
  (Transformation|SetRelativeScale3D _potmesh "0, 0, 0")
  (Transformation|SetWorldLocation _bouldercollision (+ (Transformation|GetWorldLocation _bouldercollision) "0.000000,0.000000,100000.000000") false false)
  (Components|Activation|Activate (Variables|Default|GetPotSmashFX) false)
  (Class|FMODAudioComponent|Play (Variables|Default|GetFMODPotSmash)))

(event Custom|SpawnCoin
  (bind _returnvalue (Game|SpawnActorfromClass "/Game/Blueprints/Collectables/GoldCoin.GoldCoin_C" (Variables|Default|GetCoinSpawn) "Undefined" "MultiplyWithRoot" 0 0))
  (Default|AutoCollect _returnvalue)
  (Physics|SetSimulatePhysics (Variables|/Game/Blueprints/Collectables/GoldCoin.GoldCoin_C|GetCoinMesh _returnvalue) true)
  (Physics|AddImpulse (Variables|/Game/Blueprints/Collectables/GoldCoin.GoldCoin_C|GetCoinMesh _returnvalue) "0.000000,0.000000,500.000000" "None" true))

(event Custom|Reset
  (bind _bouldercollision (Variables|Default|GetBoulderCollision))
  (Collision|SetCollisionResponsetoChannel (Variables|Default|GetPotMesh) "ECC_Pawn" "ECR_Block")
  (Transformation|SetRelativeScale3D (Variables|Default|GetPotMesh) "1.500000,1.500000,1.500000")
  (Transformation|SetWorldLocation _bouldercollision (+ (Transformation|GetWorldLocation _bouldercollision) "0.000000,0.000000,-100000.000000") false false)
  (Variables|Default|Setsmashable true))

(event EventBeginPlay
  (bind _self self)
  (bind _returnvalue (Transformation|GetActorTransform _self))
  (Variables|Default|SetCoinSpawn (Math|Transform|MakeTransform (Math|Vector|MakeVector (.x (.location _returnvalue)) (.y (.location _returnvalue)) (+ (.z (.location _returnvalue)) 2.5e+02)) "0, 0, 0" "1.000000,1.000000,1.000000")))

(event EventHit
  (params (Damage :type Float%20%28double-precision%29) (Hitter :type Actor%20Object%20Reference))
  (if (Variables|Default|Getsmashable)
    (if (Variables|Default|GetCoinCanSpawn)
      (CallFunction|SpawnCoin))
    (CallFunction|Smash)
    (Variables|Default|Setsmashable false)
    (Rendering|SetVisibility (Variables|Default|GetHitPrompt) false false)))

(fn ConstructionScript)