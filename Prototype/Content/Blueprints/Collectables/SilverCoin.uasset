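; SilverCoin is a spinning collectable that adds 5 to the player's score when a BP_ThirdPersonCharacter overlaps it.
; While Spinning is true, Tick rotates the coin mesh by a fixed step each frame, independent of delta time.
; Overlap plays Pickup, destroys only the mesh, stops the spin and credits player 0's character rather than the overlapping actor.
; The actor itself remains, with no guard against repeat overlaps.
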(event EventBeginPlay)

(event Collision|EventActorBeginOverlap
  (params (OtherActor :type Actor%20Object%20Reference))
  (Utilities|Casting|CastToBP_ThirdPersonCharacter OtherActor)
  (Audio|Components|Audio|Play (Variables|Default|GetPickup) 0.0)
  (Components|DestroyComponent (Variables|Default|GetCoinMesh))
  (Variables|Default|SetSpinning false)
  (bind _asbp_third_person_character (Utilities|Casting|CastToBP_ThirdPersonCharacter (Game|GetPlayerCharacter 0)))
  (Variables|/Game/ThirdPerson/Blueprints/BP_ThirdPersonCharacter.BP_ThirdPersonCharacter_C|SetSCORE _asbp_third_person_character (+ (Variables|/Game/ThirdPerson/Blueprints/BP_ThirdPersonCharacter.BP_ThirdPersonCharacter_C|GetSCORE _asbp_third_person_character) 5)))

(event EventTick
  (params (DeltaSeconds :type Float%20%28single-precision%29))
  (if (Variables|Default|GetSpinning)
    (Transformation|AddLocalRotation (Variables|Default|GetCoinMesh) "0.000000,5.000000,0.000000" false false)))

(fn ConstructionScript)