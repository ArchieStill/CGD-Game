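; Relic collectable that the third-person character picks up by touching it.
; On BeginPlay a switch on RelicType sets the mesh, though only Mask has one assigned; Sword, Shield and Totem set an empty mesh.
; Overlap by BP_ThirdPersonCharacter plays an FMOD pickup sound and destroys the mesh and FX components.
; The actor itself remains, with no guard against replaying the sound and no recording of the pickup.
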(event EventBeginPlay
  (bind _relicmesh (Variables|Default|GetRelicMesh))
  (switch Utilities|FlowControl|Switch|SwitchonRelicType (Variables|Default|GetRelicType)
    (:NewEnumerator0
      (Components|StaticMesh|SetStaticMesh _relicmesh "/Game/Models/MASKRELIC/Mask.Mask"))
    (:NewEnumerator1
      (Components|StaticMesh|SetStaticMesh _relicmesh 0))
    (:NewEnumerator2
      (Components|StaticMesh|SetStaticMesh _relicmesh 0))
    (:NewEnumerator3
      (Components|StaticMesh|SetStaticMesh _relicmesh 0))))

(event Collision|EventActorBeginOverlap
  (params (OtherActor :type Actor%20Object%20Reference))
  (Utilities|Casting|CastToBP_ThirdPersonCharacter OtherActor)
  (Class|FMODAudioComponent|Play (Variables|Default|GetFMODRelicPickup))
  (Components|DestroyComponent (Variables|Default|GetRelicMesh))
  (Components|DestroyComponent (Variables|Default|GetRelicFX)))

(fn ConstructionScript)