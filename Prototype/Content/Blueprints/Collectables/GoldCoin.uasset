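; Gold coin collectable that spins in the level and adds one to the coin count in GI_PlayerData when collected.
; Overlap of its box by the third-person character's capsule triggers Collect, which plays an FMOD pickup sound, destroys the box and mesh, and stops spinning.
; AutoCollect offers a second path, spinning the coin faster for a brief delay before calling Collect.
; Rotation is a fixed step per Tick, so it depends on frame rate.
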(event OnComponentBeginOverlap(Box)
  (params (OverlappedComponent :type Primitive%20Component%20Object%20Reference) (OtherActor :type Actor%20Object%20Reference) (OtherComp :type Primitive%20Component%20Object%20Reference) (OtherBodyIndex :type Integer) (bFromSweep :type Boolean) (SweepResult :type Hit%20Result%20Structure%20%28by%20ref%29))
  (bind _asbp_third_person_character (Utilities|Casting|CastToBP_ThirdPersonCharacter OtherActor))
  (if (== (Variables|/Script/Engine.Character|GetCapsuleComponent _asbp_third_person_character) OtherComp)
    (CallFunction|Collect)))

(event Custom|Auto%20Collect
  (Variables|Default|Setauto true)
  (Utilities|FlowControl|Delay 0.4)
  (CallFunction|Collect))

(event Custom|Collect
  (Class|FMODAudioComponent|Play (Variables|Default|GetFMOD%20coin%20pickup))
  (Components|DestroyComponent (Variables|Default|GetBox))
  (Components|DestroyComponent (Variables|Default|GetCoinMesh))
  (Variables|Default|SetSpinning false)
  (bind _asgi_player_data (Utilities|Casting|CastToGI_PlayerData (Game|GetGameInstance)))
  (Math|Integer|IncrementInt (Variables|/Game/Blueprints/GI_PlayerData.GI_PlayerData_C|Getcoins _asgi_player_data)))

(event EventBeginPlay)

(event Collision|EventActorBeginOverlap
  (params (OtherActor :type Actor%20Object%20Reference)))

(event EventTick
  (params (DeltaSeconds :type Float%20%28single-precision%29))
  (if (Variables|Default|GetSpinning)
    (if (Variables|Default|Getauto)
      (Transformation|AddLocalRotation (Variables|Default|GetCoinMesh) "0.000000,25.000000,0.000000" false false)
      (else
        (Transformation|AddLocalRotation (Variables|Default|GetCoinMesh) "0.000000,5.000000,0.000000" false false)))))

(fn ConstructionScript)