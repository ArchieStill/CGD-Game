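; Smashable pot collectable that can pop out a gold or, more rarely, silver coin when hit.
; Hit rolls for a coin if spawning is allowed, launching it upward from above the pot, then smashes it.
; Overlap with the chase boulder smashes it without a coin.
; Smash fakes destruction by zero-scaling the mesh, ignoring pawns, moving boulder collision far away and playing effects, so Reset can restore the same actor.
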(event OnComponentBeginOverlap(BoulderCollision)
  (params (OverlappedComponent :type Primitive%20Component%20Object%20Reference) (OtherActor :type Actor%20Object%20Reference) (OtherComp :type Primitive%20Component%20Object%20Reference) (OtherBodyIndex :type Integer) (bFromSweep :type Boolean) (SweepResult :type Hit%20Result%20Structure%20%28by%20ref%29))
  (Utilities|Casting|CastToBP_ChaseBoulder OtherActor)
  (CallFunction|Smash))

(event Custom|Smash
  (bind _bouldercollision (Variables|Default|GetBoulderCollision))
  (bind _potmesh (Variables|Default|GetPotMesh))
  (Collision|SetCollisionResponsetoChannel _potmesh "ECC_Pawn" "ECR_Ignore")
  (Transformation|SetRelativeScale3D _potmesh "0, 0, 0")
  (Transformation|SetWorldLocation _bouldercollision (+ (Transformation|GetWorldLocation _bouldercollision) "0.000000,0.000000,100000.000000") false false)
  (Components|Activation|Activate (Variables|Default|GetPotSmashFX) false)
  (Audio|Components|Audio|Play (Variables|Default|GetPotSmashSFX) 0.0))

(event Custom|SpawnCoin
  (bind _returnvalue (Math|Random|RandomInteger 10))
  ;[0.2777 1 0.6] Random chance
  (if (>= _returnvalue 4)
    (if (>= _returnvalue 9)
      ;[0.9164 1 0.916] Silver coin spawning
      (bind _returnvalue_2 (Game|SpawnActorfromClass "/Game/Blueprints/Collectables/SilverCoin.SilverCoin_C" (Variables|Default|GetCoinSpawn) "Undefined" "MultiplyWithRoot" 0 0))
      (Physics|AddImpulse (Variables|/Game/Blueprints/Collectables/SilverCoin.SilverCoin_C|GetCoinMesh _returnvalue_2) "0.000000,0.000000,500.000000" "None" true)
      (else
        ;[1 0.8026 0.04144] Gold coin spawning
        (bind _returnvalue_3 (Game|SpawnActorfromClass "/Game/Blueprints/Collectables/GoldCoin.GoldCoin_C" (Variables|Default|GetCoinSpawn) "Undefined" "MultiplyWithRoot" 0 0))
        (Physics|AddImpulse (Variables|/Game/Blueprints/Collectables/GoldCoin.GoldCoin_C|GetCoinMesh _returnvalue_3) "0.000000,0.000000,500.000000" "None" true)))))

(event Custom|Reset
  (bind _bouldercollision (Variables|Default|GetBoulderCollision))
  (Collision|SetCollisionResponsetoChannel (Variables|Default|GetPotMesh) "ECC_Pawn" "ECR_Block")
  (Transformation|SetRelativeScale3D (Variables|Default|GetPotMesh) "1.500000,1.500000,1.500000")
  (Transformation|SetWorldLocation _bouldercollision (+ (Transformation|GetWorldLocation _bouldercollision) "0.000000,0.000000,-100000.000000") false false)
  (Variables|Default|Setsmashable true))

(event EventBeginPlay
  (bind _self self)
  (bind _returnvalue (Transformation|GetActorTransform _self))
  (Variables|Default|SetCoinSpawn (Math|Transform|MakeTransform (Math|Vector|MakeVector (.x (.location _returnvalue)) (.y (.location _returnvalue)) (+ (.z (.location _returnvalue)) 2.5e+02)) "0, 0, 0" "1.000000,1.000000,1.000000")))

(event EventHit
  (params (Damage :type Float%20%28double-precision%29) (Hitter :type Actor%20Object%20Reference))
  (if (Variables|Default|Getsmashable)
    (if (Variables|Default|GetCoinCanSpawn)
      (CallFunction|SpawnCoin))
    (CallFunction|Smash)
    (Variables|Default|Setsmashable false)))

(fn ConstructionScript)