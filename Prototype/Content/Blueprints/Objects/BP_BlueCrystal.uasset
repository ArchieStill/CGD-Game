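; Blue crystal that, when hit, lights up and temporarily shows a linked object through BPI_Showable.
; Hit activates it only while inactive, swapping five crystal meshes to emissive turquoise and starting a countdown.
; Tick runs the timers: in the last quarter of the active time, crystal and object blink on and off together at a fixed interval.
; When the countdown ends, the crystal returns to its base material and hides the object.
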(event EventTick
  (params (DeltaSeconds :type Float%20%28single-precision%29))
  (CallFunction|UpdateTimers DeltaSeconds))

(event EventHit
  (params (Damage :type Float%20%28double-precision%29) (Hitter :type Actor%20Object%20Reference))
  (Math|Float|CompareFloat (Variables|Default|Getactive_timer) 0.0
    (:==
      _)
    (:<
      _))
  (CallFunction|Activate))

(fn ConstructionScript
  (Variables|Default|Setblink_point (* (Variables|Default|Gettime_active) 0.25)))

(fn OpenDoor)

(fn UpdateTimers
  (params (Delta%20Seconds :type Float%20%28double-precision%29))
  (Math|Float|CompareFloat (Variables|Default|Getactive_timer) 0.0
    (:>
      (Math|Float|CompareFloat (Variables|Default|Getactive_timer) (Variables|Default|Getblink_point)
        (:>
          _)
        (:==
          (bind _output_get (Variables|Default|Setblink_timer (- (Variables|Default|Getblink_timer) Delta%20Seconds) :!label _label))
          (Math|Float|CompareFloat _output_get 0.0
            (:>
              _)
            (:==
              (CallFunction|Blink :!label _label_2)
              (Variables|Default|Setblink_timer (Variables|Default|Gettime_to_blink)))
            (:<
              (goto _label_2))))
        (:<
          (goto _label)))
      (bind _output_get_2 (Variables|Default|Setactive_timer (- (Variables|Default|Getactive_timer) Delta%20Seconds)))
      (Math|Float|CompareFloat _output_get_2 0.0
        (:==
          _)
        (:<
          _))
      (CallFunction|Deactivate))))

(fn Activate
  (Rendering|Material|SetMaterial (Variables|Default|GetCrystalBase) 0 "/Game/Materials/M_EmissiveTurquoise.M_EmissiveTurquoise")
  (bind _asbpi_showable (Utilities|Casting|CastToBPI_Showable (Variables|Default|GetObjectToShow)))
  (Default|Show _asbpi_showable)
  (Variables|Default|Setlit true)
  (Variables|Default|Setblink_timer 0.0)
  (Variables|Default|Setactive_timer (Variables|Default|Gettime_active)))

(fn Deactivate
  (Rendering|Material|SetMaterial (Variables|Default|GetCrystalBase) 0 "/Game/Materials/Crystal/M_CrystalBase.M_CrystalBase")
  (bind _asbpi_showable (Utilities|Casting|CastToBPI_Showable (Variables|Default|GetObjectToShow)))
  (Default|Hide _asbpi_showable))

(fn Blink
  (bind _objecttoshow (Variables|Default|GetObjectToShow))
  (if (Variables|Default|Getlit)
    (Rendering|Material|SetMaterial (Variables|Default|GetCrystalBase) 0 "/Game/Materials/Crystal/M_CrystalBase.M_CrystalBase")
    (Variables|Default|Setlit false)
    (bind _asbpi_showable (Utilities|Casting|CastToBPI_Showable _objecttoshow))
    (Default|Hide _asbpi_showable)
    (else
      (Rendering|Material|SetMaterial (Variables|Default|GetCrystalBase) 0 "/Game/Materials/M_EmissiveTurquoise.M_EmissiveTurquoise")
      (Variables|Default|Setlit true)
      (bind _asbpi_showable_2 (Utilities|Casting|CastToBPI_Showable _objecttoshow))
      (Default|Show _asbpi_showable_2))))