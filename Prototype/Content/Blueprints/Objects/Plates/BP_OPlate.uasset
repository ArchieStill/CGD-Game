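; BP_OPlate is a shape plate, with an O component, that lights up once when a third-person character steps into its trigger.
; The trigger overlap calls Activate, which swaps the O component to a lit crystal material and sets the Activated flag to block repeat triggers.
; When ForBoss is set, it also finds the dark room boss and reports its shape through ActivateShapePlate.
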(event OnComponentBeginOverlap(trigger)
  (params (OverlappedComponent :type Primitive%20Component%20Object%20Reference) (OtherActor :type Actor%20Object%20Reference) (OtherComp :type Primitive%20Component%20Object%20Reference) (OtherBodyIndex :type Integer) (bFromSweep :type Boolean) (SweepResult :type Hit%20Result%20Structure%20%28by%20ref%29))
  (if (Utilities|ClassIsChildOf (Utilities|GetClass OtherActor) "/Game/ThirdPerson/Blueprints/BP_ThirdPersonCharacter.BP_ThirdPersonCharacter_C")
    (if (not (Variables|Default|Getactivated))
      (CallFunction|Activate))))

(event EventActivate
  (Rendering|Material|SetMaterial (Variables|Default|GetO) 0 "/Game/Materials/Crystal/M_CrystalLit.M_CrystalLit")
  (Variables|Default|Setactivated true)
  (if (Variables|Default|Getfor_boss)
    (bind _returnvalue (Actor|GetActorOfClass "/Game/Blueprints/Enemies/BP_DarkRoomBoss.BP_DarkRoomBoss_C"))
    (Default|ActivateShapePlate _returnvalue "NewEnumerator1")))

(fn ConstructionScript)