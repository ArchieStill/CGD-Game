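; BP_BigMenuTorch is a standing torch, named for menu use, that can be put out and relit.
; Extinguish swaps the model to a coal material, deactivates the fire effect, hides the point light and stops the FMOD crackle.
; ResetTorch restores the flame material, fire, light and sound, unless the PermanentlyExtinguished flag is set.
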(fn ConstructionScript)

(fn Extinguish
  (Rendering|Material|SetMaterial (Variables|Default|GetTorch_Standing_Test_Model) 0 "/Game/ART+VISUALS/Materials+Textures/Torch/Coal/Coal.Coal")
  (Components|Activation|Deactivate (Variables|Default|GetTorchFire))
  (Rendering|SetVisibility (Variables|Default|GetPointLight) false false)
  (Class|FMODAudioComponent|Stop (Variables|Default|GetFMODCrackle)))

(fn ResetTorch
  (if (not (Variables|Default|Getpermanently_extinguished))
    (Rendering|Material|SetMaterial (Variables|Default|GetTorch_Standing_Test_Model) 0 "/Game/Materials/Torch/M_TorchFlame.M_TorchFlame")
    (Components|Activation|Activate (Variables|Default|GetTorchFire) true)
    (Rendering|SetVisibility (Variables|Default|GetPointLight) true false)
    (Class|FMODAudioComponent|Play (Variables|Default|GetFMODCrackle))))