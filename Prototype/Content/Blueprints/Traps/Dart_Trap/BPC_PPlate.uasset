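; Pressure plate for the dart trap that triggers its linked TrapList when overlapped by a TrapActivationBox.
; The overlap flags the plate as activated and disables the top mesh's collision to prevent retriggering.
; Tick polls that flag and runs two timelines that move the top mesh along Z, pressing it and then returning it.
; When the return finishes, collision and flags reset so the plate can fire again.
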(event Custom|TrapMechanism
  (bind _pressureplatetop (Variables|Default|GetPressurePlateTop))
  ;[1 1 1] Trap has been activated
  (if (Variables|Default|GetPressurePlateActivated)
    ;[1 1 1] Is Trap Returning?
    (if (Variables|Default|GetAnimRun)
      ;[1 1 1] Animation for Button Returning + Resets all bools restarting Button
      (bind _pressureplatefloat (Timeline|Timeline Play)
        (:Update
          ;[1 1 1] Set Position of Static Mesh
          (Transformation|SetRelativeLocation _pressureplatetop (Math|Vector|MakeVector 0.0 0.0 _pressureplatefloat) false false))
        (:Finished
          (Variables|Default|SetAnimRun false)
          (Variables|Default|SetPressurePlateActivated false)
          ;[1 1 1] Turn off Collision when returning
          (Collision|SetCollisionEnabled _pressureplatetop "QueryAndPhysics")
          (Timeline|Timeline SetNewTime)))
      (else
        ;[1 1 1] Animation for Pressure Plate Button + reset bool activated to start reset implemetation
        (bind _pressureplatefloat_2 (Timeline|Timeline_0 Play)
          (:Update
            (Transformation|SetRelativeLocation _pressureplatetop (Math|Vector|MakeVector 0.0 0.0 _pressureplatefloat_2) false false))
          (:Finished
            (Variables|Default|SetAnimRun true)))))
    (else
      (Timeline|Timeline_0 SetNewTime))))

(event Custom|CustomEvent
  ;[1 1 1] Trap Triggered
  (if (not (Variables|Default|GetTrapTriggered))
    (Variables|Default|SetTrapTriggered true)))

(event EventBeginPlay
  (|CallParentFunction) ; This node is disabled and will not be called.\nDrag off pins to build functionality.
)

(event EventTick
  (params (DeltaSeconds :type Float%20%28single-precision%29))
  ;[1 1 1] Checks if triggered every tick
  (|CallParentFunction DeltaSeconds)
  (CallFunction|TrapMechanism))

(event Collision|EventActorBeginOverlap
  (params (OtherActor :type Actor%20Object%20Reference))
  ;[1 1 1] Detect collision with pressure button
  (bind _astrap_activation_box (Utilities|Casting|CastToTrapActivationBox OtherActor))
  (Default|GetFloorDetection _astrap_activation_box)
  (Default|Trigger (Variables|Default|GetTrapList))
  (Variables|Default|SetPressurePlateActivated true)
  ;[1 1 1] Makes buttons not replayed (Dan Implementation)
  (Collision|SetCollisionEnabled (Variables|Default|GetPressurePlateTop) "NoCollision"))

(fn ConstructionScript
  (|CallParentFunction))