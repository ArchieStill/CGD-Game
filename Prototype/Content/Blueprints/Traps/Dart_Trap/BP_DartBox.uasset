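; BP_DartBox is a dart trap that, once set off, fires poison darts from its direction component.
; SetOffTrap latches TrapTriggered, and Tick then spawns a BP_PoisonDart whenever IsDartDestoyed is true, setting its speed and lifespan and adding an FMOD audio component.
; Each tick refreshes that flag from the first BP_PoisonDart found in the level, not necessarily this trap's own dart.
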(event Custom|GetDartDestroyedVariable
  ;[1 1 1] Get Dart Destroyed Bool From BP_PoisonDart
  (bind _outactors (Actor|GetAllActorsOfClass "/Game/Blueprints/Traps/Dart_Trap/BP_PoisonDart.BP_PoisonDart_C"))
  (Variables|Default|SetIsDartDestoyed (Variables|/Game/Blueprints/Traps/Dart_Trap/BP_PoisonDart.BP_PoisonDart_C|GetIsDartDestroyed (Utilities|Array|Get(acopy) _outactors))))

(event EventBeginPlay)

(event Collision|EventActorBeginOverlap
  (params (OtherActor :type Actor%20Object%20Reference))
  (|CallParentFunction OtherActor) ; This node is disabled and will not be called.\nDrag off pins to build functionality.
)

(event EventTick
  (params (DeltaSeconds :type Float%20%28single-precision%29))
  (bind _poisondartdirection (Variables|Default|GetPoisonDartDirection))
  ;[1 1 1] Check if the trap has been activated and the dart has fired
  (CallFunction|GetDartDestroyedVariable)
  (|CallParentFunction DeltaSeconds)
  (if (Variables|Default|GetTrapTriggered)
    (if (Variables|Default|GetIsDartDestoyed)
      ;[1 1 1] If the trap is active and the dart has not been fired yet, make a new dart object
      (bind _returnvalue (Game|SpawnActorfromClass "/Game/Blueprints/Traps/Dart_Trap/BP_PoisonDart.BP_PoisonDart_C" (Math|Transform|MakeTransform (Transformation|GetWorldLocation _poisondartdirection) (Transformation|GetWorldRotation _poisondartdirection) "1.000000,1.000000,1.000000") "Undefined" "MultiplyWithRoot" self 0))
      ;[1 1 1] Comment
      (AddComponent|AddFMODAudioComponent false)
      ;[1 1 1] Set the dart speed and lifespan
      (Default|SetDartLifeSpan _returnvalue (Variables|Default|GetPoison%20Dart%20Life%20Span))
      (Default|SetDartSpeed _returnvalue (Variables|Default|GetPoison%20Dart%20Speed))
      ;[1 1 1] Ensure dart is not spammed
      (if true
        _))))

(event EventSetOffTrap
  (if (not (Variables|Default|GetTrapTriggered))
    (Variables|Default|SetTrapTriggered true)))

(fn ConstructionScript
  (|CallParentFunction))