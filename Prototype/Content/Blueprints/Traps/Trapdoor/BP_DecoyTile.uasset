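; Decoy floor tile trap that drops away so the player falls through.
; Overlapping a TrapActivationBox plays FMOD sound, adds a Niagara effect, disables trapdoor collision and sets DecoyActivated.
; While that flag is set, Tick plays the falling-platform animation and, at full opacity, starts two chained timelines driving a dynamic material's opacity.
; The rotation-based swing and return logic, including collision restore, is disconnected.
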(event Custom|TrapMechanism
  (bind _newvar_0 (Variables|Default|GetNewVar_0))
  ;[1 1 1] Trap has been activated
  (if (Variables|Default|GetDecoyActivated)
    (Components|Animation|PlayAnimation (Variables|Default|GetFallingPlatform) "/Game/Blueprints/Traps/Trapdoor/FallingPlatform_Anim.FallingPlatform_Anim" false)
    (if (== (Variables|Default|GetOpacity) 1.0)
      (bind _transparecy (Timeline|Alpha PlayFromStart)
        (:Update
          (bind _output_get (Variables|Default|SetOpacity _transparecy))
          (Development|PrintString (Utilities|String|ToString(Float) _output_get))
          (Rendering|Material|SetScalarParameterValue _newvar_0 "OpacityInstance" _transparecy :!class /Script/Engine.MaterialInstanceDynamic))
        (:Finished
          (Variables|Default|SetDecoyActivated false)
          (bind _transparecy_2 (Timeline|Timeline PlayFromStart)
            (:Update
              (bind _output_get_2 (Variables|Default|SetOpacity _transparecy_2))
              (Development|PrintString (Utilities|String|ToString(Float) _output_get_2))
              (Rendering|Material|SetScalarParameterValue _newvar_0 "OpacityInstance" _transparecy_2 :!class /Script/Engine.MaterialInstanceDynamic))))))))

(event Custom|CustomEvent
  ;[1 1 1] Trap Triggered
  (if (not (Variables|Default|GetTrapTriggered))
    (Variables|Default|SetTrapTriggered true)))

(event EventBeginPlay
  (|CallParentFunction)
  (bind _returnvalue (Rendering|Material|CreateDynamicMaterialInstance (Variables|Default|GetFallingPlatform) 0 "/Game/Blueprints/Traps/Trapdoor/M_Transparency.M_Transparency" "None" :!class /Script/Engine.PrimitiveComponent))
  (Variables|Default|SetNewVar_0 _returnvalue))

(event EventTick
  (params (DeltaSeconds :type Float%20%28single-precision%29))
  ;[1 1 1] Checks if triggered every tick
  (|CallParentFunction DeltaSeconds)
  (CallFunction|TrapMechanism))

(event Collision|EventActorBeginOverlap
  (params (OtherActor :type Actor%20Object%20Reference))
  ;[1 1 1] Detect collision with falling platform
  (bind _astrap_activation_box (Utilities|Casting|CastToTrapActivationBox OtherActor))
  (Default|GetFloorDetection _astrap_activation_box)
  (Variables|Default|SetDecoyActivated true)
  ;[1 1 1] Trapdoor FMOD
  (Class|FMODAudioComponent|Play (Variables|Default|GetFMODTrapdoor))
  ;[1 1 1] Particle System
  (AddComponent|AddNiagaraComponent false (Math|Transform|MakeTransform "0, 0, 0" "0, 0, 0" "0.050000,0.050000,0.050000"))
  ;[1 1 1] Makes sure player falls (Dan Implementation)
  (Collision|SetCollisionEnabled (Variables|Default|GetTrapdoor) "NoCollision"))

(fn ConstructionScript
  (|CallParentFunction))