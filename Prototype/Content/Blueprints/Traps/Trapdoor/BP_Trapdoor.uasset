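; Trapdoor trap that drops the player when it overlaps a TrapActivationBox, playing an FMOD sound and disabling the cube's collision.
; The overlap sets a flag that Tick polls to play the trapdoor montage and run an Alpha timeline fading a dynamic material's opacity.
; When the montage completes, the timeline reverses, restoring the opacity and re-enabling collision.
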(event Custom|TrapMechanism
  ;[0.05729 0.0556 0.05687] TrapdoorAnimation
  ;;[0.05729 0.0556 0.05687] Trap has been activated
  (if (Variables|Bools|GetDecoyActivated)
    (Variables|Bools|SetDecoyActivated false)
    ;;[0.05729 0.0556 0.05687] Play Montage
    (Animation|Montage|PlayMontage (Variables|Default|GetSkeletalMesh) "/Game/Blueprints/Traps/Trapdoor/Animations/V3Montage.V3Montage"
      (:then
        ;;[0.05729 0.0556 0.05687] Set Alpha of Trapdoor
        (bind (_direction _transparecy) (Timeline|Alpha Play)
          (:Update
            (Rendering|Material|SetScalarParameterValue (Variables|References|GetOpacityInstance) "Opacity Instance" _transparecy :!class /Script/Engine.MaterialInstanceDynamic)
            ;;[0.05729 0.0556 0.05687] Change Collision depending on Timeline Direction
            (switch Utilities|FlowControl|Switch|SwitchonETimelineDirection _direction
              (:Forward
                (Utilities|FlowControl|Delay 0.25)
                (Collision|SetCollisionEnabled (Variables|Default|GetCube) "NoCollision"))
              (:Backward
                (Collision|SetCollisionEnabled (Variables|Default|GetCube) "QueryAndPhysics"))))))
      (:OnCompleted
        (Timeline|Alpha ReverseFromEnd)))))

(event EventBeginPlay
  ;[0.05729 0.0556 0.05687] Create Dynamic instance which gets Opactity Parameter
  (|CallParentFunction)
  (bind _returnvalue (Rendering|Material|CreateDynamicMaterialInstance (Variables|Default|GetSkeletalMesh) 0 "/Game/Materials/Traps/M_OpacityVar.M_OpacityVar" (Utilities|Name|MakeLiteralName "Opacity Instance") :!class /Script/Engine.PrimitiveComponent))
  (Variables|References|SetOpacityInstance _returnvalue))

(event EventTick
  (params (DeltaSeconds :type Float%20%28single-precision%29))
  ;[0.05729 0.0556 0.05687] Checks if triggered every tick
  (|CallParentFunction DeltaSeconds)
  (CallFunction|TrapMechanism))

(event Collision|EventActorBeginOverlap
  (params (OtherActor :type Actor%20Object%20Reference))
  ;[0.05729 0.0556 0.05687] Trapdoor Collision
  ;;[0.05729 0.0556 0.05687] Detect collision with falling platform
  (bind _astrap_activation_box (Utilities|Casting|CastToTrapActivationBox OtherActor))
  (Default|GetFloorDetection _astrap_activation_box)
  (Variables|Bools|SetDecoyActivated true)
  ;;[0.05729 0.0556 0.05687] Trapdoor FMOD (RILEY)
  (Class|FMODAudioComponent|Play (Variables|Default|GetFMODTrapdoor))
  ;;[0.05729 0.0556 0.05687] Makes sure player falls (DAN)
  (Collision|SetCollisionEnabled (Variables|Default|GetCube) "NoCollision"))

(fn ConstructionScript
  (|CallParentFunction))