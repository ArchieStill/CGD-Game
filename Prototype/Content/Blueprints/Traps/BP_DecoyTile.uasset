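; BP_DecoyTile is a trap floor tile that swings open as a trapdoor when it overlaps a TrapActivationBox.
; The overlap sets DecoyActivated, spawns a small Niagara effect and disables trapdoor collision.
; Tick polls TrapMechanism, which plays the TrapdoorSwing timeline to pitch the door, then the Return timeline to restore it.
; When the return finishes, it clears the state flags and re-enables collision.
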(event Custom|TrapMechanism
  (bind _trapdoor (Variables|Default|GetTrapdoor))
  ;[1 1 1] Falling Platform
  (if (Variables|Default|GetDecoyActivated)
    (if (Variables|Default|GetIsTrapReturning)
      (bind _swingreturn (Timeline|Return Play)
        (:Update
          (Transformation|SetRelativeRotation _trapdoor (Math|Rotator|MakeRotator 0.0 _swingreturn 0.0) false false))
        (:Finished
          (Variables|Default|SetIsTrapReturning false)
          (Variables|Default|SetDecoyActivated false)
          (Collision|SetCollisionEnabled _trapdoor "QueryAndPhysics")
          (Timeline|Return SetNewTime)))
      (else
        (bind _swing (Timeline|TrapdoorSwing Play)
          (:Update
            (Transformation|SetRelativeRotation _trapdoor (Math|Rotator|MakeRotator 0.0 _swing 0.0) false false))
          (:Finished
            (Variables|Default|SetIsTrapReturning true)))))
    (else
      (Timeline|TrapdoorSwing SetNewTime))))

(event Custom|CustomEvent
  ;[1 1 1] Trap Triggered
  (if (not (Variables|Default|GetTrapTriggered))
    (Variables|Default|SetTrapTriggered true)))

(event EventBeginPlay
  (|CallParentFunction) ; This node is disabled and will not be called.\nDrag off pins to build functionality.
)

(event EventTick
  (params (DeltaSeconds :type Float%20%28single-precision%29))
  (|CallParentFunction DeltaSeconds)
  (CallFunction|TrapMechanism))

(event Collision|EventActorBeginOverlap
  (params (OtherActor :type Actor%20Object%20Reference))
  ;[1 1 1] Detect collision with falling platform
  (bind _astrap_activation_box (Utilities|Casting|CastToTrapActivationBox OtherActor))
  (Default|GetFloorDetection _astrap_activation_box)
  (Variables|Default|SetDecoyActivated true)
  ;[1 1 1] Particle System
  (AddComponent|AddNiagaraComponent false (Math|Transform|MakeTransform "0, 0, 0" "0, 0, 0" "0.050000,0.050000,0.050000"))
  (Collision|SetCollisionEnabled (Variables|Default|GetTrapdoor) "NoCollision"))

(fn ConstructionScript
  (|CallParentFunction))