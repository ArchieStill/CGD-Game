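; BP_HammerSlammer is a trap with a hammer arm that kills the player character on contact.
; Tick calls Play on ArmTimeline every frame, and the timeline's output sets the pitch of ArmPivot's relative rotation.
; Overlapping KillBox with a BP_ThirdPersonCharacter runs ExecuteDeathSequence on that character's BPC_DeathComponent.
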(event OnComponentBeginOverlap(KillBox)
  (params (OverlappedComponent :type Primitive%20Component%20Object%20Reference) (OtherActor :type Actor%20Object%20Reference) (OtherComp :type Primitive%20Component%20Object%20Reference) (OtherBodyIndex :type Integer) (bFromSweep :type Boolean) (SweepResult :type Hit%20Result%20Structure%20%28by%20ref%29))
  (bind _asbp_third_person_character (Utilities|Casting|CastToBP_ThirdPersonCharacter OtherActor))
  (Default|ExecuteDeathSequence (Actor|GetComponentbyClass _asbp_third_person_character "/Game/Blueprints/DeathSystem/BPC_DeathComponent.BPC_DeathComponent_C")))

(event EventBeginPlay
  (|CallParentFunction) ; This node is disabled and will not be called.\nDrag off pins to build functionality.
)

(event Collision|EventActorBeginOverlap
  (params (OtherActor :type Actor%20Object%20Reference))
  (|CallParentFunction OtherActor) ; This node is disabled and will not be called.\nDrag off pins to build functionality.
)

(event EventTick
  (params (DeltaSeconds :type Float%20%28single-precision%29))
  (bind _newarmrotation (Timeline|ArmTimeline Play)
    (:Update
      (Transformation|SetRelativeRotation (Variables|Default|GetArmPivot) (Math|Rotator|MakeRotator 0.0 _newarmrotation 0.0) false false))))

(fn ConstructionScript
  (|CallParentFunction))