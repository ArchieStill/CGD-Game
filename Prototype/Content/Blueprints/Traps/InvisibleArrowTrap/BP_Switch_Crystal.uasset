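; Crystal switch in the invisible arrow trap folder that toggles a set of linked objects when hit.
; Hit, gated by CanUse, flips Active and calls Activate or Deactivate on each ObjectsToActivate entry through BPI_Activateable, printing failed casts.
; The Tick cooldown only runs while CanUse is already true, and nothing here clears that flag, so it never blocks hits.
; Red and blue material swaps are disconnected, and BeginPlay is empty.
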(event EventBeginPlay
  ;[1 1 1] Sets Initial height
)

(event EventHit
  (params (Damage :type Float%20%28double-precision%29) (Hitter :type Actor%20Object%20Reference))
  ;[1 1 1] Activates "object to activate" if inactive
  (if (Variables|Default|Getcan%20use)
    (if (Variables|Default|Getactive)
      (for _array_element (Variables|Default|Getobjects%20to%20activate)
        (bind _asbpi_activateable (Utilities|Casting|CastToBPI_Activateable _array_element)
          (:then
            (Default|Deactivate _asbpi_activateable))
          (:CastFailed
            (Development|PrintString "cast failed"))))
      (Variables|Default|Setactive false)
      (else
        (for _array_element_2 (Variables|Default|Getobjects%20to%20activate)
          (bind _asbpi_activateable_2 (Utilities|Casting|CastToBPI_Activateable _array_element_2)
            (:then
              (Default|Activate _asbpi_activateable_2))
            (:CastFailed
              (Development|PrintString "cast failed"))))
        (Variables|Default|Setactive true)))))

(event EventTick
  (params (DeltaSeconds :type Float%20%28single-precision%29))
  (if (Variables|Default|Getcan%20use)
    (bind _output_get (Variables|Default|Settimer (- (stale _output_get) DeltaSeconds)))
    (if (< _output_get 0.0)
      (Variables|Default|Setcan%20use true)
      (Variables|Default|Settimer (Variables|Default|Getcooldown)))))

(fn ConstructionScript)