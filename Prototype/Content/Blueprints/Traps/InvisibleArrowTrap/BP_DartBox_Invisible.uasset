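; BP_DartBox_Invisible is a trap dispenser that fires poison darts and can switch between visible and invisible states.
; Trigger clears CanShoot, waits briefly, spawns BP_PoisonDart_Invisible at PoisonDartDirection, passes it the Visible state, plays an FMOD sound and registers itself as the dart's owning box.
; Activate and Deactivate swap a DispenserBlock material between transparent and emissive orange and update Visible.
; Nothing here resets CanShoot.
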(event EventBeginPlay
  (|CallParentFunction) ; This node is disabled and will not be called.\nDrag off pins to build functionality.
)

(event Collision|EventActorBeginOverlap
  (params (OtherActor :type Actor%20Object%20Reference))
  (|CallParentFunction OtherActor) ; This node is disabled and will not be called.\nDrag off pins to build functionality.
)

(event EventTick
  (params (DeltaSeconds :type Float%20%28single-precision%29))
  (|CallParentFunction DeltaSeconds) ; This node is disabled and will not be called.\nDrag off pins to build functionality.
)

(event EventTrigger
  (bind _poisondartdirection (Variables|Default|GetPoisonDartDirection))
  (if (Variables|Default|GetCanShoot)
    (Variables|Default|SetCanShoot false)
    (Utilities|FlowControl|Delay 0.1)
    (bind _returnvalue (Game|SpawnActorfromClass "/Game/Blueprints/Traps/InvisibleArrowTrap/BP_PoisonDart_Invisible.BP_PoisonDart_Invisible_C" (Math|Transform|MakeTransform (Transformation|GetWorldLocation _poisondartdirection) (Transformation|GetWorldRotation _poisondartdirection) "1.000000,1.000000,1.000000") "Undefined" "MultiplyWithRoot" self 0))
    (Default|Show _returnvalue (Variables|Default|GetVisible))
    (Class|FMODAudioComponent|Play (Variables|Default|GetFMODDartSound))
    (Variables|/Game/Blueprints/Traps/Dart_Trap/BP_PoisonDart.BP_PoisonDart_C|SetOwningDartBox _returnvalue self)))

(event EventDeactivate
  (Rendering|Material|SetMaterial (Variables|Default|GetDispenserBlock) 1 "/Game/Materials/M_EmissiveOrange.M_EmissiveOrange")
  (Variables|Default|SetVisible true))

(event EventActivate
  (Rendering|Material|SetMaterial (Variables|Default|GetDispenserBlock) 1 "/Game/Materials/MI_Orange_Transparent.MI_Orange_Transparent")
  (Variables|Default|SetVisible false))

(fn ConstructionScript
  (|CallParentFunction))