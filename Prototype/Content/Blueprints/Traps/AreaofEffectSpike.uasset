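; Area-of-effect spike floor trap that raises spikes with sound and Niagara effects and kills the player through their death component.
; A detection overlap calls Trigger, which activates this trap only for a TrapActivationBox, then after a delay activates nearby Spike-tagged traps not yet detected.
; After another delay it kills any player inside the search box.
; Tick drives the spike movement timeline, and a separate hit box kills on contact when CanSpike is set.
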(event OnComponentBeginOverlap(DetectionBox)
  (params (OverlappedComponent :type Primitive%20Component%20Object%20Reference) (OtherActor :type Actor%20Object%20Reference) (OtherComp :type Primitive%20Component%20Object%20Reference) (OtherBodyIndex :type Integer) (bFromSweep :type Boolean) (SweepResult :type Hit%20Result%20Structure%20%28by%20ref%29))
  ;[1 1 1] Detection
  (Variables|Default|SetBOOLBOOL true)
  (CallFunction|Trigger OtherActor)
  (Utilities|FlowControl|Delay 1.2)
  (for _array_element (Collision|GetOverlappingActors (Variables|Default|GetSearchBox) "AreaofEffectSpike_C" :!class /Script/Engine.PrimitiveComponent)
    (if (Actor|ActorHasTag _array_element "Spike")
      (bind _asareaof_effect_spike (Utilities|Casting|CastToAreaofEffectSpike _array_element))
      (if (not (Variables|AreaofEffectSpike_C|GetBOOLBOOL _asareaof_effect_spike))
        (Variables|AreaofEffectSpike_C|SetFloorTrapActivated _asareaof_effect_spike true))))
  (Audio|PlaySound2D "/Game/Audio/Samples/Effects/Spike_Trap_v1.Spike_Trap_v1" 0.1 1.0 0.0 0 0 false)
  (AddComponent|AddNiagaraComponent false (Math|Transform|MakeTransform "0, 0, 0" "0, 0, 0" "0.050000,0.050000,0.050000"))
  (Utilities|FlowControl|Delay 0.5)
  (for _array_element_2 (Collision|GetOverlappingActors (Variables|Default|GetSearchBox) 0 :!class /Script/Engine.PrimitiveComponent)
    (bind _asbp_third_person_character (Utilities|Casting|CastToBP_ThirdPersonCharacter _array_element_2))
    (Default|ExecuteDeathSequence (Variables|/Game/ThirdPerson/Blueprints/BP_ThirdPersonCharacter.BP_ThirdPersonCharacter_C|GetBPC_Death%20Component _asbp_third_person_character))))

(event OnComponentBeginOverlap(HitBox)
  (params (OverlappedComponent :type Primitive%20Component%20Object%20Reference) (OtherActor :type Actor%20Object%20Reference) (OtherComp :type Primitive%20Component%20Object%20Reference) (OtherBodyIndex :type Integer) (bFromSweep :type Boolean) (SweepResult :type Hit%20Result%20Structure%20%28by%20ref%29))
  ;[1 1 1] Player Overlap
  (bind _asbp_third_person_character (Utilities|Casting|CastToBP_ThirdPersonCharacter OtherActor))
  (if (Variables|Default|Getcan%20spike)
    (Default|ExecuteDeathSequence (Actor|GetComponentbyClass _asbp_third_person_character "/Game/Blueprints/DeathSystem/BPC_DeathComponent.BPC_DeathComponent_C"))
    (Variables|Default|Setcan%20spike true)))

(event EventTick
  (params (DeltaSeconds :type Float%20%28single-precision%29))
  ;[1 1 1] Spear Movement
  (if (Variables|Default|GetFloorTrapActivated)
    (bind _movement (Timeline|Spear_Movement Play)
      (:Update
        (Transformation|SetRelativeLocation (Variables|Default|GetSpikes) (Math|Vector|MakeVector 0.0 0.0 _movement) false false))
      (:Finished
        (Variables|Default|SetFloorTrapActivated false)))
    (else
      (Timeline|Spear_Movement PlayFromStart))))

(fn ConstructionScript
  (|CallParentFunction))

(fn Start)

(fn Trigger
  (params (Object :type Object%20Object%20Reference))
  (bind _astrap_activation_box (Utilities|Casting|CastToTrapActivationBox Object))
  (Default|GetFloorDetection _astrap_activation_box)
  (if (not (Variables|Default|GetFloorTrapActivated))
    (Variables|Default|SetFloorTrapActivated true)
    ;[1 1 1] Play Audio
    (Audio|PlaySound2D "/Game/Audio/Samples/Effects/Spike_Trap_v1.Spike_Trap_v1" 0.1 1.0 0.0 0 0 false)
    ;[1 1 1] Particle
    (AddComponent|AddNiagaraComponent false (Math|Transform|MakeTransform "0, 0, 0" "0, 0, 0" "0.200000,0.200000,0.200000"))))