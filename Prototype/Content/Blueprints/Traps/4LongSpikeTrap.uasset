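; Long spike trap with four spike sections that kills the player character.
; A TrapActivationBox entering DetectionLongBox arms it, playing a sound, spawning Niagara dust and opening a three-second lethal window.
; Tick runs a timeline moving the sections along separate tracks while active, and restarts it every idle frame.
; Each section's hit box calls BPC_DeathComponent only when the capsule begins overlapping during that window; an overlapping-actor kill check is unwired.
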(event OnComponentBeginOverlap(FrontHitBox)
  (params (OverlappedComponent :type Primitive%20Component%20Object%20Reference) (OtherActor :type Actor%20Object%20Reference) (OtherComp :type Primitive%20Component%20Object%20Reference) (OtherBodyIndex :type Integer) (bFromSweep :type Boolean) (SweepResult :type Hit%20Result%20Structure%20%28by%20ref%29))
  ;[1 1 1] Front Box
  (bind _asbp_third_person_character (Utilities|Casting|CastToBP_ThirdPersonCharacter OtherActor))
  (if (== OtherComp (Variables|/Script/Engine.Character|GetCapsuleComponent _asbp_third_person_character))
    (if (Variables|Default|GetCanLargeSpike)
      (Default|ExecuteDeathSequence (Actor|GetComponentbyClass _asbp_third_person_character "/Game/Blueprints/DeathSystem/BPC_DeathComponent.BPC_DeathComponent_C")))))

(event OnComponentBeginOverlap(MiddleHitBox)
  (params (OverlappedComponent :type Primitive%20Component%20Object%20Reference) (OtherActor :type Actor%20Object%20Reference) (OtherComp :type Primitive%20Component%20Object%20Reference) (OtherBodyIndex :type Integer) (bFromSweep :type Boolean) (SweepResult :type Hit%20Result%20Structure%20%28by%20ref%29))
  ;[1 1 1] Middle Box
  (bind _asbp_third_person_character (Utilities|Casting|CastToBP_ThirdPersonCharacter OtherActor))
  (if (== OtherComp (Variables|/Script/Engine.Character|GetCapsuleComponent _asbp_third_person_character))
    (if (Variables|Default|GetCanLargeSpike)
      (Default|ExecuteDeathSequence (Actor|GetComponentbyClass _asbp_third_person_character "/Game/Blueprints/DeathSystem/BPC_DeathComponent.BPC_DeathComponent_C")))))

(event OnComponentBeginOverlap(BackHitBox)
  (params (OverlappedComponent :type Primitive%20Component%20Object%20Reference) (OtherActor :type Actor%20Object%20Reference) (OtherComp :type Primitive%20Component%20Object%20Reference) (OtherBodyIndex :type Integer) (bFromSweep :type Boolean) (SweepResult :type Hit%20Result%20Structure%20%28by%20ref%29))
  ;[1 1 1] Back Box
  (bind _asbp_third_person_character (Utilities|Casting|CastToBP_ThirdPersonCharacter OtherActor))
  (if (== OtherComp (Variables|/Script/Engine.Character|GetCapsuleComponent _asbp_third_person_character))
    (if (Variables|Default|GetCanLargeSpike)
      (Default|ExecuteDeathSequence (Actor|GetComponentbyClass _asbp_third_person_character "/Game/Blueprints/DeathSystem/BPC_DeathComponent.BPC_DeathComponent_C")))))

(event OnComponentBeginOverlap(DetectionLongBox)
  (params (OverlappedComponent :type Primitive%20Component%20Object%20Reference) (OtherActor :type Actor%20Object%20Reference) (OtherComp :type Primitive%20Component%20Object%20Reference) (OtherBodyIndex :type Integer) (bFromSweep :type Boolean) (SweepResult :type Hit%20Result%20Structure%20%28by%20ref%29))
  ;[1 1 1] Trap Detection
  (bind _astrap_activation_box (Utilities|Casting|CastToTrapActivationBox OtherActor))
  (Default|GetFloorDetection _astrap_activation_box)
  (if (not (Variables|Default|GetLargeTrapActivation))
    (Variables|Default|SetLargeTrapActivation true)
    ;;[1 1 1] Sound Activation
    (Audio|PlaySound2D "/Game/Audio/Samples/Effects/Spike_Trap_v1.Spike_Trap_v1" 0.1 1.0 0.0 0 0 false)
    (Utilities|FlowControl|Sequence
      (:then_0
        (Variables|Default|SetCanLargeSpike true)
        (Utilities|FlowControl|Delay 3.0)
        (Variables|Default|SetCanLargeSpike false))
      (:then_1
        ;;[1 1 1] Dust Effect NEEDS WORK
        (AddComponent|AddNiagaraComponent false (Math|Transform|MakeTransform "0.000000,0.000000,-320.000000" "0, 0, 0" "0.200000,0.200000,0.200000"))
        (AddComponent|AddNiagaraComponent false (Math|Transform|MakeTransform "0.000000,0.000000,-150.000000" "0, 0, 0" "0.200000,0.200000,0.200000"))
        (AddComponent|AddNiagaraComponent false (Math|Transform|MakeTransform "0, 0, 0" "0, 0, 0" "0.200000,0.200000,0.200000"))))))

(event OnComponentBeginOverlap(MiddleSecondHitBox)
  (params (OverlappedComponent :type Primitive%20Component%20Object%20Reference) (OtherActor :type Actor%20Object%20Reference) (OtherComp :type Primitive%20Component%20Object%20Reference) (OtherBodyIndex :type Integer) (bFromSweep :type Boolean) (SweepResult :type Hit%20Result%20Structure%20%28by%20ref%29))
  ;[1 1 1] Middle Second Box
  (bind _asbp_third_person_character (Utilities|Casting|CastToBP_ThirdPersonCharacter OtherActor))
  (if (== OtherComp (Variables|/Script/Engine.Character|GetCapsuleComponent _asbp_third_person_character))
    (if (Variables|Default|GetCanLargeSpike)
      (Default|ExecuteDeathSequence (Actor|GetComponentbyClass _asbp_third_person_character "/Game/Blueprints/DeathSystem/BPC_DeathComponent.BPC_DeathComponent_C")))))

(event Collision|EventActorBeginOverlap
  (params (OtherActor :type Actor%20Object%20Reference)))

(event EventTick
  (params (DeltaSeconds :type Float%20%28single-precision%29))
  ;[1 1 1] Object Animation
  (if (Variables|Default|GetLargeTrapActivation)
    (bind (_direction _frontspikemovement _middlesecondmovement _middlespikemovement _rearspikemovement) (Timeline|Large_Spear_Movement Play)
      (:Update
        (Transformation|SetRelativeLocation (Variables|Default|GetFront) (Math|Vector|MakeVector 0.0 -3.3e+02 _frontspikemovement) false false)
        (Transformation|SetRelativeLocation (Variables|Default|GetMiddleSecond) (Math|Vector|MakeVector 0.0 -1.5e+02 _middlesecondmovement) false false)
        (Transformation|SetRelativeLocation (Variables|Default|GetMiddle) (Math|Vector|MakeVector 0.0 45.0 _middlespikemovement) false false)
        (Transformation|SetRelativeLocation (Variables|Default|GetBack) (Math|Vector|MakeVector 0.0 225.0 _rearspikemovement) false false))
      (:Finished
        (Variables|Default|SetLargeTrapActivation false)))
    (else
      (Timeline|Large_Spear_Movement PlayFromStart))))

(fn ConstructionScript)