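; Swinging hammer trap with two arms that loop continuously from BeginPlay and crush the player.
; Chained timelines swing the arms, then return them with a shake, with FMOD slam and cog sounds.
; Left and right kill boxes flag overlaps with TrapActivationBox actors.
; When Tick finds both flags set, it runs the player's death component sequence and plays the FMOD death sound.
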(event OnComponentBeginOverlap(KillBoxRight)
  (params (OverlappedComponent :type Primitive%20Component%20Object%20Reference) (OtherActor :type Actor%20Object%20Reference) (OtherComp :type Primitive%20Component%20Object%20Reference) (OtherBodyIndex :type Integer) (bFromSweep :type Boolean) (SweepResult :type Hit%20Result%20Structure%20%28by%20ref%29))
  ;[0.05729 0.0556 0.05687] When Player is hit by killbox
  (Utilities|Casting|CastToTrapActivationBox OtherActor)
  (Variables|Booleans|SetRightHit true))

(event OnComponentEndOverlap(KillBoxRight)
  (params (OverlappedComponent :type Primitive%20Component%20Object%20Reference) (OtherActor :type Actor%20Object%20Reference) (OtherComp :type Primitive%20Component%20Object%20Reference) (OtherBodyIndex :type Integer))
  ;[0.05729 0.0556 0.05687] When Player is hit by killbox
  (Utilities|Casting|CastToTrapActivationBox OtherActor)
  (Variables|Booleans|SetRightHit false))

(event OnComponentBeginOverlap(KillBoxLeft)
  (params (OverlappedComponent :type Primitive%20Component%20Object%20Reference) (OtherActor :type Actor%20Object%20Reference) (OtherComp :type Primitive%20Component%20Object%20Reference) (OtherBodyIndex :type Integer) (bFromSweep :type Boolean) (SweepResult :type Hit%20Result%20Structure%20%28by%20ref%29))
  ;[0.05729 0.0556 0.05687] When Player is hit by killbox
  (Utilities|Casting|CastToTrapActivationBox OtherActor)
  (Variables|Booleans|SetLeftHit true))

(event OnComponentEndOverlap(KillBoxLeft)
  (params (OverlappedComponent :type Primitive%20Component%20Object%20Reference) (OtherActor :type Actor%20Object%20Reference) (OtherComp :type Primitive%20Component%20Object%20Reference) (OtherBodyIndex :type Integer))
  ;[0.05729 0.0556 0.05687] When Player is hit by killbox
  (Utilities|Casting|CastToTrapActivationBox OtherActor)
  (Variables|Booleans|SetLeftHit false))

(event Custom|HammerEvent
  ;[0.05729 0.0556 0.05687] Animation
  ;;[0.05729 0.0556 0.05687] Collapsing Animation
  (bind (_direction _leftrotate _rightrotate) (Timeline|Arm%20Swing Play)
    (:Update
      ;;[0.05729 0.0556 0.05687] Left Swing
      (Transformation|SetRelativeRotation (Variables|Default|GetLeftArm) (Math|Rotator|MakeRotator 0.0 _leftrotate 0.0) false false)
      (Transformation|SetRelativeRotation (Variables|Default|GetRightArm) (Math|Rotator|MakeRotator 0.0 _rightrotate 0.0) false false))
    (:Finished
      (Class|FMODAudioComponent|Play (Variables|Default|GetFMODSlam))
      ;;[0.05729 0.0556 0.05687] Return Animation, Extended 4 Seconds
      (bind (_direction_2 _returnleft _returnright _shake) (Timeline|Finish%20Shake%20Return PlayFromStart)
        (:Update
          ;;[0.05729 0.0556 0.05687] Left Swing Return
          (Transformation|SetRelativeRotation (Variables|Default|GetLeftArm) (Math|Rotator|MakeRotator 0.0 _returnleft 0.0) false false)
          (Transformation|SetRelativeRotation (Variables|Default|GetRightArm) (Math|Rotator|MakeRotator 0.0 _returnright 0.0) false false)
          ;;[0.05729 0.0556 0.05687] Shake Animation
          (Transformation|SetRelativeLocation (Variables|Default|GetRightArm) (Math|Vector|MakeVector _shake _shake 0.0) false false))
        (:Finished
          (Class|FMODAudioComponent|Stop (Variables|Default|GetFMODCogs))
          (Timeline|Arm%20Swing PlayFromStart))
        (:FMOD
          (Class|FMODAudioComponent|Play (Variables|Default|GetFMODCogs)))))))

(event EventBeginPlay
  ;[0.05729 0.0556 0.05687] When Game Begins, Animation Starts
  (|CallParentFunction)
  (CallFunction|HammerEvent))

(event EventTick
  (params (DeltaSeconds :type Float%20%28single-precision%29))
  ;[0.05729 0.0556 0.05687] Checks whether the player can be killed on tick, enables events
  ;;[0.05729 0.0556 0.05687] Set ThirdPerson Reference
  (bind _asbp_third_person_character (Utilities|Casting|CastToBP_ThirdPersonCharacter (Game|GetPlayerCharacter 0)))
  (Variables|Default|SetAs%20BP%20Third%20Person%20Character _asbp_third_person_character)
  ;;[0.05729 0.0556 0.05687] Is the player getting squashed by both hammers
  (if (and (Variables|Booleans|GetRightHit) (Variables|Booleans|GetLeftHit))
    (Variables|Booleans|SetRightHit false)
    (Variables|Booleans|SetLeftHit false)
    ;;[0.05729 0.0556 0.05687] FMOD Death
    (Class|FMODAudioComponent|SetParameter (Variables|/Game/ThirdPerson/Blueprints/BP_ThirdPersonCharacter.BP_ThirdPersonCharacter_C|GetFMODDeath (Variables|Default|GetAs%20BP%20Third%20Person%20Character)) "DeathType" 1.0)
    ;;[0.05729 0.0556 0.05687] Kill Player
    (Default|ExecuteDeathSequence (Actor|GetComponentbyClass (Variables|Default|GetAs%20BP%20Third%20Person%20Character) "/Game/Blueprints/DeathSystem/BPC_DeathComponent.BPC_DeathComponent_C"))
    ;;[0.05729 0.0556 0.05687] FMOD (RILEY)
    (Class|FMODAudioComponent|Play (Variables|/Game/ThirdPerson/Blueprints/BP_ThirdPersonCharacter.BP_ThirdPersonCharacter_C|GetFMODDeath (Variables|Default|GetAs%20BP%20Third%20Person%20Character)))))

(fn ConstructionScript
  (|CallParentFunction))

(fn GetDeathComponent
  (params (Object :type BP%20Third%20Person%20Character%20Object%20Reference))
  (return 0))