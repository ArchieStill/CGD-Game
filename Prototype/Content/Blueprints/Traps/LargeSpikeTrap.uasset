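; Large spike trap that animates three spike rows and kills the third-person character on contact.
; A TrapActivationBox entering the detection box sets the activation flag and plays sound and dust.
; Tick runs the timeline moving the rows while flagged, otherwise restarts it every frame.
; Front, middle and back hit boxes call the character's death component when CanLargeSpike is set; the post-delay overlap kill checks are unwired.
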(event OnComponentBeginOverlap(FrontHitBox)
  (params (OverlappedComponent :type Primitive%20Component%20Object%20Reference) (OtherActor :type Actor%20Object%20Reference) (OtherComp :type Primitive%20Component%20Object%20Reference) (OtherBodyIndex :type Integer) (bFromSweep :type Boolean) (SweepResult :type Hit%20Result%20Structure%20%28by%20ref%29))
  ;[1 1 1] Front Box
  (bind _asbp_third_person_character (Utilities|Casting|CastToBP_ThirdPersonCharacter OtherActor))
  (if (Variables|Default|GetCanLargeSpike)
    (Default|ExecuteDeathSequence (Actor|GetComponentbyClass _asbp_third_person_character "/Game/Blueprints/DeathSystem/BPC_DeathComponent.BPC_DeathComponent_C"))
    (Variables|Default|SetCanLargeSpike true)))

(event OnComponentBeginOverlap(MiddleHitBox)
  (params (OverlappedComponent :type Primitive%20Component%20Object%20Reference) (OtherActor :type Actor%20Object%20Reference) (OtherComp :type Primitive%20Component%20Object%20Reference) (OtherBodyIndex :type Integer) (bFromSweep :type Boolean) (SweepResult :type Hit%20Result%20Structure%20%28by%20ref%29))
  ;[1 1 1] Middle Box
  (bind _asbp_third_person_character (Utilities|Casting|CastToBP_ThirdPersonCharacter OtherActor))
  (if (Variables|Default|GetCanLargeSpike)
    (Default|ExecuteDeathSequence (Actor|GetComponentbyClass _asbp_third_person_character "/Game/Blueprints/DeathSystem/BPC_DeathComponent.BPC_DeathComponent_C"))
    (Variables|Default|SetCanLargeSpike true)))

(event OnComponentBeginOverlap(BackHitBox)
  (params (OverlappedComponent :type Primitive%20Component%20Object%20Reference) (OtherActor :type Actor%20Object%20Reference) (OtherComp :type Primitive%20Component%20Object%20Reference) (OtherBodyIndex :type Integer) (bFromSweep :type Boolean) (SweepResult :type Hit%20Result%20Structure%20%28by%20ref%29))
  ;[1 1 1] Back Box
  (bind _asbp_third_person_character (Utilities|Casting|CastToBP_ThirdPersonCharacter OtherActor))
  (if (Variables|Default|GetCanLargeSpike)
    (Default|ExecuteDeathSequence (Actor|GetComponentbyClass _asbp_third_person_character "/Game/Blueprints/DeathSystem/BPC_DeathComponent.BPC_DeathComponent_C"))
    (Variables|Default|SetCanLargeSpike true)))

(event OnComponentBeginOverlap(DetectionLongBox)
  (params (OverlappedComponent :type Primitive%20Component%20Object%20Reference) (OtherActor :type Actor%20Object%20Reference) (OtherComp :type Primitive%20Component%20Object%20Reference) (OtherBodyIndex :type Integer) (bFromSweep :type Boolean) (SweepResult :type Hit%20Result%20Structure%20%28by%20ref%29))
  (bind _astrap_activation_box (Utilities|Casting|CastToTrapActivationBox OtherActor))
  (Default|GetFloorDetection _astrap_activation_box)
  (if (not (Variables|Default|GetLargeTrapActivation))
    (Variables|Default|SetLargeTrapActivation true)
    ;[1 1 1] Sound Activation
    (Audio|PlaySound2D "/Game/Audio/Samples/Effects/Spike_Trap_v1.Spike_Trap_v1" 0.1 1.0 0.0 0 0 false)
    ;[1 1 1] Dust Effect
    (AddComponent|AddNiagaraComponent false (Math|Transform|MakeTransform "0, 0, 0" "0, 0, 0" "0.200000,0.200000,0.200000"))
    (Utilities|FlowControl|Delay 0.5)
    (bind _output_get (Variables|Default|SetOverlapping%20Actors (Collision|GetOverlappingActors (Variables|Default|GetFrontHitBox) 0 :!class /Script/Engine.PrimitiveComponent)))
    (Utilities|Array|Add _output_get 0)))

(event Collision|EventActorBeginOverlap
  (params (OtherActor :type Actor%20Object%20Reference)))

(event EventTick
  (params (DeltaSeconds :type Float%20%28single-precision%29))
  ;[1 1 1] Object Animation
  (if (Variables|Default|GetLargeTrapActivation)
    (bind (_direction _frontspikemovement _middlespikemovement _rearspikemovement) (Timeline|Large_Spear_Movement Play)
      (:Update
        (Transformation|SetRelativeLocation (Variables|Default|GetFront) (Math|Vector|MakeVector 0.0 -3.2e+02 _frontspikemovement) false false)
        (Transformation|SetRelativeLocation (Variables|Default|GetMiddle) (Math|Vector|MakeVector 0.0 -1.5e+02 _middlespikemovement) false false)
        (Transformation|SetRelativeLocation (Variables|Default|GetBack) (Math|Vector|MakeVector 0.0 0.0 _rearspikemovement) false false))
      (:Finished
        (Variables|Default|SetLargeTrapActivation false)))
    (else
      (Timeline|Large_Spear_Movement PlayFromStart))))

(fn ConstructionScript)