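; BP_LightArcsSpin is a Hammer level actor that spins a beam effect horizontally around the point where it began play.
; Each Tick moves the Start and End components to opposite sides of a circle, using sine and cosine of elapsed time scaled by Speed, with Distance as radius.
; End's world position feeds the Niagara Beam End variable before that move, so it trails by one update.
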(event EventBeginPlay
  (Variables|Default|SetStartPos (Transformation|GetActorLocation)))

(event EventTick
  (params (DeltaSeconds :type Float%20%28single-precision%29))
  (bind _distance (Variables|Default|GetDistance))
  (bind _startpos (Variables|Default|GetStartPos))
  (Class|NiagaraComponent|SetVariablePosition (Variables|Default|GetBeam) "Beam End" (Transformation|GetWorldLocation (Variables|Default|GetEnd)))
  (Variables|Default|SetLifeTime (+ (Variables|Default|GetLifeTime) DeltaSeconds))
  (Transformation|SetWorldLocation (Variables|Default|GetStart) (+ _startpos (Math|Vector|MakeVector (* (Math|Trig|Sin(Degrees) (* (Variables|Default|GetLifeTime) (Variables|Default|GetSpeed))) _distance) (* (Math|Trig|Cos(Degrees) (* (Variables|Default|GetLifeTime) (Variables|Default|GetSpeed))) _distance) 0.0)) false false)
  (Transformation|SetWorldLocation (Variables|Default|GetEnd) (+ _startpos (Math|Vector|MakeVector (* (Math|Trig|Sin(Degrees) (- (* (Variables|Default|GetLifeTime) (Variables|Default|GetSpeed)) 1.8e+02)) _distance) (* (Math|Trig|Cos(Degrees) (- (* (Variables|Default|GetLifeTime) (Variables|Default|GetSpeed)) 1.8e+02)) _distance) 0.0)) false false))

(fn ConstructionScript)