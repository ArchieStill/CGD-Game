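; BP_OcclusionTriggerBox is a trigger volume that toggles occlusion on a set of actors as the player character enters and leaves it.
; Begin and end overlap events react only to BP_ThirdPersonCharacter and loop over the OccludedObjects list.
; OccludeObject passes the on or off state to each actor's BPC_OcclusionComponent, which handles the occlusion itself.
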(event Collision|EventActorBeginOverlap
  (params (OtherActor :type Actor%20Object%20Reference))
  (Utilities|Casting|CastToBP_ThirdPersonCharacter OtherActor)
  (for _array_element (Variables|Default|GetOccluded%20Objects)
    (CallFunction|OccludeObject _array_element true)))

(event Collision|EventActorEndOverlap
  (params (OtherActor :type Actor%20Object%20Reference))
  (Utilities|Casting|CastToBP_ThirdPersonCharacter OtherActor)
  (for _array_element (Variables|Default|GetOccluded%20Objects)
    (CallFunction|OccludeObject _array_element false)))

(fn ConstructionScript)

(fn OccludeObject
  (params (Actor :type Actor%20Object%20Reference) (Should%20Occlude :type Boolean))
  (Default|ShouldOcclude (Actor|GetComponentbyClass Actor "/Game/Materials/Occlusion/BPC_OcclusionComponent.BPC_OcclusionComponent_C") Should%20Occlude))