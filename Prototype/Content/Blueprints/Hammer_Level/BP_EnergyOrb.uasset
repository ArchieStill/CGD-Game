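; BP_EnergyOrb is a homing projectile in the Hammer level that flies toward a target actor.
; Each tick it sets its ProjectileMovement velocity to the normalized direction toward TargetActor, scaled by Speed, so it steers instantly without easing.
; It destroys itself when it overlaps any actor carrying a BPC_PlayerLink component, with no other effect applied here.
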(event EventTick
  (params (DeltaSeconds :type Float%20%28single-precision%29))
  (Variables|/Script/Engine.MovementComponent|SetVelocity (Variables|Default|GetProjectileMovement) (* (Math|Vector|Normalize (- (Transformation|GetActorLocation (Variables|Default|GetTarget%20Actor)) (Transformation|GetActorLocation))) (Variables|Default|GetSpeed))))

(event Collision|EventActorBeginOverlap
  (params (OtherActor :type Actor%20Object%20Reference))
  (if (Utilities|IsValid (Actor|GetComponentbyClass OtherActor "/Game/Blueprints/Hammer_Level/BPC_PlayerLink.BPC_PlayerLink_C"))
    (Actor|DestroyActor)))

(fn ConstructionScript)