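; BP_Hammer_Interaction handles the player's hammer: pickup, carrying, recall and colour changes.
; Pickup stores a BP_Hammer_Temp reference, and Tick pins a held hammer above the player, facing the pawn's forward vector.
; IA_RetrieveHammer flags a released hammer as retrieving, and Tick feeds it the player's location as a moving target.
; IA_Throw is empty; its launch logic along the character's LightArrow is disconnected for build safety.
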(event Custom|PickUpHammer
  (params (Actor :type Actor%20Object%20Reference))
  ;[0 0 0] Picks up Hammer and assigns reference
  (bind _asbp_hammer_temp (Utilities|Casting|CastToBP_Hammer_Temp Actor))
  (Variables|Default|SetHasHammer true)
  (Variables|Default|SetHammer _asbp_hammer_temp)
  (Variables|Default|SetRetrieving false))

(event Custom|ChangeHammerColour
  (params (New%20Colour :type ENUM_Colours%20Enum :default "NewEnumerator0"))
  ;[0 0 0] Changes Hammer colour when triggered
  (if (Variables|Default|GetHasHammer)
    (Default|UpdateColour (Variables|Default|GetHammer) New%20Colour)))

(event Input|EnhancedActionEvents|EnhancedInputActionIA_Throw
  (params (ActionValue :type Boolean) (ElapsedSeconds :type Float%20%28double-precision%29) (TriggeredSeconds :type Float%20%28double-precision%29) (InputAction :type Input%20Action%20Object%20Reference :default "/Game/ThirdPerson/Input/Actions/IA_Throw.IA_Throw"))
  ;[0 0 0] Throw Hammer
  ;;[1 1 1] Had to decouple for build safety
)

(event Input|EnhancedActionEvents|EnhancedInputActionIA_RetrieveHammer
  (params (ActionValue :type Boolean) (ElapsedSeconds :type Float%20%28double-precision%29) (TriggeredSeconds :type Float%20%28double-precision%29) (InputAction :type Input%20Action%20Object%20Reference :default "/Game/ThirdPerson/Input/Actions/IA_RetrieveHammer.IA_RetrieveHammer"))
  (bind _hammer (Variables|Default|GetHammer))
  ;[0 0 0] Retrieve Hammer
  (:Started
    (if (and (!= (Variables|Default|GetHammer) 0) (== (Variables|Default|GetHasHammer) false))
      (Variables|/Game/Blueprints/Hammer_Level/BP_Hammer_Temp.BP_Hammer_Temp_C|SetRetrieving _hammer true)
      (Variables|/Game/Blueprints/Hammer_Level/BP_Hammer_Temp.BP_Hammer_Temp_C|SetMoving _hammer false)
      (Variables|Default|SetRetrieving true))))

(event EventTick
  (params (DeltaSeconds :type Float%20%28single-precision%29))
  (bind _returnvalue (Game|Player|GetPlayerPawn 0))
  (bind _hammer (Variables|Default|GetHammer))
  (bind _returnvalue_2 (Transformation|GetActorLocation _returnvalue))
  (if (Variables|Default|GetHasHammer)
    ;[0 0 0] Moves Hammer with Player when picked up
    (Transformation|SetActorLocation _hammer (+ _returnvalue_2 "0.000000,0.000000,100.000000") false true)
    (Transformation|SetActorRotation _hammer (Math|Conversions|RotationFromXVector (Transformation|GetActorForwardVector _returnvalue)))
    (else
      ;[0 0 0] Update Hammer's target position each frame to be the Player's current location
      (if (Variables|Default|GetRetrieving)
        (Variables|/Game/Blueprints/Hammer_Level/BP_Hammer_Temp.BP_Hammer_Temp_C|SetRetrieveTargetLocation (Variables|Default|GetHammer) _returnvalue_2)))))