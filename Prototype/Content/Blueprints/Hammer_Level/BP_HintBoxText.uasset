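; Level hint volume that offers the player an optional text hint while they stand inside it.
; On overlap it caches the HintDisplay from BP_ThirdPersonCharacter, passes it HintText and sets the "Press R for a hint" prompt.
; After a retriggerable delay the prompt fades in unless a hint is showing or the overlap has ended.
; Leaving fades the display out and clears both state flags; key 5 prints a debug message.
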(event Collision|EventActorBeginOverlap
  (params (OtherActor :type Actor%20Object%20Reference))
  (if (Utilities|IsValid (Variables|Default|GetHint%20Display))
    _
    (else
      ;[1 1 1] Gets reference to Hint Display
      (bind _asbp_third_person_character (Utilities|Casting|CastToBP_ThirdPersonCharacter (Game|GetPlayerCharacter 0)))
      (Variables|Default|SetHint%20Display (Variables|/Game/ThirdPerson/Blueprints/BP_ThirdPersonCharacter.BP_ThirdPersonCharacter_C|GetHint%20Display _asbp_third_person_character))))
  ;[1 1 1] If not displaying a hint, the game will prompt the Player for an optional hint after a set delay. The player acn press the relevant keybind at any time for the hint.
  (Variables|Default|SetShould%20Display%20Prompt true)
  (Default|SetCurrentHint (Variables|Default|GetHint%20Display) (Variables|Default|GetHint%20Text))
  (Default|UpdateTextDisplay (Variables|Default|GetHint%20Display) "Press R for a hint")
  (Utilities|FlowControl|RetriggerableDelay (Variables|Default|GetDelay%20Before%20Display))
  (if (not (Variables|Default|GetIs%20Displaying%20Hint))
    (if (Variables|Default|GetShould%20Display%20Prompt)
      (Default|SetFadeinandOut (Variables|Default|GetHint%20Display) true false))))

(event Collision|EventActorEndOverlap
  (params (OtherActor :type Actor%20Object%20Reference))
  (Default|SetFadeinandOut (Variables|Default|GetHint%20Display) false true)
  (Variables|Default|SetShould%20Display%20Prompt false)
  (Variables|Default|SetIs%20Displaying%20Hint false))

(event Input|KeyboardEvents|5
  (params (Key :type Key%20Structure :default "None"))
  (:Pressed
    (Development|PrintString "Hello")))

(fn ConstructionScript)