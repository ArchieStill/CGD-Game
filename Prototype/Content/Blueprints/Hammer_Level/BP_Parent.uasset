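; BP_Parent makes a list of Children actors follow its owner's position, acting as a manual alternative to attachment.
; On BeginPlay it stores each child's world-space offset from the owner in the Vectors array, at the matching index.
; Every Tick it moves each child to the owner's location plus that offset without sweeping, so only translation follows, not rotation or scale.
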(event EventBeginPlay
  (for (_array_element _array_index) (Variables|Default|GetChildren)
    (Utilities|Array|SetArrayElem (Variables|Default|GetVectors) _array_index (- (Transformation|GetActorLocation _array_element) (Transformation|GetActorLocation (Components|GetOwner))))))

(event EventTick
  (params (DeltaSeconds :type Float%20%28single-precision%29))
  (for (_array_element _array_index) (Variables|Default|GetChildren)
    (Transformation|SetActorLocation _array_element (+ (Transformation|GetActorLocation (Components|GetOwner)) (Utilities|Array|Get(acopy) (Variables|Default|GetVectors) _array_index)) false false)))