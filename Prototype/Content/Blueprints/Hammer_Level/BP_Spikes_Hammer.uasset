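; Moving spike trap for the hammer level that responds to colour effects; touching the player character only prints a hit message.
; A timeline updated from Tick offsets the actor from its start transform along its arrow's forward vector.
; ApplyEffect scales the timeline play rate to speed up, slow, reverse or freeze it, tinting the meshes with a matching overlay material.
; A shared retriggerable delay restores normal speed and clears the overlay.
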(event Collision|EventActorBeginOverlap
  (params (OtherActor :type Actor%20Object%20Reference))
  (Utilities|Casting|CastToBP_ThirdPersonCharacter OtherActor)
  (Development|PrintString "Hit Player"))

(event EventApplyEffect
  (params (Colour :type ENUM_Colours%20Enum :default "NewEnumerator0"))
  (switch Utilities|FlowControl|Switch|SwitchonENUM_Colours Colour
    (:NewEnumerator1
      (Variables|Default|SetTime%20Multiplier 2.0)
      (for _array_element (Variables|Default|GetComponents)
        (bind _asmesh_component (Utilities|Casting|CastToMeshComponent _array_element))
        (Rendering|Material|SetOverlayMaterial _asmesh_component "/Game/Materials/MI_Red_Transparent.MI_Red_Transparent" :!class /Script/Engine.MeshComponent)))
    (:NewEnumerator2
      (Variables|Default|SetTime%20Multiplier 0.25)
      (for _array_element_2 (Variables|Default|GetComponents)
        (bind _asmesh_component_2 (Utilities|Casting|CastToMeshComponent _array_element_2))
        (Rendering|Material|SetOverlayMaterial _asmesh_component_2 "/Game/Materials/MI_Blue_Transparent.MI_Blue_Transparent" :!class /Script/Engine.MeshComponent)))
    (:NewEnumerator3
      (Variables|Default|SetTime%20Multiplier -1.0)
      (for _array_element_3 (Variables|Default|GetComponents)
        (bind _asmesh_component_3 (Utilities|Casting|CastToMeshComponent _array_element_3))
        (Rendering|Material|SetOverlayMaterial _asmesh_component_3 "/Game/Materials/MI_Yellow_Transparent.MI_Yellow_Transparent" :!class /Script/Engine.MeshComponent)))
    (:NewEnumerator4
      (Variables|Default|SetTime%20Multiplier 0.0)
      (for _array_element_4 (Variables|Default|GetComponents)
        (bind _asmesh_component_4 (Utilities|Casting|CastToMeshComponent _array_element_4))
        (Rendering|Material|SetOverlayMaterial _asmesh_component_4 "/Game/Materials/MI_Green_Transparent.MI_Green_Transparent" :!class /Script/Engine.MeshComponent))))
  (Utilities|FlowControl|RetriggerableDelay 5.0)
  (Variables|Default|SetTime%20Multiplier 1.0)
  (for _array_element_5 (Variables|Default|GetComponents)
    (bind _asmesh_component_5 (Utilities|Casting|CastToMeshComponent _array_element_5))
    (Rendering|Material|SetOverlayMaterial _asmesh_component_5 0 :!class /Script/Engine.MeshComponent)))

(event EventTick
  (params (DeltaSeconds :type Float%20%28single-precision%29))
  (bind _start_pos (Variables|Default|GetStart%20Pos))
  (Components|Timeline|SetPlayRate (Variables|Default|GetOffset) (* (Variables|Default|GetTime%20Multiplier) (Variables|Default|GetBase%20Speed)))
  (bind _z_offset (Timeline|Offset Play)
    (:Update
      (Transformation|SetActorRelativeTransform (Math|Transform|MakeTransform (+ (.location _start_pos) (* _z_offset (Math|Vector|GetForwardVector (Variables|Default|GetArrow)) (Variables|Default|GetDistance%20Mult))) (.rotation _start_pos) (.scale _start_pos)) false false))))

(event EventBeginPlay
  (Variables|Default|SetStart%20Pos (Transformation|GetActorTransform))
  (Utilities|Array|Add (Variables|Default|GetComponents) (Variables|Default|GetSpike3))
  (Utilities|Array|Add (Variables|Default|GetComponents) (Variables|Default|GetSpike2))
  (Utilities|Array|Add (Variables|Default|GetComponents) (Variables|Default|GetSpike1))
  (Utilities|Array|Add (Variables|Default|GetComponents) (Variables|Default|GetSpike))
  (Utilities|Array|Add (Variables|Default|GetComponents) (Variables|Default|GetCube))
  (Utilities|Array|Add (Variables|Default|GetComponents) (Variables|Default|GetCube1)))

(fn ConstructionScript
  (|CallParentFunction))