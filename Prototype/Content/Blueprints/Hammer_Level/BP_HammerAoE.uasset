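; BP_HammerAoE is a short-lived, coloured area-of-effect explosion actor for the hammer level that triggers activatable objects it touches.
; On BeginPlay it sets the Explosion material to match its Colour enum.
; Tick counts Lifetime down and destroys the actor once it runs out.
; On overlap with a BP_ActivatableActor it applies its Colour through ApplyEffect and then calls ActivateObject.
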(event EventBeginPlay
  ;[0 0 0] Sets Colour on spawn
  (switch Utilities|FlowControl|Switch|SwitchonENUM_Colours (Variables|Default|Getcolour)
    (:NewEnumerator0
      (Rendering|Material|SetMaterial (Variables|Default|Getexplosion) 0 "/Game/Materials/M_White.M_White"))
    (:NewEnumerator1
      (Rendering|Material|SetMaterial (Variables|Default|Getexplosion) 0 "/Game/Materials/M_Red_Transparent_.M_Red_Transparent_"))
    (:NewEnumerator2
      (Rendering|Material|SetMaterial (Variables|Default|Getexplosion) 0 "/Game/Materials/MI_Blue_Transparent.MI_Blue_Transparent"))
    (:NewEnumerator3
      (Rendering|Material|SetMaterial (Variables|Default|Getexplosion) 0 "/Game/Materials/MI_Yellow_Transparent.MI_Yellow_Transparent"))
    (:NewEnumerator4
      (Rendering|Material|SetMaterial (Variables|Default|Getexplosion) 0 "/Game/Materials/MI_Green_Transparent.MI_Green_Transparent"))))

(event EventTick
  (params (DeltaSeconds :type Float%20%28single-precision%29))
  ;[0 0 0] Destroys Actor after a set lifetime
  (bind _output_get (Variables|Default|Setlifetime (- (Variables|Default|Getlifetime) DeltaSeconds)))
  (Math|Float|CompareFloat _output_get 0.0
    (:==
      _)
    (:<
      _))
  (Actor|DestroyActor))

(event Collision|EventActorBeginOverlap
  (params (OtherActor :type Actor%20Object%20Reference))
  ;[0 0 0] If it collides with an ActivatableActor, it activates it and applies its colour to the object
  (bind _asbp_activatable_actor (Utilities|Casting|CastToBP_ActivatableActor OtherActor))
  (Default|ApplyEffect _asbp_activatable_actor (Variables|Default|GetColour))
  (Default|ActivateObject _asbp_activatable_actor))

(fn ConstructionScript)