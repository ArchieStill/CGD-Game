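; BP_RagdollActor is a physics actor in the Hammer level that bounces off what it hits until it meets a BP_RagdollTrigger.
; While Bounce is on, each hit drives the Capsule's linear velocity along the normalized impact impulse, scaled by ForceScalar and optionally added to the current velocity.
; Hitting or overlapping the trigger turns bouncing off and applies DampingScalar as the Capsule's angular damping.
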(event Collision|EventHit
  (params (MyComp :type Primitive%20Component%20Object%20Reference) (Other :type Actor%20Object%20Reference) (OtherComp :type Primitive%20Component%20Object%20Reference) (bSelfMoved :type Boolean) (HitLocation :type Vector :default "0, 0, 0") (HitNormal :type Vector :default "0, 0, 0") (NormalImpulse :type Vector :default "0, 0, 0") (Hit :type Hit%20Result%20Structure%20%28by%20ref%29))
  (Utilities|Casting|CastToBP_RagdollTrigger Other
    (:then
      (Variables|Default|SetBounce false)
      (Class|PrimitiveComponent|SetAngularDamping (Variables|Default|GetCapsule) (Variables|Default|GetDamping%20Scalar)))
    (:CastFailed
      (if (Variables|Default|GetBounce)
        (Physics|SetPhysicsLinearVelocity (Variables|Default|GetCapsule) (* (Math|Vector|Normalize NormalImpulse) (Variables|Default|GetForce%20Scalar)) (Variables|Default|GetAdd%20to%20Current%20Velocity) "None")))))

(event Collision|EventActorBeginOverlap
  (params (OtherActor :type Actor%20Object%20Reference))
  (Utilities|Casting|CastToBP_RagdollTrigger OtherActor)
  (Variables|Default|SetBounce false)
  (Class|PrimitiveComponent|SetAngularDamping (Variables|Default|GetCapsule) (Variables|Default|GetDamping%20Scalar)))

(fn ConstructionScript)