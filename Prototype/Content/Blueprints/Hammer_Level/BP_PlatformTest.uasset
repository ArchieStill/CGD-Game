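; BP_PlatformTest is a test platform that spins continuously and responds to colour effects that alter its local time scale.
; Tick rotates the actor at a fixed rate scaled by TimeMultiplier.
; ApplyEffect maps a colour to normal, faster, slower, reversed or frozen motion, tinting the cube with an overlay material for non-white colours.
; A retriggerable delay restores normal speed and clears the overlay after two seconds.
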(event EventApplyEffect
  (params (Colour :type ENUM_Colours%20Enum :default "NewEnumerator0"))
  (switch Utilities|FlowControl|Switch|SwitchonENUM_Colours Colour
    (:NewEnumerator0
      (Variables|Default|SetTime%20Multiplier 1.0))
    (:NewEnumerator1
      (Variables|Default|SetTime%20Multiplier 2.0)
      (Rendering|Material|SetOverlayMaterial (Variables|Default|GetCube) "/Game/Materials/MI_Red_Transparent.MI_Red_Transparent" :!class /Script/Engine.MeshComponent))
    (:NewEnumerator2
      (Variables|Default|SetTime%20Multiplier 0.25)
      (Rendering|Material|SetOverlayMaterial (Variables|Default|GetCube) "/Game/Materials/MI_Blue_Transparent.MI_Blue_Transparent" :!class /Script/Engine.MeshComponent))
    (:NewEnumerator3
      (Variables|Default|SetTime%20Multiplier -1.0)
      (Rendering|Material|SetOverlayMaterial (Variables|Default|GetCube) "/Game/Materials/MI_Yellow_Transparent.MI_Yellow_Transparent" :!class /Script/Engine.MeshComponent))
    (:NewEnumerator4
      (Variables|Default|SetTime%20Multiplier 0.0)
      (Rendering|Material|SetOverlayMaterial (Variables|Default|GetCube) "/Game/Materials/MI_Green_Transparent.MI_Green_Transparent" :!class /Script/Engine.MeshComponent)))
  (Utilities|FlowControl|RetriggerableDelay 2.0)
  (Variables|Default|SetTime%20Multiplier 1.0)
  (Rendering|Material|SetOverlayMaterial (Variables|Default|GetCube) 0 :!class /Script/Engine.MeshComponent))

(event EventTick
  (params (DeltaSeconds :type Float%20%28single-precision%29))
  (Transformation|AddActorLocalRotation (* "0.000000,300.000000,0.000000" (* DeltaSeconds (Variables|Default|GetTime%20Multiplier))) false false))

(fn ConstructionScript
  (|CallParentFunction))