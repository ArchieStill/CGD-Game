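; BP_SpinningObject is a Hammer level object that continuously spins three cylinder components in place.
; Event Tick adds local rotation to each cylinder, scaled by delta seconds for frame-rate independence, with Cylinder2 on a different axis from Cylinder1 and Cylinder3.
; A multi-axis Sphere rotation is present but never runs, and the construction script is empty.
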(event EventTick
  (params (DeltaSeconds :type Float%20%28single-precision%29))
  (Transformation|AddLocalRotation (Variables|Default|GetCylinder2) (* "0.000000,0.000000,45.000000" DeltaSeconds) false false)
  (Transformation|AddLocalRotation (Variables|Default|GetCylinder1) (* "45.000000,0.000000,0.000000" DeltaSeconds) false false)
  (Transformation|AddLocalRotation (Variables|Default|GetCylinder3) (* "45.000000,0.000000,0.000000" DeltaSeconds) false false))

(fn ConstructionScript)