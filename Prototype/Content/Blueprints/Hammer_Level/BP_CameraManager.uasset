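; Camera effects manager owned by the third-person character, acting as a debug-key testbed for post-process effects on its FollowCamera.
; BeginPlay caches the camera from the owner, and NumPad 9 flip-flops the vignette on and off.
; NumPad 0 resets a flashbang timer, but its fade logic is disconnected and Tick is empty.
; Other unwired experiments cover distance-based depth of field and an oscillating vignette.
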(event EventTick
  (params (DeltaSeconds :type Float%20%28single-precision%29)))

(event EventBeginPlay
  ;[0 0 0] Gets Player's camera as a reference
  (bind _asbp_third_person_character (Utilities|Casting|CastToBP_ThirdPersonCharacter (Components|GetOwner)))
  (bind _output_get (Variables|Default|SetFollow%20Camera (Variables|/Game/ThirdPerson/Blueprints/BP_ThirdPersonCharacter.BP_ThirdPersonCharacter_C|GetFollowCamera _asbp_third_person_character))))

(event Input|KeyboardEvents|NumPadZero
  (params (Key :type Key%20Structure :default "None"))
  ;[0 0 0] Flashbang
  (:Pressed
    (Variables|Default|SetTimer (Variables|Default|GetMax%20Timer))))

(event Input|KeyboardEvents|NumPadNine
  (params (Key :type Key%20Structure :default "None"))
  (bind _follow_camera (Variables|Default|GetFollow%20Camera))
  (bind _postprocesssettings (Variables|/Script/Engine.CameraComponent|GetPostProcessSettings _follow_camera))
  ;[0 0 0] Toggle Vignette
  (:Pressed
    (Utilities|FlowControl|FlipFlop
      (:A
        (Utilities|Struct|SetmembersinPostProcessSettings _postprocesssettings 1.0))
      (:B
        (Utilities|Struct|SetmembersinPostProcessSettings _postprocesssettings 0.0)))))