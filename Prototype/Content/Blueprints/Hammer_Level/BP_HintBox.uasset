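; BP_HintBox is an actor in Hammer_Level that fades an on-screen hint in and out as actors enter and leave its overlap area.
; On BeginPlay it creates its own BP_HintDisplay widget for player 0, adds it to the viewport and stores it.
; Begin and end overlap call SetFadeInAndOut on that widget, without filtering the overlapping actor.
; The ActivateHint event is an empty stub.
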(event Custom|Activate%20Hint)

(event Collision|EventActorBeginOverlap
  (params (OtherActor :type Actor%20Object%20Reference))
  (Default|SetFadeinandOut (Variables|Default|GetDisplay%20Widget) true false))

(event Collision|EventActorEndOverlap
  (params (OtherActor :type Actor%20Object%20Reference))
  (Default|SetFadeinandOut (Variables|Default|GetDisplay%20Widget) false true))

(event EventBeginPlay
  ;[1 1 1] Add Hint Display To HUD
  (bind _returnvalue (UserInterface|CreateWidget "/Game/Blueprints/Widget/BP_HintDisplay.BP_HintDisplay_C" (Game|GetPlayerController 0)))
  (UserInterface|Viewport|AddtoViewport _returnvalue 0)
  (Variables|Default|SetDisplay%20Widget _returnvalue))

(fn ConstructionScript)