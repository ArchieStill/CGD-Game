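; BP_ColourChanger is a Hammer Level pickup-style actor that changes the colour of the player's hammer on overlap.
; On BeginPlay it sets its Cylinder's material to match its Colour enum, choosing white, red, blue, yellow or green.
; When a BP_ThirdPersonCharacter overlaps it, it passes that Colour to ChangeHammerColour on the character's BP_Hammer_Interaction component.
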(event Collision|EventActorBeginOverlap
  (params (OtherActor :type Actor%20Object%20Reference))
  (bind _asbp_third_person_character (Utilities|Casting|CastToBP_ThirdPersonCharacter OtherActor))
  (Default|ChangeHammerColour (Actor|GetComponentbyClass _asbp_third_person_character "/Game/Blueprints/Hammer_Level/BP_Hammer_Interaction.BP_Hammer_Interaction_C") (Variables|Default|Getcolour)))

(event EventTick
  (params (DeltaSeconds :type Float%20%28single-precision%29)))

(event EventBeginPlay
  (switch Utilities|FlowControl|Switch|SwitchonENUM_Colours (Variables|Default|Getcolour)
    (:NewEnumerator0
      (Rendering|Material|SetMaterial (Variables|Default|GetCylinder) 0 "/Game/Materials/M_White.M_White"))
    (:NewEnumerator1
      (Rendering|Material|SetMaterial (Variables|Default|GetCylinder) 0 "/Game/Materials/M_Red.M_Red"))
    (:NewEnumerator2
      (Rendering|Material|SetMaterial (Variables|Default|GetCylinder) 0 "/Game/Materials/M_Blue.M_Blue"))
    (:NewEnumerator3
      (Rendering|Material|SetMaterial (Variables|Default|GetCylinder) 0 "/Game/Materials/M_Yellow.M_Yellow"))
    (:NewEnumerator4
      (Rendering|Material|SetMaterial (Variables|Default|GetCylinder) 0 "/Game/Materials/M_Green.M_Green"))))

(fn ConstructionScript)