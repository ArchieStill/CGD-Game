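; BP_CodeCrystal is a crystal in a relic code puzzle that players hit to enter a sequence.
; When hit while active, it reports its index to the CodeManager and flashes purple if the manager accepts it as the correct entry.
; Show and ShowBad swap five crystal meshes to a purple or red glow material for one second, then reset them to dark grey, signalling success or failure.
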(event Custom|ShowBad
  ;[1 1 1] Flashes red to show failure
  (Rendering|Material|SetMaterial (Variables|Default|GetCrystalBase2) 0 "/Game/Materials/EmissiveRed.EmissiveRed")
  (Rendering|Material|SetMaterial (Variables|Default|GetCrystalBase3) 0 "/Game/Materials/EmissiveRed.EmissiveRed")
  (Rendering|Material|SetMaterial (Variables|Default|GetCrystalBase) 0 "/Game/Materials/EmissiveRed.EmissiveRed")
  (Rendering|Material|SetMaterial (Variables|Default|GetCrystalBase4) 0 "/Game/Materials/EmissiveRed.EmissiveRed")
  (Rendering|Material|SetMaterial (Variables|Default|GetCrystalBase1) 0 "/Game/Materials/EmissiveRed.EmissiveRed")
  (Utilities|FlowControl|Delay 1.0)
  (Rendering|Material|SetMaterial (Variables|Default|GetCrystalBase2) 0 "/Game/Materials/M_DarkGrey.M_DarkGrey")
  (Rendering|Material|SetMaterial (Variables|Default|GetCrystalBase3) 0 "/Game/Materials/M_DarkGrey.M_DarkGrey")
  (Rendering|Material|SetMaterial (Variables|Default|GetCrystalBase) 0 "/Game/Materials/M_DarkGrey.M_DarkGrey")
  (Rendering|Material|SetMaterial (Variables|Default|GetCrystalBase4) 0 "/Game/Materials/M_DarkGrey.M_DarkGrey")
  (Rendering|Material|SetMaterial (Variables|Default|GetCrystalBase1) 0 "/Game/Materials/M_DarkGrey.M_DarkGrey"))

(event Custom|Show
  ;[1 1 1] Flashes purple and then resets
  (Rendering|Material|SetMaterial (Variables|Default|GetCrystalBase2) 0 "/Game/Materials/GlowPurple.GlowPurple")
  (Rendering|Material|SetMaterial (Variables|Default|GetCrystalBase3) 0 "/Game/Materials/GlowPurple.GlowPurple")
  (Rendering|Material|SetMaterial (Variables|Default|GetCrystalBase) 0 "/Game/Materials/GlowPurple.GlowPurple")
  (Rendering|Material|SetMaterial (Variables|Default|GetCrystalBase4) 0 "/Game/Materials/GlowPurple.GlowPurple")
  (Rendering|Material|SetMaterial (Variables|Default|GetCrystalBase1) 0 "/Game/Materials/GlowPurple.GlowPurple")
  (Utilities|FlowControl|Delay 1.0)
  (Rendering|Material|SetMaterial (Variables|Default|GetCrystalBase2) 0 "/Game/Materials/M_DarkGrey.M_DarkGrey")
  (Rendering|Material|SetMaterial (Variables|Default|GetCrystalBase3) 0 "/Game/Materials/M_DarkGrey.M_DarkGrey")
  (Rendering|Material|SetMaterial (Variables|Default|GetCrystalBase) 0 "/Game/Materials/M_DarkGrey.M_DarkGrey")
  (Rendering|Material|SetMaterial (Variables|Default|GetCrystalBase4) 0 "/Game/Materials/M_DarkGrey.M_DarkGrey")
  (Rendering|Material|SetMaterial (Variables|Default|GetCrystalBase1) 0 "/Game/Materials/M_DarkGrey.M_DarkGrey"))

(event EventHit
  (params (Damage :type Float%20%28double-precision%29) (Hitter :type Actor%20Object%20Reference))
  ;[1 1 1] Flashes purple when hit if it is the correct entry in the code, notifies the manager it was hit
  (if (Variables|Default|Getactive)
    (bind _success (Default|CrystalHit (Variables|Default|GetcodeManager) (Variables|Default|Getindex)))
    (if _success
      (CallFunction|Show))))

(fn ConstructionScript)