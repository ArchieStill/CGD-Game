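; BP_CodeCrystalManager runs a memory-sequence crystal puzzle, started when the player's capsule enters its box.
; It shows a random code crystal by crystal through a self-calling delayed event, then activates the crystals for hits checked by CrystalHit.
; A mistake flashes all crystals bad and generates a new same-length code, while success lengthens the next.
; Completed codes light the RelicStatue; the third makes it spit, flags the secret trigger complete and destroys the crystals.
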(event OnComponentBeginOverlap(Box)
  (params (OverlappedComponent :type Primitive%20Component%20Object%20Reference) (OtherActor :type Actor%20Object%20Reference) (OtherComp :type Primitive%20Component%20Object%20Reference) (OtherBodyIndex :type Integer) (bFromSweep :type Boolean) (SweepResult :type Hit%20Result%20Structure%20%28by%20ref%29))
  ;[1 1 1] Activates puzzle if the player enters the area
  (if (not (Variables|Default|Getstarted))
    (bind _asbp_third_person_character (Utilities|Casting|CastToBP_ThirdPersonCharacter OtherActor))
    (if (== OtherComp (Variables|/Script/Engine.Character|GetCapsuleComponent _asbp_third_person_character))
      (Variables|Default|Setstarted true)
      (CallFunction|GenerateCode))))

(event Custom|GenerateCode
  ;[1 1 1] Creates a code of a specified length using as many crystals as input
  (Utilities|Array|Clear (Variables|Default|Getcode))
  (for _index (range 0 (- (Variables|Default|GetcodeLength) 1))
    (Utilities|Array|Add (Variables|Default|Getcode) (Math|Random|RandomInteger (Utilities|Array|Length (Variables|Default|Getcrystals)))))
  (Variables|Default|Setloop%20index 0)
  (CallFunction|ShowCode))

(event Custom|Show%20Code
  ;[1 1 1] Displays the code one at a time (for loops don't work with a delay)
  (if (< (Variables|Default|Getloop%20index) (Utilities|Array|Length (Variables|Default|Getcode)))
    (Default|Show (Utilities|Array|Get(acopy) (Variables|Default|Getcrystals) (Utilities|Array|Get(acopy) (Variables|Default|Getcode) (Variables|Default|Getloop%20index))))
    (Utilities|FlowControl|Delay 1.5)
    (Math|Integer|IncrementInt (Variables|Default|Getloop%20index)
      (:%20%20
        (CallFunction|ShowCode)))
    (else
      ;[1 1 1] Allows the crystals to be hit
      (for _array_element (Variables|Default|Getcrystals)
        (Variables|/Game/Blueprints/RelicPuzzle2/BP_CodeCrystal.BP_CodeCrystal_C|Setactive _array_element true)))))

(event Custom|CodeCompleted
  ;[1 1 1] Resets the state of the code manager and crystals
  (for _array_element (Variables|Default|Getcrystals)
    (Variables|/Game/Blueprints/RelicPuzzle2/BP_CodeCrystal.BP_CodeCrystal_C|Setactive _array_element false)
    (Default|Show _array_element))
  (Variables|Default|SetcurrentCodeIndex 0)
  (Math|Integer|IncrementInt (Variables|Default|GetcodeLength)
    (:%20%20
      (bind _result (Math|Integer|IncrementInt (Variables|Default|GetcodesCompleted))
        (:%20%20
          (Utilities|FlowControl|Sequence
            (:then_0
              ;[1 1 1] Shows progression with the statue
              (switch int _result
                (:1
                  (Rendering|SetVisibility (Variables|/Game/Blueprints/RelicPuzzle/BP_RelicStatue.BP_RelicStatue_C|GetPointLight (Variables|Default|GetRelicStatue)) true false))
                (:2
                  (Rendering|SetVisibility (Variables|/Game/Blueprints/RelicPuzzle/BP_RelicStatue.BP_RelicStatue_C|GetPointLight1 (Variables|Default|GetRelicStatue)) true false))
                (:3
                  (Rendering|SetVisibility (Variables|/Game/Blueprints/RelicPuzzle/BP_RelicStatue.BP_RelicStatue_C|GetRectLight (Variables|Default|GetRelicStatue)) true false)
                  (Default|Spit (Variables|Default|GetRelicStatue))
                  (bind _returnvalue (Actor|GetActorOfClass "/Game/Audio/BP/BP_SecretFoundTrigger2.BP_SecretFoundTrigger2_C"))
                  (Variables|/Game/Audio/BP/BP_SecretFoundTrigger2.BP_SecretFoundTrigger2_C|SetPuzzleComplete _returnvalue true))))
            (:then_1
              (if (== (Variables|Default|GetcodesCompleted) 3)
                ;[1 1 1] Destroys the crystals as the puzzle is complete
                (Utilities|FlowControl|Delay 2.0)
                (for _array_element_2 (Variables|Default|Getcrystals)
                  (Actor|DestroyActor _array_element_2))
                (else
                  ;[1 1 1] Generates a new puzzle
                  (Utilities|FlowControl|Delay 2.0)
                  (CallFunction|GenerateCode))))))))))

(event Custom|CodeFailed
  ;[1 1 1] Resets the code and summons a new one of the same length
  (Variables|Default|SetcurrentCodeIndex 0)
  (Utilities|FlowControl|Delay 2.0)
  (CallFunction|GenerateCode))

(event EventBeginPlay
  ;[1 1 1] Sets up variables in the crystals
  (for (_array_element _array_index) (Variables|Default|Getcrystals)
    (Variables|/Game/Blueprints/RelicPuzzle2/BP_CodeCrystal.BP_CodeCrystal_C|Setindex _array_element _array_index)
    (Variables|/Game/Blueprints/RelicPuzzle2/BP_CodeCrystal.BP_CodeCrystal_C|SetcodeManager _array_element self)))

(fn ConstructionScript)

(fn CrystalHit
  (params (index :type Integer))
  ;[1 1 1] Checks if the crystal hit is the correct one in the sequence
  (if (== index (Utilities|Array|Get(acopy) (Variables|Default|Getcode) (Variables|Default|GetcurrentCodeIndex)))
    (Math|Integer|IncrementInt (Variables|Default|GetcurrentCodeIndex)
      (:%20%20
        (if (< (Variables|Default|GetcurrentCodeIndex) (Utilities|Array|Length (Variables|Default|Getcode)))
          (return true)
          (else
            ;[1 1 1] Sets up the next code as this one was completed
            (CallFunction|CodeCompleted)
            (return true)))))
    (else
      ;[1 1 1] Fails the code if it is not correct and makes the crystals flash red
      (for _array_element (Variables|Default|Getcrystals)
        (Variables|/Game/Blueprints/RelicPuzzle2/BP_CodeCrystal.BP_CodeCrystal_C|Setactive _array_element false)
        (Default|ShowBad _array_element))
      (CallFunction|CodeFailed)
      (return false))))