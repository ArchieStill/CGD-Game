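; Boulder chase trigger that releases a chase boulder after the player arrives and redirects it onto flat ground.
; Player overlap with Box starts a Tick countdown, which then activates the referenced boulder on a downward slope direction and switches music through the level's music trigger.
; When a boulder hits Box1, its direction is leveled, with a bounce and controller rumble; the direction guard compares the value to itself, so always passes.
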(event OnComponentBeginOverlap(Box)
  (params (OverlappedComponent :type Primitive%20Component%20Object%20Reference) (OtherActor :type Actor%20Object%20Reference) (OtherComp :type Primitive%20Component%20Object%20Reference) (OtherBodyIndex :type Integer) (bFromSweep :type Boolean) (SweepResult :type Hit%20Result%20Structure%20%28by%20ref%29))
  (if (not (Variables|Default|GetTimerStart))
    (Utilities|Casting|CastToBP_ThirdPersonCharacter OtherActor)
    (Variables|Default|SetTimerStart true)))

(event OnComponentBeginOverlap(Box1)
  (params (OverlappedComponent :type Primitive%20Component%20Object%20Reference) (OtherActor :type Actor%20Object%20Reference) (OtherComp :type Primitive%20Component%20Object%20Reference) (OtherBodyIndex :type Integer) (bFromSweep :type Boolean) (SweepResult :type Hit%20Result%20Structure%20%28by%20ref%29))
  (bind _asbp_chase_boulder (Utilities|Casting|CastToBP_ChaseBoulder OtherActor))
  (if (not (Utilities|Operators|NotEqual(!=) (Variables|/Game/Blueprints/BoulderChase/BP_ChaseBoulder.BP_ChaseBoulder_C|Getdirection _asbp_chase_boulder) (stale _output_get) 0.0))
    (bind _output_get (Variables|/Game/Blueprints/BoulderChase/BP_ChaseBoulder.BP_ChaseBoulder_C|Setdirection _asbp_chase_boulder "0.000000,1.000000,0.000000"))
    (Variables|/Game/Blueprints/BoulderChase/BP_ChaseBoulder.BP_ChaseBoulder_C|SetActive _asbp_chase_boulder true)
    (Game|Feedback|ClientPlayForceFeedback (Game|GetPlayerController 0) "/Game/Blueprints/Rumble/Boulder/FFE_Rumble_BoulderBang.FFE_Rumble_BoulderBang" "None" false false false)
    (Default|Bounce _asbp_chase_boulder 3e+02)))

(event EventTick
  (params (DeltaSeconds :type Float%20%28single-precision%29))
  (if (Variables|Default|GetTimerStart)
    (Variables|Default|SetTimer (- (Variables|Default|GetTimer) DeltaSeconds))
    (if (<= (Variables|Default|GetTimer) 0.0)
      (bind _asbp_chase_boulder (Utilities|Casting|CastToBP_ChaseBoulder (Variables|Default|GetBoulder)))
      (Variables|/Game/Blueprints/BoulderChase/BP_ChaseBoulder.BP_ChaseBoulder_C|Setdirection _asbp_chase_boulder "0.000000,1.000000,-2.000000")
      (Variables|/Game/Blueprints/BoulderChase/BP_ChaseBoulder.BP_ChaseBoulder_C|SetActive _asbp_chase_boulder true)
      (Variables|Default|SetTimerStart false)
      (Variables|Default|SetTimer 1.0)
      (bind _returnvalue (Actor|GetActorOfClass "/Game/Audio/BP_MusicTrigger.BP_MusicTrigger_C"))
      (Default|SwitchMusic _returnvalue))))

(fn ConstructionScript)