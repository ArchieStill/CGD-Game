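; A boulder-chase hurdle that the chase boulder smashes when it overlaps the hurdle's box collision.
; On impact it activates a destruction effect, plays an FMOD smash sound and rumbles the first player's controller.
; Instead of destroying itself, it teleports the collision box far upward and scales the cube to zero.
; Reset reverses this for an activated hurdle, restoring collision and cube scale for reuse.
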(event OnComponentBeginOverlap(BoxCollision)
  (params (OverlappedComponent :type Primitive%20Component%20Object%20Reference) (OtherActor :type Actor%20Object%20Reference) (OtherComp :type Primitive%20Component%20Object%20Reference) (OtherBodyIndex :type Integer) (bFromSweep :type Boolean) (SweepResult :type Hit%20Result%20Structure%20%28by%20ref%29))
  (bind _boxcollision (Variables|Default|GetBoxCollision))
  (Utilities|Casting|CastToBP_ChaseBoulder OtherActor)
  (Transformation|SetWorldLocation _boxcollision (+ (Transformation|GetWorldLocation _boxcollision) "0.000000,0.000000,10000.000000") false true)
  (Transformation|SetRelativeScale3D (Variables|Default|GetCube) "0, 0, 0")
  (Components|Activation|Activate (Variables|Default|GetObstacleDestroy) false)
  (Class|FMODAudioComponent|Play (Variables|Default|GetFMODBoulderSmash))
  (Variables|Default|SetActivted true)
  (Game|Feedback|ClientPlayForceFeedback (Game|GetPlayerController 0) "/Game/Blueprints/Rumble/Boulder/FFE_Rumble_SmallBang.FFE_Rumble_SmallBang" "None" false false false))

(event Custom|Reset
  (bind _boxcollision (Variables|Default|GetBoxCollision))
  (if (Variables|Default|GetActivted)
    (Transformation|SetWorldLocation _boxcollision (+ (Transformation|GetWorldLocation _boxcollision) "0.000000,0.000000,-10000.000000") false true)
    (Transformation|SetRelativeScale3D (Variables|Default|GetCube) "2.000000,2.000000,2.000000")
    (Variables|Default|SetActivted false)))

(fn ConstructionScript)