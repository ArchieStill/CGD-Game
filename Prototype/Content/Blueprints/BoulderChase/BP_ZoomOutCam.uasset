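; Trigger actor for the boulder chase that zooms the player camera out and can send a linked boulder moving downward.
; When the third-person character enters PlayerBox, it calls ZoomCamOut and, if GoDown is set, activates the BP_ChaseBoulder with a downward direction.
; Tick also checks GoDown, performing the same one-shot boulder activation without waiting for overlap and then disabling the box's overlap events.
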(event OnComponentBeginOverlap(PlayerBox)
  (params (OverlappedComponent :type Primitive%20Component%20Object%20Reference) (OtherActor :type Actor%20Object%20Reference) (OtherComp :type Primitive%20Component%20Object%20Reference) (OtherBodyIndex :type Integer) (bFromSweep :type Boolean) (SweepResult :type Hit%20Result%20Structure%20%28by%20ref%29))
  (bind _asbp_third_person_character (Utilities|Casting|CastToBP_ThirdPersonCharacter OtherActor))
  (Default|ZoomCamOut _asbp_third_person_character)
  (bind _asbp_chase_boulder (Utilities|Casting|CastToBP_ChaseBoulder (Variables|Default|GetBoulder)))
  (if (Variables|Default|GetGoDown)
    (Variables|Default|SetGoDown false)
    (Variables|/Game/Blueprints/BoulderChase/BP_ChaseBoulder.BP_ChaseBoulder_C|Setdirection _asbp_chase_boulder "0.000000,0.000000,-2.000000")
    (Variables|/Game/Blueprints/BoulderChase/BP_ChaseBoulder.BP_ChaseBoulder_C|SetActive _asbp_chase_boulder true)))

(event EventTick
  (params (DeltaSeconds :type Float%20%28single-precision%29))
  (if (Variables|Default|GetGoDown)
    (Variables|Default|SetGoDown false)
    (bind _asbp_chase_boulder (Utilities|Casting|CastToBP_ChaseBoulder (Variables|Default|GetBoulder)))
    (Variables|/Game/Blueprints/BoulderChase/BP_ChaseBoulder.BP_ChaseBoulder_C|Setdirection _asbp_chase_boulder "0.000000,0.000000,-2.000000")
    (Variables|/Game/Blueprints/BoulderChase/BP_ChaseBoulder.BP_ChaseBoulder_C|SetActive _asbp_chase_boulder true)
    (Variables|/Script/Engine.PrimitiveComponent|SetbGenerateOverlapEvents (Variables|Default|GetPlayerBox) false)))

(fn ConstructionScript)