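; Trigger volume for the boulder chase that sets a BP_ChaseBoulder in motion when it enters the box.
; Only an overlap by the boulder's Sphere component counts, and only while the boulder's CanKill flag is still off.
; The trigger passes its Direction to the boulder, activates it, records its start position and makes it lethal.
; It also plays a boulder-bang rumble on the first player's controller.
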(event OnComponentBeginOverlap(Box)
  (params (OverlappedComponent :type Primitive%20Component%20Object%20Reference) (OtherActor :type Actor%20Object%20Reference) (OtherComp :type Primitive%20Component%20Object%20Reference) (OtherBodyIndex :type Integer) (bFromSweep :type Boolean) (SweepResult :type Hit%20Result%20Structure%20%28by%20ref%29))
  (bind _asbp_chase_boulder (Utilities|Casting|CastToBP_ChaseBoulder OtherActor))
  (if (and (== OtherComp (Variables|/Game/Blueprints/BoulderChase/BP_ChaseBoulder.BP_ChaseBoulder_C|GetSphere _asbp_chase_boulder)) (not (Variables|/Game/Blueprints/BoulderChase/BP_ChaseBoulder.BP_ChaseBoulder_C|GetCanKill _asbp_chase_boulder)))
    (Variables|/Game/Blueprints/BoulderChase/BP_ChaseBoulder.BP_ChaseBoulder_C|Setdirection _asbp_chase_boulder (Variables|Default|GetDirection))
    (Variables|/Game/Blueprints/BoulderChase/BP_ChaseBoulder.BP_ChaseBoulder_C|SetActive _asbp_chase_boulder true)
    (Game|Feedback|ClientPlayForceFeedback (Game|GetPlayerController 0) "/Game/Blueprints/Rumble/Boulder/FFE_Rumble_BoulderBang.FFE_Rumble_BoulderBang" "None" false false false)
    (Variables|/Game/Blueprints/BoulderChase/BP_ChaseBoulder.BP_ChaseBoulder_C|Setstartpos _asbp_chase_boulder (Transformation|GetActorLocation _asbp_chase_boulder))
    (Variables|/Game/Blueprints/BoulderChase/BP_ChaseBoulder.BP_ChaseBoulder_C|SetCanKill _asbp_chase_boulder true)))

(event EventBeginPlay)

(event Collision|EventActorBeginOverlap
  (params (OtherActor :type Actor%20Object%20Reference)))

(event EventTick
  (params (DeltaSeconds :type Float%20%28single-precision%29)))

(fn ConstructionScript)