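; BP_KeyDoor is a level exit door in the BoulderChase area that opens for a player carrying the key.
; When the third-person character overlaps the detect volume with HasKey set, it calls that character's LevelEnd with the next level and swaps the door mesh to a doorless version.
; A Triggered flag keeps the FMOD level-complete sound from replaying.
; Disconnected leftover nodes hold an alpha game-over widget and a delayed main-menu load.
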(event OnComponentBeginOverlap(DoorDetect)
  (params (OverlappedComponent :type Primitive%20Component%20Object%20Reference) (OtherActor :type Actor%20Object%20Reference) (OtherComp :type Primitive%20Component%20Object%20Reference) (OtherBodyIndex :type Integer) (bFromSweep :type Boolean) (SweepResult :type Hit%20Result%20Structure%20%28by%20ref%29))
  (bind _asbp_third_person_character (Utilities|Casting|CastToBP_ThirdPersonCharacter OtherActor))
  (if (Variables|/Game/ThirdPerson/Blueprints/BP_ThirdPersonCharacter.BP_ThirdPersonCharacter_C|GetHasKey _asbp_third_person_character)
    (Default|LevelEnd _asbp_third_person_character (Variables|Default|GetNext%20Level))
    (Components|StaticMesh|SetStaticMesh (Variables|Default|GetDoor) "/Game/Models/KeyDoorless.KeyDoorless")
    (if (not (Variables|Default|GetTriggered))
      (Variables|Default|SetTriggered true)
      (Class|FMODAudioComponent|Play (Variables|Default|GetFMODLevelComplete)))))

(fn ConstructionScript)