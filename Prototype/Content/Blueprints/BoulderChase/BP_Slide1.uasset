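; Slide segment in the BoulderChase folder that shifts its two cubes forward as trigger boxes are overlapped.
; BeginPlay stores the offset from Cube to Cube1; Box and Box1 alternately move their cube by that offset, gated by a shared flag and triggered by any overlapping actor.
; Two Stopjumpingbox triggers call FinishSlideJump on an overlapping third-person character.
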(event OnComponentBeginOverlap(Box)
  (params (OverlappedComponent :type Primitive%20Component%20Object%20Reference) (OtherActor :type Actor%20Object%20Reference) (OtherComp :type Primitive%20Component%20Object%20Reference) (OtherBodyIndex :type Integer) (bFromSweep :type Boolean) (SweepResult :type Hit%20Result%20Structure%20%28by%20ref%29))
  (bind _cube (Variables|Default|GetCube))
  (if (not (Variables|Default|Getbox1active))
    (Transformation|SetWorldLocation _cube (+ (Transformation|GetWorldLocation _cube) (Variables|Default|Getdistance)) false false)
    (Variables|Default|Setbox1active true)))

(event OnComponentBeginOverlap(Box1)
  (params (OverlappedComponent :type Primitive%20Component%20Object%20Reference) (OtherActor :type Actor%20Object%20Reference) (OtherComp :type Primitive%20Component%20Object%20Reference) (OtherBodyIndex :type Integer) (bFromSweep :type Boolean) (SweepResult :type Hit%20Result%20Structure%20%28by%20ref%29))
  (bind _cube1 (Variables|Default|GetCube1))
  (if (Variables|Default|Getbox1active)
    (Transformation|SetWorldLocation _cube1 (+ (Transformation|GetWorldLocation _cube1) (Variables|Default|Getdistance)) false false)
    (Variables|Default|Setbox1active false)))

(event OnComponentBeginOverlap(stopjumpingbox1)
  (params (OverlappedComponent :type Primitive%20Component%20Object%20Reference) (OtherActor :type Actor%20Object%20Reference) (OtherComp :type Primitive%20Component%20Object%20Reference) (OtherBodyIndex :type Integer) (bFromSweep :type Boolean) (SweepResult :type Hit%20Result%20Structure%20%28by%20ref%29))
  (bind _asbp_third_person_character (Utilities|Casting|CastToBP_ThirdPersonCharacter OtherActor))
  (Default|FinishSlideJump _asbp_third_person_character))

(event OnComponentBeginOverlap(stopjumpingbox)
  (params (OverlappedComponent :type Primitive%20Component%20Object%20Reference) (OtherActor :type Actor%20Object%20Reference) (OtherComp :type Primitive%20Component%20Object%20Reference) (OtherBodyIndex :type Integer) (bFromSweep :type Boolean) (SweepResult :type Hit%20Result%20Structure%20%28by%20ref%29))
  (bind _asbp_third_person_character (Utilities|Casting|CastToBP_ThirdPersonCharacter OtherActor))
  (Default|FinishSlideJump _asbp_third_person_character))

(event EventBeginPlay
  (Variables|Default|Setdistance (- (Transformation|GetWorldLocation (Variables|Default|GetCube1)) (Transformation|GetWorldLocation (Variables|Default|GetCube))))
  (Development|PrintString (Utilities|String|ToString(Vector) (Math|Vector|GetForwardVector (Variables|Default|GetCube))) true true "(R=0.000000,G=0.660000,B=1.000000,A=1.000000)" 5.0))

(fn ConstructionScript)