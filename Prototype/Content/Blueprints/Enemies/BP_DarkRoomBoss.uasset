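; Dark room boss enemy that is defeated by activating shape plates matching the shape shown on its chest.
; A correct plate removes that shape, picks a random remaining one, swaps the chest child actor (cross or circle), and destroys the boss once none remain.
; On BeginPlay it fires a single spike attack, spawning a random number of spike indicators at fixed height, randomly offset around the player.
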(event EventBeginPlay
  (|CallParentFunction)
  (CallFunction|SpikeAttack))

(event Collision|EventActorBeginOverlap
  (params (OtherActor :type Actor%20Object%20Reference)))

(event EventTick
  (params (DeltaSeconds :type Float%20%28single-precision%29)))

(fn ConstructionScript
  (|CallParentFunction))

(fn ActivateShapePlate
  (params (shape :type ENM_DarkRoomBossShape%20Enum :default "NewEnumerator0"))
  (bind _shapes_left (Variables|Default|Getshapes_left))
  (if (== shape (Math|Conversions|ToInteger(Byte) (Variables|Default|Getcurrent_shape)))
    (Utilities|Array|RemoveItem _shapes_left shape)
    (Variables|Default|Setcurrent_shape (.OutItem (Utilities|Array|Random _shapes_left)))
    (CallFunction|UpdateChestShape)
    (CallFunction|CheckifDead)))

(fn CheckifDead
  (if (Utilities|Array|IsEmpty (Variables|Default|Getshapes_left))
    (Actor|DestroyActor)))

(fn UpdateChestShape
  (bind _chest_shape (Variables|Default|Getchest_shape))
  (switch Utilities|FlowControl|Switch|SwitchonENM_DarkRoomBossShape (Variables|Default|Getcurrent_shape)
    (:NewEnumerator0
      (ChildActorComponent|SetChildActorClass _chest_shape "/Game/Blueprints/Components/DarkRoomBoss/BP_DarkRoomBossCross.BP_DarkRoomBossCross_C"))
    (:NewEnumerator1
      (ChildActorComponent|SetChildActorClass _chest_shape "/Game/Blueprints/Components/DarkRoomBoss/BP_DarkRoomBossCircle.BP_DarkRoomBossCircle_C"))))

(fn SpikeAttack
  (bind _returnvalue (Game|GetPlayerCharacter 0))
  (bind _returnvalue_2 (Math|Random|RandomUnitVector))
  (bind _max_spike_distance_from_player (Variables|Default|Getmax_spike_distance_from_player))
  (bind _returnvalue_3 (Transformation|GetActorLocation _returnvalue))
  (bind _returnvalue_4 (* _returnvalue_2 _max_spike_distance_from_player))
  (bind _returnvalue_5 (+ _returnvalue_3 _returnvalue_4))
  (for _index (range 0 (Math|Random|RandomIntegerinRange (Variables|Default|Getmin_spikes_per_attack) (Variables|Default|Getmax_spikes_per_attack)))
    (Game|SpawnActorfromClass "/Game/Blueprints/Components/DarkRoomBoss/BP_DarkRoomBossSpikeIndicator.BP_DarkRoomBossSpikeIndicator_C" (Math|Transform|MakeTransform (Math|Vector|MakeVector (.x _returnvalue_5) (.y _returnvalue_5) -0.995) "0, 0, 0" "1.000000,1.000000,1.000000") "Undefined" "MultiplyWithRoot" 0 0)))