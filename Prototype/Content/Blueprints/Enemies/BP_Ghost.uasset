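; Ghost enemy that relentlessly homes in on the player character and deals effectively lethal damage on contact.
; Every Tick it snaps its rotation to face player 0 and moves along its local forward axis at Speed, scaled by delta time, with no pathfinding.
; A Hitbox overlap with BP_ThirdPersonCharacter calls that character's TakeDamage with a huge amount.
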(event OnComponentBeginOverlap(hitbox)
  (params (OverlappedComponent :type Primitive%20Component%20Object%20Reference) (OtherActor :type Actor%20Object%20Reference) (OtherComp :type Primitive%20Component%20Object%20Reference) (OtherBodyIndex :type Integer) (bFromSweep :type Boolean) (SweepResult :type Hit%20Result%20Structure%20%28by%20ref%29))
  (bind _asbp_third_person_character (Utilities|Casting|CastToBP_ThirdPersonCharacter OtherActor))
  (Default|TakeDamage _asbp_third_person_character 1e+06))

(event EventBeginPlay
  (|CallParentFunction) ; This node is disabled and will not be called.\nDrag off pins to build functionality.
)

(event Collision|EventActorBeginOverlap
  (params (OtherActor :type Actor%20Object%20Reference)))

(event EventTick
  (params (DeltaSeconds :type Float%20%28single-precision%29))
  (Transformation|SetActorRotation (Math|Rotator|FindLookatRotation (Transformation|GetActorLocation) (Transformation|GetActorLocation (Game|GetPlayerCharacter 0))))
  (Transformation|AddActorLocalOffset (Math|Vector|MakeVector (* (Variables|Default|Getspeed) DeltaSeconds) 0.0 0.0) false false))

(fn ConstructionScript
  (|CallParentFunction))