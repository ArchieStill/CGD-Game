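; Enemy that arms itself when the player character overlaps its hitbox, then flashes and blows up after a countdown.
; While detonating, Tick runs two timers slowed by TimeMultiplier: one toggles the body between red and white, the other triggers the explosion.
; The explosion spawns an effect actor sized to the BlastRadius sphere, damages overlapping players and other enemies, destroys explodable doors, then destroys itself.
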(event OnComponentBeginOverlap(hitbox)
  (params (OverlappedComponent :type Primitive%20Component%20Object%20Reference) (OtherActor :type Actor%20Object%20Reference) (OtherComp :type Primitive%20Component%20Object%20Reference) (OtherBodyIndex :type Integer) (bFromSweep :type Boolean) (SweepResult :type Hit%20Result%20Structure%20%28by%20ref%29))
  (if (Utilities|ClassIsChildOf (Utilities|GetClass OtherActor) "/Game/ThirdPerson/Blueprints/BP_ThirdPersonCharacter.BP_ThirdPersonCharacter_C")
    (Variables|Default|Setdetonating true)))

(event EventBeginPlay
  (|CallParentFunction) ; This node is disabled and will not be called.\nDrag off pins to build functionality.
)

(event Collision|EventActorBeginOverlap
  (params (OtherActor :type Actor%20Object%20Reference)))

(event EventTick
  (params (DeltaSeconds :type Float%20%28single-precision%29))
  (|CallParentFunction DeltaSeconds)
  (CallFunction|UpdateDetonation DeltaSeconds))

(fn ConstructionScript
  (|CallParentFunction))

(fn Explode
  (bind _returnvalue (Transformation|GetActorTransform))
  (bind _blast_radius (Variables|Default|Getblast_radius))
  (bind _blast_damage (Variables|Default|Getblast_damage))
  (Game|SpawnActorfromClass "/Game/Blueprints/Objects/BP_Explosion.BP_Explosion_C" (Math|Transform|MakeTransform (.location _returnvalue) (.rotation _returnvalue) (Math|Conversions|ToVector(Float) (/ (Components|Sphere|GetScaledSphereRadius _blast_radius) 5e+01))) "Undefined" "MultiplyWithRoot" 0 0)
  (for _array_element (Collision|GetOverlappingActors _blast_radius 0 :!class /Script/Engine.PrimitiveComponent)
    (bind _asbp_third_person_character (Utilities|Casting|CastToBP_ThirdPersonCharacter _array_element)
      (:then
        (Default|TakeDamage _asbp_third_person_character _blast_damage))
      (:CastFailed
        (bind _asbp_enemy_parent (Utilities|Casting|CastToBP_EnemyParent _array_element)
          (:then
            (if (not (== _asbp_enemy_parent self))
              (Default|TakeDamage _asbp_enemy_parent _blast_damage)))
          (:CastFailed
            (if (Utilities|ClassIsChildOf (Utilities|GetClass _array_element) "/Game/Blueprints/Objects/BP_ExplodableDoor.BP_ExplodableDoor_C")
              (Actor|DestroyActor _array_element)))))))
  (Actor|DestroyActor))

(fn UpdateFlash
  (params (Delta%20Seconds :type Float%20%28double-precision%29))
  (bind _body (Variables|Default|Getbody))
  (bind _output_get (Variables|Default|Setflash_timer (- (Variables|Default|Getflash_timer) (/ Delta%20Seconds (Variables|Default|Gettime_multiplier)))))
  (Math|Float|CompareFloat _output_get 0.0
    (:==
      _)
    (:<
      _))
  (if (== (Rendering|Material|GetMaterial _body 0) "/Game/Materials/M_Red.M_Red")
    (Rendering|Material|SetMaterial _body 0 "/Game/Materials/M_White.M_White")
    (else
      (Rendering|Material|SetMaterial _body 0 "/Game/Materials/M_Red.M_Red")))
  (Variables|Default|Setflash_timer (Variables|Default|Getflash_timer_max)))

(fn UpdateDetonation
  (params (Delta%20Seconds :type Float%20%28double-precision%29))
  (if (Variables|Default|Getdetonating)
    (CallFunction|UpdateFlash Delta%20Seconds)
    (bind _output_get (Variables|Default|Setdetonation_timer (- (Variables|Default|Getdetonation_timer) (/ Delta%20Seconds (Variables|Default|Gettime_multiplier)))))
    (Math|Float|CompareFloat _output_get 0.0
      (:==
        _)
      (:<
        _))
    (CallFunction|Explode)))