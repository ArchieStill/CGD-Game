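; Boss enemy that attacks with a laser, damages the player through an overlap box, and takes hits only while stunned.
; BeginPlay spawns a self-sustaining damage-type laser at its arrow and attaches it, switched off.
; Tick feeds player position to the AI blackboard and fakes attack animation by swapping static meshes, firing the laser on the final step.
; Stun and activation functions set state, mirrored to the blackboard except when un-stunning.
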(event OnComponentBeginOverlap(Box)
  (params (OverlappedComponent :type Primitive%20Component%20Object%20Reference) (OtherActor :type Actor%20Object%20Reference) (OtherComp :type Primitive%20Component%20Object%20Reference) (OtherBodyIndex :type Integer) (bFromSweep :type Boolean) (SweepResult :type Hit%20Result%20Structure%20%28by%20ref%29))
  ;[1 1 1] If the player is in the area of damage box then apply damage to the player character
  (bind _asbp_third_person_character (Utilities|Casting|CastToBP_ThirdPersonCharacter OtherActor))
  (Default|TakeDamage _asbp_third_person_character 3.0))

(event EventBeginPlay
  (bind _arrow (Variables|Default|GetArrow))
  (|CallParentFunction)
  (AI|Components|Blackboard|SetValueasBool (AI|GetBlackboard (Pawn|GetController)) (Utilities|Name|MakeLiteralName "IsActivated") false)
  ;[1 1 1] Create a Laser object at the point of the arrow
  (bind _returnvalue (Game|SpawnActorfromClass "/Game/Blueprints/PuzzleObjects/BP_Laser.BP_Laser_C" (Math|Transform|MakeTransform (Transformation|GetWorldLocation _arrow) (Transformation|GetWorldRotation _arrow) "6.000000,6.000000,1.000000") "Undefined" "MultiplyWithRoot" 0 0))
  ;[1 1 1] Make a reference to the object
  (bind _output_get (Variables|Default|SetLaser _returnvalue))
  ;[1 1 1] Set it to be self sustaining, if it were not it would add to a counter that measures the amount of frames the laser is to be active for. When the laser frame counter eaches the goal frame count it deactivates
  (Variables|/Game/Blueprints/PuzzleObjects/BP_Laser.BP_Laser_C|SetSelfSustaining _output_get true)
  (Default|AddActortoIgnore _output_get self)
  ;[1 1 1] Turn off the laser until it is needed
  (Default|SetActive _output_get false)
  ;[1 1 1] Set the type of laser to one of three types, specifically damage. Can be altered to a non-lethal slow one or a simple "none " option
  (bind _returnvalue_2 (Utilities|GetDataTableRow "/Game/LaserTypesTable.LaserTypesTable" (Utilities|Name|MakeLiteralName "Damage"))
    (:then
      (Default|SetLaserType _output_get _returnvalue_2)
      ;[1 1 1] Make laser a child actor (I believe) of the main boss actor for easier referencing and working with later.
      (Transformation|AttachActorToActor (Variables|Default|GetLaser) self "None" "KeepWorld" "KeepWorld" "KeepWorld" true))))

(event Collision|EventActorBeginOverlap
  (params (OtherActor :type Actor%20Object%20Reference)))

(event EventTick
  (params (DeltaSeconds :type Float%20%28single-precision%29))
  ;[1 1 1] Update boss' blackboard info regards player location
  (AI|Components|Blackboard|SetValueasVector (AI|GetBlackboard (Pawn|GetController)) (Utilities|Name|MakeLiteralName "PlayerPos") (Transformation|GetActorLocation (Game|GetPlayerCharacter 0)))
  ;[1 1 1] Increment the laser attack animation timer by one
  (Variables|Default|SetAttackAnimationTimer (+ DeltaSeconds (Variables|Default|GetAttackAnimationTimer)))
  (if (Variables|Default|GetPlayAttackAnimation)
    ;[1 1 1] If the Attack Animation timer reaches a certain threshold move onto playing the animation
    (if (>= (Variables|Default|GetAttackAnimationTimer) 0.2)
      ;[1 1 1] Increment the frame the animation is on and reset the timer
      (Variables|Default|SetAttackAnimationFrame (+ (Variables|Default|GetAttackAnimationFrame) 1.0))
      (Variables|Default|SetAttackAnimationTimer 0.0)
      ;[1 1 1] Switch statement to go between three different poses and a reset pin at the bottom
      (switch int (Math|Float|Truncate (Variables|Default|GetAttackAnimationFrame))
        (:1
          (Components|StaticMesh|SetStaticMesh (Variables|Default|GetBossIdle1) "/Game/Models/Boss/BossAttack1.BossAttack1"))
        (:2
          (Components|StaticMesh|SetStaticMesh (Variables|Default|GetBossIdle1) "/Game/Models/Boss/BossAttack2.BossAttack2"))
        (:3
          (Components|StaticMesh|SetStaticMesh (Variables|Default|GetBossIdle1) "/Game/Models/Boss/BossAttack3.BossAttack3"))
        (:4
          ;[1 1 1] Activate the laser attack and hold on the last frame
          (Default|SetActive (Variables|Default|GetLaser) true)
          (Utilities|FlowControl|Delay 2.0)
          ;[1 1 1] Reset the current attack animation frame and turn of playing attack animation
          (Variables|Default|SetAttackAnimationFrame 0.0)
          (Variables|Default|SetPlayAttackAnimation false)
          ;[1 1 1] Turn off the laser attack
          (Default|SetActive (Variables|Default|GetLaser) false))))
    (else
      ;[1 1 1] If the boss should not play its attack animation and is not actively attacking, give the boss its idle pose
      (if (not (Variables|Default|GetIsAttacking))
        (Components|StaticMesh|SetStaticMesh (Variables|Default|GetBossIdle1) "/Game/Models/Boss/BossIdle1.BossIdle1")))))

(event EventHitEvent
  (params (Damage :type Float%20%28double-precision%29))
  ;[1 1 1] If the boss is hit and they are not invulnerable to damage, apply damage to the boss
  (Development|PrintString (Utilities|String|ToString(Float) (Variables|Default|Gethealth)))
  (if (Variables|Default|Getis_stunned)
    (|CallParentFunction Damage 0)))

(fn ConstructionScript)

(fn ActivateStun
  (if (not (Variables|Default|Getis_stunned))
    (Development|PrintString "BOSS STUNNED")
    (Default|SetActive (Variables|Default|GetLaser) false)
    (AI|Components|Blackboard|SetValueasBool (AI|GetBlackboard (Pawn|GetController)) (Utilities|Name|MakeLiteralName "IsStunned") true)
    (Variables|Default|Setis_stunned true)))

(fn DeActivateStun
  (Development|PrintString "BOSS NOT STUNNED")
  (Variables|Default|Setis_stunned false))

(fn ActivateBoss
  (AI|Components|Blackboard|SetValueasBool (AI|GetBlackboard (Pawn|GetController)) (Utilities|Name|MakeLiteralName "IsActivated") true))