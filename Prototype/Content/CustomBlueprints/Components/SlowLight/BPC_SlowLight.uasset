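; BPC_SlowLight is a component for BP_ThirdPersonCharacter that spawns and removes BP_SlowLightObj actors.
; BeginPlay copies the character's LightTransform once, and CreateLight spawns at that stored location and rotation, records the actor in an array and sets CanRemove.
; When CanRemove is set, RemoveLight destroys array entries and clears the flag, but removing indices during the forward loop can skip entries.
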(event EventBeginPlay
  (bind _asbp_third_person_character (Utilities|Casting|CastToBP_ThirdPersonCharacter (Components|GetOwner)))
  (Variables|Default|SetSpawnTransform (Variables|/Game/ThirdPerson/Blueprints/BP_ThirdPersonCharacter.BP_ThirdPersonCharacter_C|GetLightTransform _asbp_third_person_character)))

(fn CreateLight
  (bind _spawntransform (Variables|Default|GetSpawnTransform))
  (bind _returnvalue (Game|SpawnActorfromClass "/Game/CustomBlueprints/Components/SlowLight/BP_SlowLightObj.BP_SlowLightObj_C" (Math|Transform|MakeTransform (.location _spawntransform) (.rotation _spawntransform) "1.000000,1.000000,1.000000") "Undefined" "MultiplyWithRoot" (Components|GetOwner) 0))
  (Utilities|Array|Add (Variables|Default|GetSlowLightRef) _returnvalue)
  (Variables|Default|SetCanRemove true))

(fn RemoveLight
  (bind _slowlightref (Variables|Default|GetSlowLightRef))
  (if (Variables|Default|GetCanRemove)
    (for (_array_element _array_index) _slowlightref
      (Actor|DestroyActor _array_element)
      (Utilities|Array|RemoveIndex _slowlightref _array_index)
      (Variables|Default|SetCanRemove false))))