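; BP_DarkRoomBossSpikeIndicator is a timed indicator for the dark room boss's spike attack, marking where a spike appears.
; Tick counts SpikeTimer down to zero, then applies Damage to the first BP_ThirdPersonCharacter overlapping its Hitsphere.
; It spawns a BP_DarkRoomBossSpike at its own X/Y and the SpikeSpawnAltitude height, then destroys itself.
; Damage comes from this overlap check at expiry, independent of the spawned spike.
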(event EventBeginPlay)

(event Collision|EventActorBeginOverlap
  (params (OtherActor :type Actor%20Object%20Reference)))

(event EventTick
  (params (DeltaSeconds :type Float%20%28single-precision%29))
  (bind _returnvalue (Transformation|GetActorTransform))
  (bind _output_get (Variables|Default|Setspike_timer (- (Variables|Default|Getspike_timer) DeltaSeconds)))
  (Math|Float|CompareFloat _output_get 0.0
    (:==
      _)
    (:<
      _))
  (bind _asbp_third_person_character (Utilities|Casting|CastToBP_ThirdPersonCharacter (Utilities|Array|Get(acopy) (Collision|GetOverlappingActors (Variables|Default|Gethitsphere) "/Game/ThirdPerson/Blueprints/BP_ThirdPersonCharacter.BP_ThirdPersonCharacter_C" :!class /Script/Engine.PrimitiveComponent)))
    (:then
      (Default|TakeDamage _asbp_third_person_character (Variables|Default|Getdamage)))
    (:CastFailed
      _))
  (Game|SpawnActorfromClass "/Game/CustomBlueprints/Components/DarkRoomBoss/BP_DarkRoomBossSpike.BP_DarkRoomBossSpike_C" (Math|Transform|MakeTransform (Math|Vector|MakeVector (.x (.location _returnvalue)) (.y (.location _returnvalue)) (Variables|Default|Getspike_spawn_altitude)) "0, 0, 0" "1.000000,1.000000,1.000000") "Undefined" "MultiplyWithRoot" 0 0)
  (Actor|DestroyActor))

(fn ConstructionScript)