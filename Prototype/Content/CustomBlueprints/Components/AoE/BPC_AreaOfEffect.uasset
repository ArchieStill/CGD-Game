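; Actor component that spawns and removes an area-of-effect bound around its owner, apparently for an ultimate ability.
; AwakeAreaOfEffect spawns BP_AreaOfEffectBound at the owner's X/Y, scales it by EffectSize, passes on FollowPlayer and stores it in an array.
; RemoveAreaOfEffect destroys stored bounds, removing entries while iterating the same array.
; A CanCallRemove flag, set on spawn and cleared on removal, gates repeated destroy calls.
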(event EventBeginPlay)

(event EventTick
  (params (DeltaSeconds :type Float%20%28single-precision%29)))

(fn AwakeAreaOfEffect
  (bind _returnvalue (Components|GetOwner))
  (bind _returnvalue_2 (Transformation|GetActorTransform _returnvalue))
  ;[1 0.5776 0.002125] Spawns in the area of effect and scales it to the desired size, It also spawns it to the centre of the player location
  (bind _returnvalue_3 (Game|SpawnActorfromClass "/Game/CustomBlueprints/Components/AoE/BP_AreaOfEffectBound.BP_AreaOfEffectBound_C" (Math|Transform|MakeTransform (Math|Vector|MakeVector (.x (.location _returnvalue_2)) (.y (.location _returnvalue_2)) 0.0) "0, 0, 0" (Math|Conversions|ToVector(Float) (Variables|Default|GetEffect%20Size))) "AlwaysSpawn" "OverrideRootScale" _returnvalue 0))
  ;[1 0.5776 0.002125] Adds the Area of Effect to array in case someone manages to spawn multiple
  (Utilities|Array|Add (Variables|Default|GetArea%20Of%20Effect%20Ref) _returnvalue_3)
  ;[1 0.5776 0.002125] Rather than meddling with a public vairable this just calls a function in the newly created Area of Effect that tells it whether or not to follow the player when active
  (Default|SetFollowPlayer _returnvalue_3 (Variables|Default|GetFollow%20Player))
  ;[1 0.5776 0.002125] This just stops an error where Unreal keeps trying to destroy an actor that is already destroyed
  (Variables|Default|SetCanCallRemove true))

(fn RemoveAreaOfEffect
  (bind _area_of_effect_ref (Variables|Default|GetArea%20Of%20Effect%20Ref))
  ;[1 0.5776 0.002125] Used as a gate to stop Unreal trying to destroy an actor that doesn't exist every update
  (if (Variables|Default|GetCanCallRemove)
    ;[1 0.5776 0.002125] For any Area of Effect that this component has spawned, destroy it and remove it from the array so Unreal does not try to access an empty array index after a few uses of the ultimate
    (for (_array_element _array_index) _area_of_effect_ref
      (Actor|DestroyActor _array_element)
      (Utilities|Array|RemoveIndex _area_of_effect_ref _array_index)
      ;[1 0.5776 0.002125] Update the gate so Unreal does not do the error thing mentioned earlier
      (Variables|Default|SetCanCallRemove false))))