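; BP_Gun is an automatic gun that fires a BP_Bullet at a fixed interval, with no input or trigger check.
; BeginPlay fills ShotCooldown from ShotCooldownMax, and Tick subtracts delta time from it every frame.
; When the cooldown reaches zero or below, it spawns the bullet at the gun's own transform and resets the timer.
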(event EventBeginPlay
  (Variables|Default|Setshot_cooldown (Variables|Default|Getshot_cooldown_max)))

(event EventTick
  (params (DeltaSeconds :type Float%20%28single-precision%29))
  (Variables|Default|Setshot_cooldown (- (Variables|Default|Getshot_cooldown) DeltaSeconds))
  (Math|Float|CompareFloat (Variables|Default|Getshot_cooldown) 0.0
    (:==
      _)
    (:<
      _))
  (Game|SpawnActorfromClass "/Game/CustomBlueprints/Normal/BP_Bullet.BP_Bullet_C" (Transformation|GetActorTransform) "Undefined" "MultiplyWithRoot" 0 0)
  (Variables|Default|Setshot_cooldown (Variables|Default|Getshot_cooldown_max)))

(fn ConstructionScript)