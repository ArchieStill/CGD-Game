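; Physics-driven ball boss that constantly accelerates toward the player and deals damage on overlap.
; A BP_FalseHammerHitWhenPlayerHit hit costs HP only while all guardians are dead, destroying the boss at zero.
; Each surviving hit spawns a guardian, plus another at one HP, and shows the protection sphere until Tick finds them all gone.
; Damage also triggers a leap and lunge at the player that doubles contact damage until impact stops it.
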(event OnComponentBeginOverlap(Sphere1)
  (params (OverlappedComponent :type Primitive%20Component%20Object%20Reference) (OtherActor :type Actor%20Object%20Reference) (OtherComp :type Primitive%20Component%20Object%20Reference) (OtherBodyIndex :type Integer) (bFromSweep :type Boolean) (SweepResult :type Hit%20Result%20Structure%20%28by%20ref%29))
  (bind _asbp_third_person_character (Utilities|Casting|CastToBP_ThirdPersonCharacter OtherActor))
  (if (Variables|Default|Getcancel%20vel%20when%20hit)
    (Default|TakeDamage _asbp_third_person_character 3.0)
    (else
      (Default|TakeDamage _asbp_third_person_character 1.5))))

(event OnComponentHit(Sphere)
  (params (HitComponent :type Primitive%20Component%20Object%20Reference) (OtherActor :type Actor%20Object%20Reference) (OtherComp :type Primitive%20Component%20Object%20Reference) (NormalImpulse :type Vector :default "0, 0, 0") (Hit :type Hit%20Result%20Structure%20%28by%20ref%29))
  (if (Variables|Default|Getcancel%20vel%20when%20hit)
    (Utilities|FlowControl|Delay 0.1)
    (Variables|Default|Setcancel%20vel%20when%20hit false)
    (Physics|SetPhysicsLinearVelocity (Variables|Default|GetSphere) "0, 0, 0" false "None")))

(event Custom|Damaged
  (Physics|AddImpulse (Variables|Default|GetSphere) "0.000000,0.000000,2000.000000" "None" true)
  (Utilities|FlowControl|Delay 1.2)
  (Physics|AddImpulse (Variables|Default|GetSphere) (* (Math|Vector|Normalize (- (Transformation|GetActorLocation (Game|GetPlayerCharacter 0)) (Transformation|GetWorldLocation (Variables|Default|GetSphere)))) 8e+03) "None" true)
  (Variables|Default|Setcancel%20vel%20when%20hit true))

(event EventBeginPlay
  (Rendering|SetVisibility (Variables|Default|GetProtectionSphere) false false))

(event EventTick
  (params (DeltaSeconds :type Float%20%28single-precision%29))
  (bind _returnvalue (Game|GetPlayerCharacter 0))
  (bind _sphere (Variables|Default|GetSphere))
  (bind _returnvalue_2 (Transformation|GetActorLocation _returnvalue))
  (bind _returnvalue_3 (Transformation|GetWorldLocation _sphere))
  (bind _returnvalue_4 (- _returnvalue_2 _returnvalue_3))
  (bind (_x _y) (Math|Vector|BreakVector _returnvalue_4))
  (Physics|AddForce (Variables|Default|GetSphere) (* (Math|Vector|Normalize (Math|Vector|MakeVector _x _y 0.0)) 5e+02) "None" true)
  (if (not (Variables|Default|Getguardiansdead))
    (Variables|Default|Setguardiansdead true)
    (bind _array_element (Utilities|Array|ForEachLoopwithBreak (Variables|Default|GetGuardians))
      (:LoopBody
        (if (Utilities|IsValid _array_element)
          (Variables|Default|Setguardiansdead false)))
      (:Completed
        (if (Variables|Default|Getguardiansdead)
          (Rendering|SetVisibility (Variables|Default|GetProtectionSphere) false false))))))

(event EventHit
  (params (Damage :type Float%20%28double-precision%29) (Hitter :type Actor%20Object%20Reference))
  (Utilities|Casting|CastToBP_FalseHammerHitWhenPlayerHit Hitter)
  (if (Variables|Default|Getguardiansdead)
    (bind _result (Math|Integer|DecrementInt (Variables|Default|Gethp))
      (:%20%20
        (if (<= _result 0)
          (Actor|DestroyActor)
          (else
            (CallFunction|Damaged)
            (Variables|Default|Setguardiansdead false)
            (bind _returnvalue (Game|SpawnActorfromClass "/Game/CustomBlueprints/BP_BallBossGuardian.BP_BallBossGuardian_C" (Transformation|GetActorTransform) "AdjustIfPossibleButAlwaysSpawn" "MultiplyWithRoot" 0 0))
            (Variables|/Game/CustomBlueprints/BP_BallBossGuardian.BP_BallBossGuardian_C|Settarget _returnvalue (Variables|Default|GetSphere))
            (Utilities|Array|Add (Variables|Default|GetGuardians) _returnvalue)
            (Rendering|SetVisibility (Variables|Default|GetProtectionSphere) true false)
            (if (== (Variables|Default|Gethp) 1)
              (bind _returnvalue_2 (Game|SpawnActorfromClass "/Game/CustomBlueprints/BP_BallBossGuardian.BP_BallBossGuardian_C" (Transformation|GetActorTransform (Variables|Default|Get2nd%20guardian%20spawn)) "AdjustIfPossibleButAlwaysSpawn" "MultiplyWithRoot" 0 0))
              (Variables|/Game/CustomBlueprints/BP_BallBossGuardian.BP_BallBossGuardian_C|Settarget _returnvalue_2 (Variables|Default|GetSphere))
              (Utilities|Array|Add (Variables|Default|GetGuardians) _returnvalue_2))))))))

(fn ConstructionScript)