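; Tutorial portal actor that teleports the third-person player character to a linked teleport pad.
; On overlap of its collider, it gets the pad's teleport location, moves the character there keeping its current rotation, and updates the character's location enum.
; The construction script applies the portal material and labels the portal with the name of its location enum value.
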(event OnComponentBeginOverlap(PortalCollidor)
  (params (OverlappedComponent :type Primitive%20Component%20Object%20Reference) (OtherActor :type Actor%20Object%20Reference) (OtherComp :type Primitive%20Component%20Object%20Reference) (OtherBodyIndex :type Integer) (bFromSweep :type Boolean) (SweepResult :type Hit%20Result%20Structure%20%28by%20ref%29))
  (bind _asbp_third_person_character (Utilities|Casting|CastToBP_ThirdPersonCharacter OtherActor))
  (bind _output_get (Default|GetTeleportLocation (Variables|Default|GetTeleportLocationPad)))
  (Transformation|Teleport _asbp_third_person_character _output_get (Transformation|GetActorRotation _asbp_third_person_character))
  (Default|UpdateLocationEnum _asbp_third_person_character (Variables|Default|Getlocation_enum)))

(event EventBeginPlay)

(event Collision|EventActorBeginOverlap
  (params (OtherActor :type Actor%20Object%20Reference)))

(event EventTick
  (params (DeltaSeconds :type Float%20%28single-precision%29)))

(fn ConstructionScript
  (Rendering|Material|SetMaterial (Variables|Default|GetPortal) 0 (Variables|Default|GetPortalMaterial))
  (Rendering|Components|TextRender|SetText (Variables|Default|GetPortalName) (Utilities|Text|ToText(String) (Utilities|String|EnumtoString (Variables|Default|Getlocation_enum)))))