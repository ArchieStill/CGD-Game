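; Ball boss guardian actor that damages the player character on contact and is visually tethered to a target point.
; Overlapping Sphere1 applies fixed damage to BP_ThirdPersonCharacter, while a Hit event from BP_FalseHammerHitWhenPlayerHit destroys the guardian.
; Each tick, the Tether is oriented from Sphere toward Target and stretched along Z by their distance, forming a laser-like link.
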(event OnComponentBeginOverlap(Sphere1)
  (params (OverlappedComponent :type Primitive%20Component%20Object%20Reference) (OtherActor :type Actor%20Object%20Reference) (OtherComp :type Primitive%20Component%20Object%20Reference) (OtherBodyIndex :type Integer) (bFromSweep :type Boolean) (SweepResult :type Hit%20Result%20Structure%20%28by%20ref%29))
  (bind _asbp_third_person_character (Utilities|Casting|CastToBP_ThirdPersonCharacter OtherActor))
  (Default|TakeDamage _asbp_third_person_character 0.7))

(event EventTick
  (params (DeltaSeconds :type Float%20%28single-precision%29))
  (bind _tether (Variables|Default|GetTether))
  (bind _sphere (Variables|Default|GetSphere))
  (bind _target (Variables|Default|Gettarget))
  (bind _tether_2 (Variables|Default|GetTether))
  (bind _returnvalue (Transformation|GetWorldLocation _target))
  (bind _returnvalue_2 (Transformation|GetWorldScale _tether))
  (bind (_x _y) (Math|Vector|BreakVector _returnvalue_2))
  (Transformation|SetWorldTransform _tether_2 (Class|KismetAnimationLibrary|Lookat (Transformation|GetWorldTransform _sphere) _returnvalue "0.000000,0.000000,1.000000" false "0, 0, 0" 0.0) false false)
  (Transformation|SetWorldScale3D _tether_2 "0.200000,0.200000,1.000000")
  ;[1 1 1] Scales the laser to reach the blocking hit
  (Transformation|SetWorldScale3D _tether (Math|Vector|MakeVector _x _y (/ (Math|Vector|Distance(Vector) (Transformation|GetWorldLocation _sphere) _returnvalue) 1e+02))))

(event EventHit
  (params (Damage :type Float%20%28double-precision%29) (Hitter :type Actor%20Object%20Reference))
  (Utilities|Casting|CastToBP_FalseHammerHitWhenPlayerHit Hitter)
  (Actor|DestroyActor))

(fn ConstructionScript)