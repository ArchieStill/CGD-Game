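; Parent Blueprint for enemies that travel a fixed path and deal contact damage to the player.
; The construction script feeds the control points and travel duration into an InterpToMovement component.
; Hitbox overlaps track player contact, and Tick applies damage through the player character whenever the cooldown has expired.
; Each hit also shows a damage indicator, which a short timer hides again.
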(event OnComponentBeginOverlap(hitbox)
  (params (OverlappedComponent :type Primitive%20Component%20Object%20Reference) (OtherActor :type Actor%20Object%20Reference) (OtherComp :type Primitive%20Component%20Object%20Reference) (OtherBodyIndex :type Integer) (bFromSweep :type Boolean) (SweepResult :type Hit%20Result%20Structure%20%28by%20ref%29))
  (if (Utilities|ClassIsChildOf (Utilities|GetClass OtherActor) "/Game/ThirdPerson/Blueprints/BP_ThirdPersonCharacter.BP_ThirdPersonCharacter_C")
    (Variables|Default|Setin_contact_with_player true)))

(event OnComponentEndOverlap(hitbox)
  (params (OverlappedComponent :type Primitive%20Component%20Object%20Reference) (OtherActor :type Actor%20Object%20Reference) (OtherComp :type Primitive%20Component%20Object%20Reference) (OtherBodyIndex :type Integer))
  (if (Utilities|ClassIsChildOf (Utilities|GetClass OtherActor) "/Game/ThirdPerson/Blueprints/BP_ThirdPersonCharacter.BP_ThirdPersonCharacter_C")
    (Variables|Default|Setin_contact_with_player false)))

(event EventBeginPlay
  (|CallParentFunction))

(event EventTick
  (params (DeltaSeconds :type Float%20%28single-precision%29))
  (CallFunction|UpdateDamageCooldown DeltaSeconds)
  (bind _out_touched_player (CallFunction|CheckTouchingPlayer))
  (CallFunction|UpdateDamageIndicator DeltaSeconds _out_touched_player))

(fn ConstructionScript
  (bind _interptomovement (Variables|Default|GetInterpToMovement))
  (|CallParentFunction)
  (Variables|/Script/Engine.InterpToMovementComponent|SetControlPoints _interptomovement (Variables|Default|Getcontrol_points))
  (Variables|/Script/Engine.InterpToMovementComponent|SetDuration _interptomovement (Variables|Default|Gettravel_duration)))

(fn UpdateDamageIndicator
  (params (delta_seconds :type Float%20%28double-precision%29) (touched_player :type Boolean))
  (bind _damage_indicator (Variables|Default|Getdamage_indicator))
  (if touched_player
    (Rendering|SetVisibility _damage_indicator true false)
    (Variables|Default|Setdamage_indicator_disappear_timer 0.3))
  (if (Variables|/Script/Engine.SceneComponent|GetbVisible _damage_indicator)
    (bind _output_get (Variables|Default|Setdamage_indicator_disappear_timer (- (Variables|Default|Getdamage_indicator_disappear_timer) delta_seconds)))
    (Math|Float|CompareFloat _output_get 0.0
      (:==
        _)
      (:<
        _))
    (Rendering|SetVisibility _damage_indicator false false)))

(fn UpdateDamageCooldown
  (params (delta%20seconds :type Float%20%28double-precision%29))
  (Math|Float|CompareFloat (Variables|Default|Getdamage_cooldown) 0.0
    (:>
      (Variables|Default|Setdamage_cooldown (- (Variables|Default|Getdamage_cooldown) delta%20seconds)))))

(fn CheckTouchingPlayer
  (if (Variables|Default|Getin_contact_with_player)
    (Math|Float|CompareFloat (Variables|Default|Getdamage_cooldown) 0.0
      (:>
        _)
      (:==
        (bind _asbp_third_person_character (Utilities|Casting|CastToBP_ThirdPersonCharacter (Game|GetPlayerCharacter 0) :!label _label))
        (Default|TakeDamage _asbp_third_person_character (Variables|Default|Getcontact_damage))
        (Variables|Default|Setdamage_cooldown (Variables|Default|Getdamage_cooldown_max))
        (LocalVariables|Settouched%20player true))
      (:<
        (goto _label))))
  (return (LocalVariables|Gettouched%20player)))