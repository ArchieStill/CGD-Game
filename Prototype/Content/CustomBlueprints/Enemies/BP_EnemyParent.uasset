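; Base enemy Blueprint that tracks health, starting at MaxHealth on BeginPlay, and destroys the actor when health reaches zero or below.
; Hit forwards only Damage to HitEvent, ignoring Reinforced and Hitter.
; HitEvent subtracts the damage and updates the floating health bar widget before the death check, which only runs if the widget cast succeeds.
; A separate TakeDamage function duplicates the HitEvent logic.
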(event Custom|Hit%20Event
  (params (Damage :type Float%20%28double-precision%29))
  (bind _output_get (Variables|Default|Sethealth (- (Variables|Default|Gethealth) Damage)))
  (bind _aswgt_bp_floating_healthbar (Utilities|Casting|CastToWGT_BP_FloatingHealthbar (UserInterface|GetUserWidgetObject (Variables|Default|GetWidget))))
  (Default|UpdateHealthBar _aswgt_bp_floating_healthbar _output_get (Variables|Default|Getmax_health))
  (Math|Float|CompareFloat _output_get 0.0
    (:==
      _)
    (:<
      _))
  (Actor|DestroyActor))

(event EventBeginPlay
  (Variables|Default|Sethealth (Variables|Default|Getmax_health)))

(fn ConstructionScript)

(fn TakeDamage
  (params (damage :type Float%20%28double-precision%29))
  (bind _output_get (Variables|Default|Sethealth (- (Variables|Default|Gethealth) damage)))
  (bind _aswgt_bp_floating_healthbar (Utilities|Casting|CastToWGT_BP_FloatingHealthbar (UserInterface|GetUserWidgetObject (Variables|Default|GetWidget))))
  (Default|UpdateHealthBar _aswgt_bp_floating_healthbar _output_get (Variables|Default|Getmax_health))
  (Math|Float|CompareFloat _output_get 0.0
    (:==
      _)
    (:<
      _))
  (Actor|DestroyActor))

(fn Hit
  (params (Damage :type Float%20%28double-precision%29) (Reinforced :type Boolean) (Hitter :type Actor%20Object%20Reference))
  (CallFunction|HitEvent Damage)
  (return))