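; BP_HealingTurret is an enemy turret that regenerates its own health over time.
; On Tick, while Health is below MaxHealth, it adds HealRate scaled by delta seconds.
; When healing overshoots the maximum, it clamps Health and updates the floating healthbar widget, which is not refreshed during intermediate healing.
; BeginPlay, overlap, Tick and construction all call the parent implementation.
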(event EventBeginPlay
  (|CallParentFunction))

(event Collision|EventActorBeginOverlap
  (params (OtherActor :type Actor%20Object%20Reference))
  (|CallParentFunction OtherActor))

(event EventTick
  (params (DeltaSeconds :type Float%20%28single-precision%29))
  (bind _max_health (Variables|Default|Getmax_health))
  (|CallParentFunction DeltaSeconds)
  (Math|Float|CompareFloat (Variables|Default|Gethealth) (Variables|Default|Getmax_health)
    (:<
      (bind _output_get (Variables|Default|Sethealth (+ (Variables|Default|Gethealth) (* (Variables|Default|Getheal_rate) DeltaSeconds))))
      (Math|Float|CompareFloat _output_get _max_health
        (:>
          (bind _output_get_2 (Variables|Default|Sethealth _max_health))
          (bind _aswgt_bp_floating_healthbar (Utilities|Casting|CastToWGT_BP_FloatingHealthbar (UserInterface|GetUserWidgetObject (Variables|Default|GetWidget))))
          (Default|UpdateHealthBar _aswgt_bp_floating_healthbar _output_get_2 (Variables|Default|Getmax_health)))))))

(fn ConstructionScript
  (|CallParentFunction))