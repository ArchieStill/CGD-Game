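; Base turret enemy Blueprint that automatically fires BP_Bullet actors on a repeating cooldown.
; BeginPlay loads ShotCooldown from MaxShotCooldown, and Tick counts it down by delta time.
; At zero or below, it spawns a bullet at the turret's own transform and resets the cooldown, with no targeting or aiming logic in this graph.
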(event EventBeginPlay
  (|CallParentFunction)
  (Variables|Default|Setshot_cooldown (Variables|Default|Getmax_shot_cooldown)))

(event EventTick
  (params (DeltaSeconds :type Float%20%28single-precision%29))
  (|CallParentFunction 0.0)
  (bind _output_get (Variables|Default|Setshot_cooldown (- (Variables|Default|Getshot_cooldown) DeltaSeconds)))
  (Math|Float|CompareFloat _output_get 0.0
    (:==
      _)
    (:<
      _))
  (Game|SpawnActorfromClass "/Game/CustomBlueprints/Projectiles/BP_Bullet.BP_Bullet_C" (Transformation|GetActorTransform) "Undefined" "MultiplyWithRoot" 0 0)
  (Variables|Default|Setshot_cooldown (Variables|Default|Getmax_shot_cooldown)))

(fn ConstructionScript
  (|CallParentFunction))