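; BP_DarkRoomBoss is an enemy boss Blueprint that is defeated through shape plate activations.
; ActivateShapePlate compares the given shape to CurrentShape and, on a match, removes it from ShapesLeft and randomly picks the next from the remainder.
; CheckIfDead then destroys the actor once ShapesLeft is empty, although the random pick runs before that check.
; The event graph holds only disabled placeholder events, so nothing here initializes the shapes.
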(event EventBeginPlay
  (|CallParentFunction) ; This node is disabled and will not be called.\nDrag off pins to build functionality.
)

(event Collision|EventActorBeginOverlap
  (params (OtherActor :type Actor%20Object%20Reference)))

(event EventTick
  (params (DeltaSeconds :type Float%20%28single-precision%29)))

(fn ConstructionScript
  (|CallParentFunction))

(fn ActivateShapePlate
  (params (shape :type ENM_DarkRoomBossShape%20Enum :default "NewEnumerator0"))
  (bind _shapes_left (Variables|Default|Getshapes_left))
  (if (== shape (Math|Conversions|ToInteger(Byte) (Variables|Default|Getcurrent_shape)))
    (Utilities|Array|RemoveItem _shapes_left shape)
    (Variables|Default|Setcurrent_shape (Utilities|Array|Get(acopy) _shapes_left (Math|Random|RandomInteger (Utilities|Array|Length _shapes_left))))
    (CallFunction|CheckifDead)))

(fn CheckifDead
  (if (Utilities|Array|IsEmpty (Variables|Default|Getshapes_left))
    (Actor|DestroyActor)))