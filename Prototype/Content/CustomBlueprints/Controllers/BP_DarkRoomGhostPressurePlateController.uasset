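; Controller actor for a dark room pressure plate puzzle that spawns a ghost once enough plates are activated.
; ActivatePlate increments a counter, and CheckGhostSpawn compares it to the required plate count, calling SpawnGhost when it meets or exceeds that threshold.
; SpawnGhost spawns a BP_Ghost at the GhostSpawnPoint component's world location.
; The event graph is empty and no guard prevents repeated spawns, so both functions rely on external callers.
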(event EventBeginPlay)

(event Collision|EventActorBeginOverlap
  (params (OtherActor :type Actor%20Object%20Reference)))

(event EventTick
  (params (DeltaSeconds :type Float%20%28single-precision%29)))

(fn ConstructionScript)

(fn ActivatePlate
  (Math|Integer|IncrementInt (Variables|Default|Getplates_activated)))

(fn CheckGhostSpawn
  (Math|Integer|CompareInt (Variables|Default|Getplates_activated) (Variables|Default|Getplates_for_ghost_spawn)
    (:>
      _)
    (:==
      _))
  (CallFunction|SpawnGhost))

(fn SpawnGhost
  (Game|SpawnActorfromClass "/Game/CustomBlueprints/Enemies/BP_Ghost.BP_Ghost_C" (Math|Transform|MakeTransform (Transformation|GetWorldLocation (Variables|Default|Getghost_spawn_point)) "0, 0, 0" "1.000000,1.000000,1.000000") "Undefined" "MultiplyWithRoot" 0 0))