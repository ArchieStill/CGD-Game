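; BP_CrystalDoor is a door that lights its crystal gem when opened, then moves after a countdown.
; OpenDoor swaps the gem to the lit material and starts the LightSigil countdown, driven by Tick.
; Once moving, Tick sets the door base's world Z to delta time minus its starting relative Z, rather than accumulating movement.
; The base scales to zero if its relative Z falls below a threshold.
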(event Custom|OpenDoor
  (Rendering|Material|SetMaterial (Variables|Default|GetCrystalGem) 0 "/Game/Materials/Crystal/M_CrystalLit.M_CrystalLit")
  (Variables|Default|SetLightOn true))

(event EventBeginPlay
  (bind _doorbase (Variables|Default|GetDoorBase))
  ;[1 1 1] Get base values of door
  (Variables|Default|SetBaseX (.x (.location (Transformation|GetRelativeTransform _doorbase))))
  (Variables|Default|SetBaseY (.y (.location (Transformation|GetRelativeTransform _doorbase))))
  (Variables|Default|SetBaseZ (.z (.location (Transformation|GetRelativeTransform _doorbase)))))

(event EventTick
  (params (DeltaSeconds :type Float%20%28single-precision%29))
  ;[1 1 1] Definitely a better way to do this lol
  (if (Variables|Default|GetLightOn)
    (CallFunction|LightSigil DeltaSeconds))
  ;[1 1 1] Move door by base Z - DT
  (if (Variables|Default|GetMoving)
    (Transformation|SetWorldTransform (Variables|Default|GetDoorBase) (Math|Transform|MakeTransform (Math|Vector|MakeVector (Variables|Default|GetBaseX) (Variables|Default|GetBaseY) (- DeltaSeconds (Variables|Default|GetBaseZ))) "0, 0, 0" "1.000000,1.000000,1.000000") false false)
    ;[1 1 1] If door reaches -100, effectively disappear
    (if (< (.z (.location (Transformation|GetRelativeTransform (Variables|Default|GetDoorBase)))) -1e+02)
      (Transformation|SetWorldScale3D (Variables|Default|GetDoorBase) "0, 0, 0"))))

(fn ConstructionScript)

(fn LightSigil
  (params (DT :type Float%20%28double-precision%29))
  (Variables|Default|SetLightTime (- (Variables|Default|GetLightTime) DT))
  (if (< (Variables|Default|GetLightTime) 0.0)
    (Variables|Default|SetMoving true)
    (Development|PrintString "DoorMoving")
    (Variables|Default|SetLightOn false)))