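; BP_HiddenObjectCrystal is a crystal that reveals a linked hidden object when hit.
; The first effective Hit swaps five crystal base meshes to an emissive turquoise material, then calls Show on ObjectToShow through the BPI_HiddenObject interface.
; The Activated flag is set only after that interface cast succeeds, blocking further hits.
; OpenDoor and the construction script are empty.
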(event EventHit
  (params (Damage :type Float%20%28double-precision%29) (Hitter :type Actor%20Object%20Reference))
  (if (not (Variables|Default|GetActivated))
    (Rendering|Material|SetMaterial (Variables|Default|GetCrystalBase) 0 "/Game/Materials/M_EmissiveTurquoise.M_EmissiveTurquoise")
    (bind _asbpi_hidden_object (Utilities|Casting|CastToBPI_HiddenObject (Variables|Default|GetObjectToShow)))
    (Default|Show _asbpi_hidden_object)
    (Variables|Default|SetActivated true)))

(fn ConstructionScript)

(fn OpenDoor)