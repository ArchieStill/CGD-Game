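; BP_Crystal is a crystal actor that activates when hit and signals a linked door.
; Its Hit event prints a debug string, swaps the five crystal base components to the lit material and sets the Activated flag.
; It then calls OpenDoor, which only lights the CrystalGem on the referenced DoorToOpen; no door movement happens in this Blueprint.
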(event EventBeginPlay)

(event Collision|EventActorBeginOverlap
  (params (OtherActor :type Actor%20Object%20Reference)))

(event EventTick
  (params (DeltaSeconds :type Float%20%28single-precision%29)))

(event EventHit
  (params (Damage :type Float%20%28double-precision%29))
  (Development|PrintString "CRYSTAL HIT")
  (Rendering|Material|SetMaterial (Variables|Default|GetCrystalBase) 0 "/Game/Materials/Crystal/M_CrystalLit.M_CrystalLit")
  (Variables|Default|SetActivated true)
  (CallFunction|OpenDoor))

(fn ConstructionScript)

(fn OpenDoor
  (Rendering|Material|SetMaterial (Variables|/Game/CustomBlueprints/Objects/BP_CrystalDoor.BP_CrystalDoor_C|GetCrystalGem (Variables|Default|GetDoorToOpen)) 0 "/Game/Materials/Crystal/M_CrystalLit.M_CrystalLit"))