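; BP_DarkRoomGhostPressurePlate is a one-shot pressure plate, named for a dark room ghost section, that fires when a BP_ThirdPersonCharacter overlaps its trigger.
; Activation turns the plate mesh red and sets an Activated flag that blocks repeat triggers from overlaps; nothing here resets it.
; It then finds the BP_DarkRoomGhostPressurePlateController with GetActorOfClass and calls ActivatePlate on it, passing no plate reference.
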(event OnComponentBeginOverlap(trigger)
  (params (OverlappedComponent :type Primitive%20Component%20Object%20Reference) (OtherActor :type Actor%20Object%20Reference) (OtherComp :type Primitive%20Component%20Object%20Reference) (OtherBodyIndex :type Integer) (bFromSweep :type Boolean) (SweepResult :type Hit%20Result%20Structure%20%28by%20ref%29))
  (if (Utilities|ClassIsChildOf (Utilities|GetClass OtherActor) "/Game/ThirdPerson/Blueprints/BP_ThirdPersonCharacter.BP_ThirdPersonCharacter_C")
    (if (not (Variables|Default|Getactivated))
      (CallFunction|Activate))))

(fn ConstructionScript)

(fn Activate
  (Rendering|Material|SetMaterial (Variables|Default|Getpressure_plate) 0 "/Game/Materials/M_Red.M_Red")
  (Variables|Default|Setactivated true)
  (bind _returnvalue (Actor|GetActorOfClass "/Game/CustomBlueprints/Controllers/BP_DarkRoomGhostPressurePlateController.BP_DarkRoomGhostPressurePlateController_C"))
  (Default|ActivatePlate _returnvalue))