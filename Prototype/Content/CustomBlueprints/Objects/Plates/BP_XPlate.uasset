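; BP_XPlate is a plate that lights up when the third-person character steps into its trigger.
; An overlap from a BP_ThirdPersonCharacter calls Activate once, guarded by the Activated flag.
; Activate swaps the XL and XR meshes to the lit crystal material and sets the flag.
; The Deactivate event is empty, so nothing here turns the plate back off.
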(event OnComponentBeginOverlap(trigger)
  (params (OverlappedComponent :type Primitive%20Component%20Object%20Reference) (OtherActor :type Actor%20Object%20Reference) (OtherComp :type Primitive%20Component%20Object%20Reference) (OtherBodyIndex :type Integer) (bFromSweep :type Boolean) (SweepResult :type Hit%20Result%20Structure%20%28by%20ref%29))
  (if (Utilities|ClassIsChildOf (Utilities|GetClass OtherActor) "/Game/ThirdPerson/Blueprints/BP_ThirdPersonCharacter.BP_ThirdPersonCharacter_C")
    (if (not (Variables|Default|Getactivated))
      (CallFunction|Activate))))

(event EventDeactivate)

(event EventActivate
  (Rendering|Material|SetMaterial (Variables|Default|GetXL) 0 "/Game/Materials/Crystal/M_CrystalLit.M_CrystalLit")
  (Variables|Default|Setactivated true))

(fn ConstructionScript)