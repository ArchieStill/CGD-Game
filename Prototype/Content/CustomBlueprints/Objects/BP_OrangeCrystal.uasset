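; BP_OrangeCrystal is a hittable crystal switch that shows or hides a linked object.
; Each Hit event toggles between Activate and Deactivate, swapping five crystal meshes between emissive and dark orange materials.
; Both functions call Show or Hide on ObjectToShow through BPI_Showable, updating the Activated flag only if that cast succeeds.
; The OpenDoor function is an empty stub.
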(event EventHit
  (params (Damage :type Float%20%28double-precision%29) (Hitter :type Actor%20Object%20Reference))
  (if (Variables|Default|GetActivated)
    (CallFunction|Deactivate)
    (else
      (CallFunction|Activate))))

(fn ConstructionScript)

(fn OpenDoor)

(fn Activate
  (Rendering|Material|SetMaterial (Variables|Default|GetCrystalBase) 0 "/Game/Materials/M_EmissiveOrange.M_EmissiveOrange")
  (bind _asbpi_showable (Utilities|Casting|CastToBPI_Showable (Variables|Default|GetObjectToShow)))
  (Default|Show _asbpi_showable)
  (Variables|Default|SetActivated true))

(fn Deactivate
  (Rendering|Material|SetMaterial (Variables|Default|GetCrystalBase) 0 "/Game/Materials/M_DarkOrange.M_DarkOrange")
  (bind _asbpi_showable (Utilities|Casting|CastToBPI_Showable (Variables|Default|GetObjectToShow)))
  (Default|Hide _asbpi_showable)
  (Variables|Default|SetActivated false))