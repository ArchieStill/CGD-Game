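; BP_SpinPlat is a spinning platform that continuously rotates its Cube component around the yaw axis.
; Tick adds relative rotation scaled by delta time and the SpinPlatSpeed variable, keeping the spin frame-rate independent.
; A SlowDown event and a debug-style 0 key binding both print a message and set the speed to the same fixed value.
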(event EventBeginPlay)

(event Collision|EventActorBeginOverlap
  (params (OtherActor :type Actor%20Object%20Reference)))

(event EventTick
  (params (DeltaSeconds :type Float%20%28single-precision%29))
  (Transformation|AddRelativeRotation (Variables|Default|GetCube) (Math|Rotator|MakeRotator 0.0 0.0 (* DeltaSeconds (Variables|Default|GetSpinPlatSpeed))) false false))

(event EventSlowDown
  (Development|PrintString "Hello")
  (Variables|Default|SetSpinPlatSpeed 1e+01))

(event Input|KeyboardEvents|0
  (params (Key :type Key%20Structure :default "None"))
  (:Pressed
    (Development|PrintString "Helasdasdasdaslo")
    (Variables|Default|SetSpinPlatSpeed 1e+01)))

(fn ConstructionScript)