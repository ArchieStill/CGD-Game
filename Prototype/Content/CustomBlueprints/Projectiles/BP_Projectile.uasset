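; BP_Projectile is a projectile actor that travels in a straight line and damages the player character on contact.
; Each Tick it moves along its local X axis by Speed and accumulates Lifetime, destroying itself once MaxLifetime is reached.
; When its Hitsphere overlaps a BP_ThirdPersonCharacter, it calls TakeDamage with Damage and destroys itself; other overlapping actors are ignored.
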(event OnComponentBeginOverlap(hitsphere)
  (params (OverlappedComponent :type Primitive%20Component%20Object%20Reference) (OtherActor :type Actor%20Object%20Reference) (OtherComp :type Primitive%20Component%20Object%20Reference) (OtherBodyIndex :type Integer) (bFromSweep :type Boolean) (SweepResult :type Hit%20Result%20Structure%20%28by%20ref%29))
  (bind _asbp_third_person_character (Utilities|Casting|CastToBP_ThirdPersonCharacter OtherActor))
  (Default|TakeDamage _asbp_third_person_character (Variables|Default|Getdamage))
  (Actor|DestroyActor))

(event EventTick
  (params (DeltaSeconds :type Float%20%28single-precision%29))
  (Transformation|AddActorLocalOffset (Math|Vector|MakeVector (* (Variables|Default|Getspeed) DeltaSeconds) 0.0 0.0) false false)
  (bind _output_get (Variables|Default|Setlifetime (+ (Variables|Default|Getlifetime) DeltaSeconds)))
  (Math|Float|CompareFloat _output_get (Variables|Default|Getmax_lifetime)
    (:>
      _)
    (:==
      _))
  (Actor|DestroyActor))

(fn ConstructionScript)