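; BP_ProtectionSphere is an actor that stays in the level until every actor in its Guardians array is gone.
; Each Tick it polls the array with IsValid, assuming all are dead until a valid entry clears the Guardiansdead flag.
; When no valid guardian remains, the sphere destroys itself.
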(event EventBeginPlay)

(event Collision|EventActorBeginOverlap
  (params (OtherActor :type Actor%20Object%20Reference)))

(event EventTick
  (params (DeltaSeconds :type Float%20%28single-precision%29))
  (if (not (Variables|Default|Getguardiansdead))
    (Variables|Default|Setguardiansdead true)
    (bind _array_element (Utilities|Array|ForEachLoopwithBreak (Variables|Default|GetGuardians))
      (:LoopBody
        (if (Utilities|IsValid _array_element)
          (Variables|Default|Setguardiansdead false)))
      (:Completed
        (if (Variables|Default|Getguardiansdead)
          (Actor|DestroyActor))))))

(fn ConstructionScript)