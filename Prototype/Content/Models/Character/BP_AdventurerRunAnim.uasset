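; Blueprint that fakes an adventurer run animation by swapping static meshes, apparently as a temporary stand-in.
; On BeginPlay an endless Delay loop cycles one static mesh component through run pose 1, idle, run pose 2 and idle at a fixed interval.
; The loop runs unconditionally, with no movement check, and a few unconnected SetStaticMesh nodes are left in the graph.
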(event EventBeginPlay
  (Utilities|FlowControl|Delay 0.2 :!label _label)
  (Components|StaticMesh|SetStaticMesh (Variables|Default|GetTempVenturerIdlePose1) "/Game/Models/Character/TempVenturerRunPose1.TempVenturerRunPose1")
  (Utilities|FlowControl|Delay 0.2)
  (Components|StaticMesh|SetStaticMesh (Variables|Default|GetTempVenturerIdlePose1) "/Game/Models/Character/TempVenturerIdlePose1.TempVenturerIdlePose1")
  (Utilities|FlowControl|Delay 0.2)
  (Components|StaticMesh|SetStaticMesh (Variables|Default|GetTempVenturerIdlePose1) "/Game/Models/Character/TempVenturerRunPose2.TempVenturerRunPose2")
  (Utilities|FlowControl|Delay 0.2)
  (Components|StaticMesh|SetStaticMesh (Variables|Default|GetTempVenturerIdlePose1) "/Game/Models/Character/TempVenturerIdlePose1.TempVenturerIdlePose1")
  (goto _label))

(fn ConstructionScript)