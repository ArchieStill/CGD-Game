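; BP_Music is a music controller actor that switches level 1 music between main and boss tracks and keeps an ambience sound replaying.
; StartBossMusic and StartMainMusic set the "Transitions" parameter on the FMODMusicLvl1 component and update the MainMusicOn flag.
; Tick feeds a Delay of about 29.5 seconds, which acts as a repeating timer that calls Play on FMODAmbience.
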(event EventBeginPlay)

(event Collision|EventActorBeginOverlap
  (params (OtherActor :type Actor%20Object%20Reference)))

(event EventTick
  (params (DeltaSeconds :type Float%20%28single-precision%29))
  (Utilities|FlowControl|Delay 29.538)
  (Class|FMODAudioComponent|Play (Variables|Default|GetFMODAmbience)))

(fn ConstructionScript)

(fn StartBossMusic
  (Class|FMODAudioComponent|SetParameter (Variables|Default|GetFMODMusicLvl1) "Transitions" 1.0)
  (Variables|Default|SetMainMusicOn false)
  (return))

(fn StartMainMusic
  (Class|FMODAudioComponent|SetParameter (Variables|Default|GetFMODMusicLvl1) "Transitions" 0.0)
  (Variables|Default|SetMainMusicOn true)
  (return))