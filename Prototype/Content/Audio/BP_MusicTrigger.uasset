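; BP_MusicTrigger is a one-shot trigger volume that advances the music when an actor leaves its box.
; The first end overlap sets Triggered before the cast to BP_ThirdPersonCharacter, so a non-player actor also uses it up.
; For the player, it finds BP_AudioEngine and starts boss music if main music is on, otherwise main music.
; Each branch ends in a short Delay with nothing after it.
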(event OnComponentEndOverlap(Box)
  (params (OverlappedComponent :type Primitive%20Component%20Object%20Reference) (OtherActor :type Actor%20Object%20Reference) (OtherComp :type Primitive%20Component%20Object%20Reference) (OtherBodyIndex :type Integer))
  (if (not (Variables|Default|GetTriggered))
    (Variables|Default|SetTriggered true)
    (Utilities|Casting|CastToBP_ThirdPersonCharacter OtherActor)
    (bind _returnvalue (Actor|GetActorOfClass "/Game/Audio/BP_AudioEngine.BP_AudioEngine_C"))
    (if (Variables|/Game/Audio/BP_AudioEngine.BP_AudioEngine_C|GetMainMusicOn _returnvalue)
      (Default|StartBossMusic _returnvalue)
      (Utilities|FlowControl|Delay 1.0)
      (else
        (Default|StartMainMusic _returnvalue)
        (Utilities|FlowControl|Delay 1.0)))))

(fn ConstructionScript)