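; Audio manager actor for the final room that switches between main music and boss music.
; BeginPlay creates both audio components and immediately fades the main track to silence.
; StartBossMusic and StartMainMusic crossfade the two tracks and update the MainMusicOn flag.
; Tick runs through a Delay, adding another unstored audio component roughly every 15 seconds.
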(event EventBeginPlay
  (bind _returnvalue (AddComponent|AddAudioComponent false))
  (bind _output_get (Variables|Default|SetMainMusic _returnvalue))
  (bind _returnvalue_2 (AddComponent|AddAudioComponent false))
  (Variables|Default|SetBossMusic _returnvalue_2)
  (Audio|Components|Audio|FadeOut _output_get 0.0 0.0 "Linear" :!class /Script/Engine.AudioComponent))

(event Collision|EventActorBeginOverlap
  (params (OtherActor :type Actor%20Object%20Reference)))

(event EventTick
  (params (DeltaSeconds :type Float%20%28single-precision%29))
  (Utilities|FlowControl|Delay 14.7685)
  (AddComponent|AddAudioComponent false))

(fn ConstructionScript)

(fn StartBossMusic
  (Audio|Components|Audio|FadeIn (Variables|Default|GetBossMusic) 1.0 0.5 0.0 "Logarithmic" :!class /Script/Engine.AudioComponent)
  (Audio|Components|Audio|FadeOut (Variables|Default|GetMainMusic) 1.0 0.0 "Logarithmic" :!class /Script/Engine.AudioComponent)
  (Variables|Default|SetMainMusicOn false)
  (return))

(fn StartMainMusic
  (Audio|Components|Audio|FadeOut (Variables|Default|GetBossMusic) 2.0 0.0 "Linear" :!class /Script/Engine.AudioComponent)
  (Audio|Components|Audio|FadeIn (Variables|Default|GetMainMusic) 2.0 0.8 0.0 "Linear" :!class /Script/Engine.AudioComponent)
  (Variables|Default|SetMainMusicOn true)
  (return))