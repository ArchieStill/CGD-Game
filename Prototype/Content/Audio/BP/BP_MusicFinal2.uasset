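; BP_MusicFinal2 controls the level 2 boss music by setting the "Transitions" parameter on FMODMusicLvl2.
; BeginPlay sets the same transition value that StartBossMusic uses.
; StartBossDrop switches to the drop value and clears MainMusicOn, while StartBossMusic restores the music value and sets the flag.
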(event EventBeginPlay
  (Class|FMODAudioComponent|SetParameter (Variables|Default|GetFMODMusicLvl2) "Transitions" 3.0))

(event EventTick
  (params (DeltaSeconds :type Float%20%28single-precision%29)))

(fn ConstructionScript)

(fn StartBossDrop
  (Class|FMODAudioComponent|SetParameter (Variables|Default|GetFMODMusicLvl2) "Transitions" 2.0)
  (Variables|Default|SetMainMusicOn false)
  (return))

(fn StartBossMusic
  (Class|FMODAudioComponent|SetParameter (Variables|Default|GetFMODMusicLvl2) "Transitions" 3.0)
  (Variables|Default|SetMainMusicOn true)
  (return))