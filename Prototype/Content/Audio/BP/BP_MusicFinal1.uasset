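; Music controller Blueprint that drives the FMODMusicLvl1 track and a looping ambience, with calls for boss music and a boss drop.
; Shortly after BeginPlay it sets the FMOD "Transitions" parameter to the same value StartBossMusic uses.
; StartBossMusic and StartBossDrop switch that parameter and toggle the MainMusicOn flag.
; A Delay on Tick replays FMODAmbience roughly every half minute.
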(event EventBeginPlay
  (Utilities|FlowControl|Delay 0.1)
  (Class|FMODAudioComponent|SetParameter (Variables|Default|GetFMODMusicLvl1) "Transitions" 3.0))

(event EventTick
  (params (DeltaSeconds :type Float%20%28single-precision%29))
  (Utilities|FlowControl|Delay 29.538)
  (Class|FMODAudioComponent|Play (Variables|Default|GetFMODAmbience)))

(fn ConstructionScript)

(fn StartBossDrop
  (Class|FMODAudioComponent|SetParameter (Variables|Default|GetFMODMusicLvl1) "Transitions" 2.0)
  (Variables|Default|SetMainMusicOn false)
  (return))

(fn StartBossMusic
  (Class|FMODAudioComponent|SetParameter (Variables|Default|GetFMODMusicLvl1) "Transitions" 3.0)
  (Variables|Default|SetMainMusicOn true)
  (return))