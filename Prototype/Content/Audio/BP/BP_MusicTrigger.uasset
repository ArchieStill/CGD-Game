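; BP_MusicTrigger is a one-shot trigger actor that switches music and boulder-chase audio when an overlap with its Box ends.
; SwitchMusic finds BP_MusicFinal1 by class and checks MainMusicOn.
; If main music is on, it starts the boss drop and plays BP_ChaseBoulder's FMOD rolling sound.
; Otherwise, it starts the main music and stops the rolling sound.
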(event OnComponentEndOverlap(Box)
  (params (OverlappedComponent :type Primitive%20Component%20Object%20Reference) (OtherActor :type Actor%20Object%20Reference) (OtherComp :type Primitive%20Component%20Object%20Reference) (OtherBodyIndex :type Integer))
  (if (not (Variables|Default|GetTriggered))
    (Variables|Default|SetTriggered true)
    (CallFunction|SwitchMusic)))

(fn ConstructionScript)

(fn SwitchMusic
  (bind _returnvalue (Actor|GetActorOfClass "/Game/Audio/BP/BP_MusicFinal1.BP_MusicFinal1_C"))
  (if (Variables|/Game/Audio/BP/BP_MusicFinal1.BP_MusicFinal1_C|GetMainMusicOn _returnvalue)
    (Default|StartBossDrop _returnvalue)
    ;[1 1 1] Play Boulder Rolling
    (bind _returnvalue_2 (Actor|GetActorOfClass "/Game/Blueprints/BoulderChase/BP_ChaseBoulder.BP_ChaseBoulder_C"))
    (Class|FMODAudioComponent|Play (Variables|/Game/Blueprints/BoulderChase/BP_ChaseBoulder.BP_ChaseBoulder_C|GetFMODBoulderRolling _returnvalue_2))
    (else
      (Default|StartMainMusic _returnvalue)
      (bind _returnvalue_3 (Actor|GetActorOfClass "/Game/Blueprints/BoulderChase/BP_ChaseBoulder.BP_ChaseBoulder_C"))
      (Class|FMODAudioComponent|Stop (Variables|/Game/Blueprints/BoulderChase/BP_ChaseBoulder.BP_ChaseBoulder_C|GetFMODBoulderRolling _returnvalue_3)))))