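; Audio trigger actor that switches the level 1 FMOD puzzle music as the player moves between a secret area and the main area.
; Entering the secret box sets the "Transitions" parameter on BP_MusicPuzzle1's music and fades out the secret's attract sound.
; Entering the main box resets only the music transition.
; The HasNotPlayed flag makes the two boxes alternate, preventing repeat triggers.
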(event OnComponentBeginOverlap(BoxCollisionSecret)
  (params (OverlappedComponent :type Primitive%20Component%20Object%20Reference) (OtherActor :type Actor%20Object%20Reference) (OtherComp :type Primitive%20Component%20Object%20Reference) (OtherBodyIndex :type Integer) (bFromSweep :type Boolean) (SweepResult :type Hit%20Result%20Structure%20%28by%20ref%29))
  (if (== (Utilities|GetClass OtherActor) (Utilities|GetClass (Game|GetPlayerCharacter 0)))
    (if (Variables|Default|GetHasNotPlayed)
      (Variables|Default|SetHasNotPlayed false)
      (bind _returnvalue (Actor|GetActorOfClass "/Game/Audio/BP/BP_MusicPuzzle1.BP_MusicPuzzle1_C"))
      (Class|FMODAudioComponent|SetParameter (Variables|/Game/Audio/BP/BP_MusicPuzzle1.BP_MusicPuzzle1_C|GetFMODMusicLvl1 _returnvalue) "Transitions" 1.0)
      (Class|FMODAudioComponent|SetParameter (Variables|Default|GetFMODSecretPuzzleAttract) "FadeOut" 1.0))))

(event OnComponentBeginOverlap(BoxCollisionMain)
  (params (OverlappedComponent :type Primitive%20Component%20Object%20Reference) (OtherActor :type Actor%20Object%20Reference) (OtherComp :type Primitive%20Component%20Object%20Reference) (OtherBodyIndex :type Integer) (bFromSweep :type Boolean) (SweepResult :type Hit%20Result%20Structure%20%28by%20ref%29))
  (if (== (Utilities|GetClass OtherActor) (Utilities|GetClass (Game|GetPlayerCharacter 0)))
    (if (not (Variables|Default|GetHasNotPlayed))
      (bind _returnvalue (Actor|GetActorOfClass "/Game/Audio/BP/BP_MusicPuzzle1.BP_MusicPuzzle1_C"))
      (Class|FMODAudioComponent|SetParameter (Variables|/Game/Audio/BP/BP_MusicPuzzle1.BP_MusicPuzzle1_C|GetFMODMusicLvl1 _returnvalue) "Transitions" 0.0)
      (Variables|Default|SetHasNotPlayed true))))

(event EventBeginPlay)

(event Collision|EventActorBeginOverlap
  (params (OtherActor :type Actor%20Object%20Reference)))

(event EventTick
  (params (DeltaSeconds :type Float%20%28single-precision%29)))

(fn ConstructionScript)