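; BP_ChaseBoulder is a rolling boulder for a chase sequence in the AlphaEnding level.
; While Active, Tick moves it along a fixed Direction and spins it about the perpendicular axis.
; Its speed rubber-bands around IdealSpeed, rising when the player is beyond the ideal distance and falling when closer, up to a maximum deviation.
; When the third-person character overlaps Sphere2, the Key component and that sphere are destroyed.
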(event OnComponentBeginOverlap(Sphere2)
  (params (OverlappedComponent :type Primitive%20Component%20Object%20Reference) (OtherActor :type Actor%20Object%20Reference) (OtherComp :type Primitive%20Component%20Object%20Reference) (OtherBodyIndex :type Integer) (bFromSweep :type Boolean) (SweepResult :type Hit%20Result%20Structure%20%28by%20ref%29))
  (Utilities|Casting|CastToBP_ThirdPersonCharacter OtherActor)
  (Components|DestroyComponent (Variables|Default|GetKey))
  (Components|DestroyComponent (Variables|Default|GetSphere2)))

(event EventTick
  (params (DeltaSeconds :type Float%20%28single-precision%29))
  (bind _returnvalue (Transformation|GetActorLocation))
  (bind _returnvalue_2 (Game|GetPlayerCharacter 0))
  (bind _distance_to_reach_max_speed_deviation (Variables|Default|Getdistance%20to%20reach%20max%20speed%20deviation))
  (bind _distance_to_reach_max_speed_deviation_2 (Variables|Default|Getdistance%20to%20reach%20max%20speed%20deviation))
  (bind _max_speed_deviation (Variables|Default|Getmax%20speed%20deviation))
  (bind _idealdistance (Variables|Default|Getidealdistance))
  (bind _returnvalue_3 (Transformation|GetActorLocation _returnvalue_2))
  (bind _returnvalue_4 (Math|Vector|Distance(Vector) _returnvalue_3 _returnvalue))
  (bind _returnvalue_5 (- _returnvalue_4 _idealdistance))
  (bind _returnvalue_6 (Math|Float|Absolute(Float) _returnvalue_5))
  (bind _returnvalue_7 (/ _returnvalue_6 _distance_to_reach_max_speed_deviation))
  (bind _returnvalue_8 (> _returnvalue_6 _distance_to_reach_max_speed_deviation_2))
  (bind _returnvalue_9 (* _returnvalue_7 _max_speed_deviation))
  (if (Variables|Default|GetActive)
    (Transformation|SetActorLocationAndRotation (+ (* DeltaSeconds (Variables|Default|Getdirection) (Variables|Default|Getspeed)) (Transformation|GetActorLocation)) (Math|Rotator|CombineRotators (Transformation|GetActorRotation) (Math|Vector|RotatorfromAxisandAngle (Math|Vector|CrossProduct (Variables|Default|Getdirection) "0.000000,0.000000,-1.000000") (/ (Variables|Default|Getspeed) 1.5e+02))))
    (if (> _returnvalue_4 _idealdistance)
      (if _returnvalue_8
        (Variables|Default|Setspeed (+ (Variables|Default|Getideal%20speed) (Variables|Default|Getmax%20speed%20deviation)))
        (else
          (Variables|Default|Setspeed (+ _returnvalue_9 (Variables|Default|Getideal%20speed)))))
      (elif _returnvalue_8
        (Variables|Default|Setspeed (+ (Variables|Default|Getideal%20speed) (* (Variables|Default|Getmax%20speed%20deviation) -1.0)))
        (else
          (Variables|Default|Setspeed (+ (* _returnvalue_9 -1.0) (Variables|Default|Getideal%20speed))))))))

(event EventBeginPlay
  (Variables|Default|Setspeed (Variables|Default|Getideal%20speed)))

(fn ConstructionScript)