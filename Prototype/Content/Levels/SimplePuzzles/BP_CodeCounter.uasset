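; BP_CodeCounter is a sequence puzzle that activates a target object, such as a door, when hammer buttons are triggered in array order.
; Until solved, Tick polls the buttons in reverse order for active ones not yet recorded in ButtonsOn.
; A correct button lights its matching glow text and advances CurrentIndex, while a wrong one resets the progress and text colours.
; Completing the sequence calls Activate through BPI_Activateable and stops the polling.
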(event EventBeginPlay
  (bind _output_get (Variables|Default|SetButtonsOn (Utilities|Array|MakeArray false)))
  (for _index (range 0 (- (Utilities|Array|Length (Variables|Default|GetButtons)) 1))
    (Utilities|Array|Add _output_get false)))

(event Collision|EventActorBeginOverlap
  (params (OtherActor :type Actor%20Object%20Reference)))

(event EventTick
  (params (DeltaSeconds :type Float%20%28single-precision%29))
  (if (not (Variables|Default|Getactivated))
    (CallFunction|CheckButtons)))

(fn ConstructionScript)

(fn CheckButtons
  (bind _buttons (Variables|Default|GetButtons))
  (bind _returnvalue (Utilities|Array|Length _buttons))
  (bind _returnvalue_2 (- _returnvalue 1))
  (for _index (range 0 _returnvalue_2)
    (bind _asbp_hammer_button (Utilities|Casting|CastToBP_HammerButton (Utilities|Array|Get(acopy) (Variables|Default|GetButtons) (- _returnvalue_2 _index))))
    (if (and (not (Utilities|Array|Get(acopy) (Variables|Default|GetButtonsOn) (- _returnvalue_2 _index))) (Variables|/Game/Levels/SimplePuzzles/BP_HammerButton.BP_HammerButton_C|Getactive _asbp_hammer_button))
      (if (== (- _returnvalue_2 _index) (Variables|Default|GetcurrentIndex))
        ;[1 1 1] Make text glow
        (bind _asbp_glow_text (Utilities|Casting|CastToBP_GlowText (Utilities|Array|Get(acopy) (Variables|Default|GetTextToGlow) (Variables|Default|GetcurrentIndex)))
          (:then
            (Rendering|Components|TextRender|SetTextRenderColor (Variables|/Game/Levels/SimplePuzzles/BP_GlowText.BP_GlowText_C|GetText _asbp_glow_text) (LocalVariables|GetTextGlowCol))
            ;[1 1 1] Add one to password array
            (Utilities|Array|SetArrayElem (Variables|Default|GetButtonsOn) (Variables|Default|GetcurrentIndex) true)
            (bind _result (Math|Integer|IncrementInt (Variables|Default|GetcurrentIndex))
              (:%20%20
                ;[1 1 1] Open door
                (if (>= _result (Utilities|Array|Length (Variables|Default|GetButtons)))
                  (bind _asbpi_activateable (Utilities|Casting|CastToBPI_Activateable (Variables|Default|GetObject%20To%20Activate)))
                  (Default|Activate _asbpi_activateable)
                  (Variables|Default|Setactivated true)))))
          (:CastFailed
            (Development|PrintString "Failed")))
        (else
          ;[1 1 1] Code incorrect - reset to 0
          (for (_ _array_index) (Variables|Default|GetButtonsOn)
            (Utilities|Array|SetArrayElem (Variables|Default|GetButtonsOn) _array_index false)
            ;[1 1 1] Revert colours
            (bind _asbp_glow_text_2 (Utilities|Casting|CastToBP_GlowText (Utilities|Array|Get(acopy) (Variables|Default|GetTextToGlow) _array_index))
              (:then
                (Rendering|Components|TextRender|SetTextRenderColor (Variables|/Game/Levels/SimplePuzzles/BP_GlowText.BP_GlowText_C|GetText _asbp_glow_text_2) (LocalVariables|GetTextBaseCol)))
              (:CastFailed
                (Development|PrintString "Failed"))))
          (Variables|Default|SetcurrentIndex 0))))))