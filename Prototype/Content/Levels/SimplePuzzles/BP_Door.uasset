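; BP_Door is a puzzle door that moves vertically to open and close when activated or deactivated.
; BeginPlay records the starting height, and a Timeline height track is added to it to set the actor's Z location.
; Activate plays the timeline and Deactivate reverses it, with an Active flag guarding against repeated calls.
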(event EventBeginPlay
  ;[1 1 1] Sets doors initail height
  (Variables|Default|Setstart%20height (.Z (Math|Vector|BreakVector (Transformation|GetActorLocation)))))

(event EventActivate
  (bind _returnvalue (Transformation|GetActorLocation))
  (bind (_x _y) (Math|Vector|BreakVector _returnvalue))
  ;[1 1 1] Opens the door
  (if (not (Variables|Default|Getactive))
    (Variables|Default|Setactive true)
    ;[1 1 1] Handles the door movements
    (bind _height (Timeline|Timeline Play)
      (:Update
        (Transformation|SetActorLocation (Math|Vector|MakeVector _x _y (+ _height (Variables|Default|Getstart%20height))) false false)))))

(event EventDeactivate
  (bind _returnvalue (Transformation|GetActorLocation))
  (bind (_x _y) (Math|Vector|BreakVector _returnvalue))
  ;[1 1 1] Closes the door
  (if (Variables|Default|Getactive)
    (Variables|Default|Setactive false)
    ;[1 1 1] Handles the door movements
    (bind _height (Timeline|Timeline Reverse)
      (:Update
        (Transformation|SetActorLocation (Math|Vector|MakeVector _x _y (+ _height (Variables|Default|Getstart%20height))) false false)))))

(fn ConstructionScript)