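; Puzzle hammer Blueprint that fakes a swing by swapping cube visibility and disposes of a chase boulder.
; HitStuff shows the strike cubes and calls BPI_Hittable on actors in its Box; Tick restores the pose after a short delay.
; A chase boulder entering the Box loses its ability to kill.
; After a hit, an in-place Boulder is "destroyed" by teleporting its sphere far away and playing explosion effects.
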(event OnComponentBeginOverlap(Box)
  (params (OverlappedComponent :type Primitive%20Component%20Object%20Reference) (OtherActor :type Actor%20Object%20Reference) (OtherComp :type Primitive%20Component%20Object%20Reference) (OtherBodyIndex :type Integer) (bFromSweep :type Boolean) (SweepResult :type Hit%20Result%20Structure%20%28by%20ref%29))
  (bind _asbp_chase_boulder (Utilities|Casting|CastToBP_ChaseBoulder OtherActor))
  (Variables|/Game/Levels/AlphaEnding/BP_ChaseBoulder.BP_ChaseBoulder_C|SetCanKill _asbp_chase_boulder false)
  (Variables|Default|SetBoulderInPlace true))

(event Custom|DestroyBoulder
  (if (Variables|Default|GetBoulderInPlace)
    (bind _asbp_chase_boulder (Utilities|Casting|CastToBP_ChaseBoulder (Variables|Default|GetBoulder)))
    (Transformation|SetWorldLocation (Variables|/Game/Levels/AlphaEnding/BP_ChaseBoulder.BP_ChaseBoulder_C|GetSphere _asbp_chase_boulder) "10000.000000,1000000.000000,1000000.000000" false true)
    (Audio|Components|Audio|Play (Variables|/Game/Levels/AlphaEnding/BP_ChaseBoulder.BP_ChaseBoulder_C|GetExplosionSFX _asbp_chase_boulder) 0.0)
    (Components|Activation|Activate (Variables|/Game/Levels/AlphaEnding/BP_ChaseBoulder.BP_ChaseBoulder_C|GetExplosionFX _asbp_chase_boulder) false)
    (Variables|Default|SetBoulderInPlace false)))

(event EventBeginPlay
  (Rendering|SetVisibility (Variables|Default|GetCube3) false false)
  (Rendering|SetVisibility (Variables|Default|GetCube4) false false))

(event EventTick
  (params (DeltaSeconds :type Float%20%28single-precision%29))
  (if (Variables|Default|Gethit)
    (Utilities|FlowControl|Delay 0.5)
    (Rendering|SetVisibility (Variables|Default|GetCube3) false false)
    (Rendering|SetVisibility (Variables|Default|GetCube4) false false)
    (Rendering|SetVisibility (Variables|Default|GetCube1) true false)
    (Rendering|SetVisibility (Variables|Default|GetCube2) true false)
    (if (Variables|Default|GetBoulderInPlace)
      (CallFunction|DestroyBoulder))
    (Variables|Default|Sethit false)))

(fn ConstructionScript)

(fn HitStuff
  (Variables|Default|Sethit true)
  (Rendering|SetVisibility (Variables|Default|GetCube3) true false)
  (Rendering|SetVisibility (Variables|Default|GetCube4) true false)
  (Rendering|SetVisibility (Variables|Default|GetCube1) false false)
  (Rendering|SetVisibility (Variables|Default|GetCube2) false false)
  (for _array_element (Collision|GetOverlappingActors (Variables|Default|GetBox) 0 :!class /Script/Engine.PrimitiveComponent)
    (bind _asbpi_hittable (Utilities|Casting|CastToBPI_Hittable _array_element))
    (Default|Hit _asbpi_hittable 0.0 self)))