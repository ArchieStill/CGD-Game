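; BP_LaserRedirector is a laser redirector that emits its own beam when hit by another laser and can turn in 90-degree steps.
; On BeginPlay it spawns an inactive BP_Laser attached to its Arrow; LaserHit sets that laser's type and activates it.
; Hit starts RotatingMovement, and Tick counts down one second, then snaps yaw to the target for an exact quarter turn.
; The Hity function duplicates the Hit logic.
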(event EventTick
  (params (DeltaSeconds :type Float%20%28single-precision%29))
  ;[1 1 1] Disables rotation after 1 second (to ensure a 90 degree turn)
  (if (Variables|Default|GetRotating)
    (bind _output_get (Variables|Default|SetRotateTimer (- (Variables|Default|GetRotateTimer) DeltaSeconds)))
    (if (<= _output_get 0.0)
      (Variables|Default|SetRotating false)
      (Transformation|SetActorRotation (Math|Rotator|MakeRotator 0.0 0.0 (Variables|Default|GetTargetRotation)))
      (Variables|/Script/Engine.RotatingMovementComponent|SetRotationRate (Variables|Default|GetRotatingMovement) "0, 0, 0"))))

(event EventHit
  (params (Damage :type Float%20%28double-precision%29))
  ;[1 1 1] Starts rotating if it isn't already
  (if (not (Variables|Default|GetRotating))
    (Variables|Default|SetRotating true)
    (Variables|Default|SetTargetRotation (+ (.Yaw (Math|Rotator|BreakRotator (Transformation|GetActorRotation))) 9e+01))
    (Variables|/Script/Engine.RotatingMovementComponent|SetRotationRate (Variables|Default|GetRotatingMovement) "0.000000,90.000000,0.000000")
    (Variables|Default|SetRotateTimer 1.0)))

(event EventBeginPlay
  ;[1 1 1] attaches the laser to the arrow
  (bind _returnvalue (Game|SpawnActorfromClass "/Game/Lasers/BP_Laser.BP_Laser_C" (Math|Transform|MakeTransform (Transformation|GetWorldLocation (Variables|Default|GetArrow)) (Transformation|GetActorRotation) "1.000000,1.000000,1.000000") "Undefined" "MultiplyWithRoot" 0 0))
  (bind _output_get (Variables|Default|SetLaser _returnvalue))
  ;;[1 1 1] Sets the laser to be inactive
  (Default|SetActive _output_get false)
  (Transformation|AttachComponentToComponent _output_get (Variables|Default|GetArrow) "None" "KeepWorld" "KeepWorld" "KeepWorld" true))

(event EventLaserHit
  (params (Location :type Vector :default "0, 0, 0") (Type :type Laser%20Type%20Structure))
  (bind _laser (Variables|Default|GetLaser))
  ;[1 1 1] Renews the laser if it receives input from another laser
  (Default|SetLaserType _laser Type)
  (Default|SetActive _laser true))

(fn ConstructionScript)

(fn Hity
  (if (not (Variables|Default|GetRotating))
    (Variables|Default|SetRotating true)
    (Variables|Default|SetTargetRotation (+ (.Yaw (Math|Rotator|BreakRotator (Transformation|GetActorRotation))) 9e+01))
    (Variables|/Script/Engine.RotatingMovementComponent|SetRotationRate (Variables|Default|GetRotatingMovement) "0.000000,90.000000,0.000000")
    (Variables|Default|SetRotateTimer 1.0)))