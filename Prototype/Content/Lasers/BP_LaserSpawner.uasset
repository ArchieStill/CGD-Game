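; BP_LaserSpawner spawns a BP_Laser at its Arrow component's location, using the spawner's rotation, when play begins.
; It looks up LaserTypeName in LaserTypesTable and, if the row exists, applies that laser type and attaches the laser to itself, keeping world transform.
; Every tick it sets the laser active.
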(event EventBeginPlay
  (bind _returnvalue (Game|SpawnActorfromClass "/Game/Lasers/BP_Laser.BP_Laser_C" (Math|Transform|MakeTransform (Transformation|GetWorldLocation (Variables|Default|GetArrow)) (Transformation|GetActorRotation) "1.000000,1.000000,1.000000") "Undefined" "MultiplyWithRoot" 0 0))
  (bind _output_get (Variables|Default|SetLaser _returnvalue))
  (bind _returnvalue_2 (Utilities|GetDataTableRow "/Game/Lasers/LaserTypesTable.LaserTypesTable" (Variables|Default|GetLaser%20Type%20Name))
    (:then
      (Default|SetLaserType _output_get _returnvalue_2)
      (Transformation|AttachActorToActor (Variables|Default|GetLaser) self "None" "KeepWorld" "KeepWorld" "KeepWorld" true))))

(event EventTick
  (params (DeltaSeconds :type Float%20%28single-precision%29))
  (Default|SetActive (Variables|Default|GetLaser) true))

(fn ConstructionScript)