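; BP_Laser is a laser beam actor that loads its default type and material from a data table on BeginPlay.
; While active, it line traces forward each Tick, stretches its mesh to the hit, and sends location and type to BPI_LaserInteractable actors.
; SetActive toggles visibility and resets a frame counter, so the beam switches off after LifetimeFrames unless reactivated.
; The trace's debug drawing is left on.
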(event EventBeginPlay
  (bind _returnvalue (Utilities|GetDataTableRow "/Game/Lasers/LaserTypesTable.LaserTypesTable" "Default")
    (:then
      (CallFunction|SetLaserType _returnvalue))))

(event EventTick
  (params (DeltaSeconds :type Float%20%28single-precision%29))
  (bind _returnvalue (Transformation|GetActorLocation))
  (bind _staticmesh (Variables|Default|GetStaticMesh))
  (bind _staticmesh_2 (Variables|Default|GetStaticMesh))
  (bind _returnvalue_2 (Transformation|GetWorldScale _staticmesh))
  (bind _returnvalue_3 (Transformation|GetWorldScale _staticmesh_2))
  (bind (_x _y) (Math|Vector|BreakVector _returnvalue_2))
  (bind (_x_2 _y_2) (Math|Vector|BreakVector _returnvalue_3))
  (CallFunction|CheckLifetime)
  (if (Variables|Default|GetActive)
    (bind (_outhit _returnvalue_4) (Collision|LineTraceForObjects _returnvalue (+ _returnvalue (* (Math|Vector|GetForwardVector (Variables|Default|GetArrow)) 1e+05)) (Utilities|Array|MakeArray "ObjectTypeQuery1" "ObjectTypeQuery3" "ObjectTypeQuery2" "ObjectTypeQuery4") false 0 "ForOneFrame"))
    (if _returnvalue_4
      (Transformation|SetWorldScale3D _staticmesh_2 (Math|Vector|MakeVector _x_2 _y_2 (/ (.Distance (Collision|BreakHitResult _outhit)) 1e+02)))
      (bind _asbpi_laser_interactable (Utilities|Casting|CastToBPI_LaserInteractable (.HitActor (Collision|BreakHitResult _outhit))))
      (Default|LaserHit _asbpi_laser_interactable (.Location (Collision|BreakHitResult _outhit)) (Variables|Default|GetLaserType))
      (else
        (Transformation|SetWorldScale3D _staticmesh (Math|Vector|MakeVector _x _y 1e+03))))))

(fn ConstructionScript)

(fn SetActive
  (params (New%20Active :type Boolean))
  (bind _output_get (Variables|Default|SetActive New%20Active))
  (if _output_get
    (Variables|Default|SetLifetimeFramesCounter 0))
  (Development|SetHiddeninGame (Variables|Default|GetStaticMesh) (not _output_get) false))

(fn CheckLifetime
  (if (Variables|Default|GetActive)
    (bind _output_get (Variables|Default|SetLifetimeFramesCounter (+ (Variables|Default|GetLifetimeFramesCounter) 1)))
    (if (>= _output_get (Variables|Default|GetLifetimeFrames))
      (CallFunction|SetActive false))))

(fn SetLaserType
  (params (Type :type Laser%20Type%20Structure))
  (bind _output_get (Variables|Default|SetLaserType Type))
  (Rendering|Material|SetMaterial (Variables|Default|GetStaticMesh) 0 (.Mat (Utilities|Struct|BreakLaserType _output_get))))